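; Weapon actor that fires projectiles in timed bursts with reload pauses for players, vehicles and AI.
; Firing RepNotify starts or cancels the self-rescheduling StartFire timer; Target changes set Firing, and Tick releases queued shots.
; Authority-only GetRotation aims from player or piloted-vehicle camera, otherwise at Target.
; Shots get random pitch/yaw spread, team and optional homing; non-player controllers retry until the target is visible.
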(event Custom|StartFire
  (bind _accuracy (Variables|Default|GetAccuracy))
  (bind _target (Variables|Default|GetTarget))
  (Development|PrintString "Fire")
  (bind _combatowner (Variables|Default|GetCombatOwner)
    (:then
      (Utilities|Casting|CastToPlayerController (Pawn|GetController _combatowner)
        (:then
          (bind (_direction _team) (Utilities|GetRotation :!label _label)
            (:Valid
              (bind _returnvalue (Game|SpawnActorfromClass (Variables|Default|GetProjClass) (Math|Transform|MakeTransform (Transformation|GetSocketLocation (Variables|Default|GetSkeletalMesh) (Variables|Default|GetGunMuzzleName)) (Math|Rotator|MakeRotator (.Roll (Math|Rotator|BreakRotator _direction)) (+ (.Pitch (Math|Rotator|BreakRotator _direction)) (Math|Random|RandomFloatinRange (* _accuracy -1.0) _accuracy)) (+ (.Yaw (Math|Rotator|BreakRotator _direction)) (Math|Random|RandomFloatinRange (* _accuracy -1.0) _accuracy))) "1.000000,1.000000,1.000000") "AlwaysSpawn" self _team 0))
              (Utilities|IsValid _returnvalue
                (:Is%20Valid
                  (Variables|Default|SetCurrentProj _returnvalue)
                  (if (and (Variables|/Script/Engine.ProjectileMovementComponent|GetbIsHomingProjectile (Variables|/Game/Blueprints/BP_Projectile.BP_Projectile_C|GetProjectileMovement _returnvalue)) (Utilities|IsValid _target))
                    (Variables|/Script/Engine.ProjectileMovementComponent|SetHomingTargetComponent (Variables|/Game/Blueprints/BP_Projectile.BP_Projectile_C|GetProjectileMovement _returnvalue) (VehicleSound|GetRootComponent _target)))
                  (Math|Integer|IncrementInt (Variables|Default|GetCurrentBurst)
                    (:%20%20
                      (if (< (Variables|Default|GetCurrentBurst) (Variables|Default|GetBurstLength))
                        (bind _returnvalue_2 (Utilities|Time|SetTimerbyEvent (delegate Custom|StartFire) (Variables|Default|GetFireSpeed)))
                        (Variables|Default|SetCurrentHandle _returnvalue_2)
                        (else
                          (bind _returnvalue_3 (Utilities|Time|SetTimerbyEvent (delegate Custom|StartFire) (Variables|Default|GetReloadTime)))
                          (Variables|Default|SetCurrentHandle _returnvalue_3)
                          (Variables|Default|SetCurrentBurst 0))))))))
            (:Invalid
              (Variables|Default|SetbFiring false))))
        (:CastFailed
          (Development|PrintString "AI")
          (if (Default|CanSeeTarget _combatowner)
            (goto _label)
            (else
              (Utilities|Time|SetTimerbyEvent (delegate Custom|StartFire) 0.1)
              (Development|PrintString "cant see"))))))
    (:else)))

(event EventTick
  (params (DeltaSeconds :type Float%20%28single-precision%29))
  (if (Math|Boolean|ANDBoolean (Variables|Default|GetbQueueFire) (not (Utilities|Time|IsTimerActivebyHandle (Variables|Default|GetCurrentHandle))) (Utilities|IsValid (Variables|Default|GetTarget)))
    (Variables|Default|SetbQueueFire false)
    (CallFunction|StartFire)))

(fn ConstructionScript)

(fn OnRepBFiring
  (if (Variables|Default|GetbFiring)
    (CallFunction|StartFire)
    (else
      (Class|KismetSystemLibrary|ClearTimerHandle (Variables|Default|GetCurrentHandle)))))

(fn OnRepTarget
  (Variables|Default|SetbFiring (Utilities|IsValid (Variables|Default|GetTarget))))