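; Placement preview actor for building structures that follows the owning player's vision trace and updates a CanPlace flag every tick.
; A chain of test macros checks He3 cost, command centre radius, flat ground, mesh overlaps, structure caps and nearby pawns, with any failure blocking placement.
; Command centres also trace upward for a territory volume, requiring one that lacks a command centre for that owner.
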(event EventTick
  (params (DeltaSeconds :type Float%20%28single-precision%29))
  (bind _primaryowner (Variables|Default|GetPrimaryOwner))
  (bind _hitresult (Default|VisionTrace _primaryowner))
  (bind (_bblockinghit _binitialoverlap _time _location _impactpoint _normal _impactnormal _physmat _hitactor) (Collision|BreakHitResult _hitresult))
  ;[1 1 1] Can Place
  (Transformation|SetActorLocation _location false false)
  (bind (_outhits _returnvalue) (Collision|MultiSphereTraceForObjects _location (+ _location "0, 0,4.000000") (/ (Math|Vector|VectorLength (.BoxExtent (Collision|GetActorBounds true))) (Math|Float|Sqrt 2.0)) (Utilities|Array|MakeArray "ObjectTypeQuery3") false (Utilities|Array|MakeArray _primaryowner) "None"))
  (Utilities|He3Test
    (:True
      (Utilities|ProximityTest
        (:True
          (Utilities|NormalTest _normal
            (:True
              (Utilities|OverlapTest _hitactor
                (:True
                  (Utilities|TerritoryTest
                    (:True
                      (Utilities|PopulationTest
                        (:True
                          (Utilities|PawnTest _outhits _returnvalue
                            (:True
                              (Variables|Default|SetbCanPlace true))
                            (:False
                              (Variables|Default|SetbCanPlace false :!label _label))))
                        (:False
                          (goto _label))))
                    (:False
                      (goto _label))))
                (:False
                  (goto _label))))
            (:False
              (goto _label))))
        (:False
          (goto _label))))
    (:False
      (goto _label))))

(fn ConstructionScript)