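; BP_Extractor is an extractor actor that generates He3 for its owning player or AI.
; On BeginPlay it claims the first BP_He3Deposit found within 128 units and marks it used, releasing it when destroyed.
; A looping Delay of 1/He3Rate adds one He3 to the PrimaryOwner's PlayerController, or its AI otherwise, up to He3Cap.
; Income runs whether or not a deposit was found.
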(event EventDestroyed
  ;[1 1 1] Add He3
  (bind _deposit (Variables|Default|GetDeposit)
    (:then
      (Variables|/Game/Environment/Objects/He3Deposit/BP_He3Deposit.BP_He3Deposit_C|SetbUsed _deposit false))
    (:else)))

(event EventBeginPlay
  ;[1 1 1] Add He3
  (|CallParentFunction)
  (CallFunction|SetDeposit)
  (Utilities|FlowControl|Delay (/ 1.0 (Variables|Default|GetHe3Rate)) :!label _label)
  (CallFunction|AddHe3)
  (goto _label))

(fn ConstructionScript)

(fn SetDeposit
  (bind _outactors (Actor|GetAllActorsOfClass "/Game/Environment/Objects/He3Deposit/BP_He3Deposit.BP_He3Deposit_C"))
  (bind _array_element (Utilities|Array|ForEachLoopwithBreak _outactors :!label _label)
    (:LoopBody
      (if (<= (Transformation|GetDistanceTo _array_element self) 128.0)
        (bind _output_get (Variables|Default|SetDeposit _array_element))
        (Variables|/Game/Environment/Objects/He3Deposit/BP_He3Deposit.BP_He3Deposit_C|SetbUsed _output_get true)
        (goto _label Break)))))

(fn AddHe3
  (bind _primaryowner (Variables|Default|GetPrimaryOwner)
    (:then
      (bind _playercontroller (Variables|/Game/Blueprints/BP_PlayerPrimary.BP_PlayerPrimary_C|GetPlayerController _primaryowner)
        (:then
          (if (< (Variables|/Game/Blueprints/BP_OpulentiumPlayerController.BP_OpulentiumPlayerController_C|GetHe3 _playercontroller) (Variables|/Game/Blueprints/BP_OpulentiumPlayerController.BP_OpulentiumPlayerController_C|GetHe3Cap _playercontroller))
            (Math|Integer|IncrementInt (Variables|/Game/Blueprints/BP_OpulentiumPlayerController.BP_OpulentiumPlayerController_C|GetHe3 _playercontroller))))
        (:else
          (bind _ai (Variables|/Game/Blueprints/BP_PlayerPrimary.BP_PlayerPrimary_C|GetAI _primaryowner)
            (:then
              (if (< (Variables|/Game/Blueprints/BP_OpulentiumAI.BP_OpulentiumAI_C|GetHe3 _ai) (Variables|/Game/Blueprints/BP_OpulentiumAI.BP_OpulentiumAI_C|GetHe3Cap _ai))
                (Math|Integer|IncrementInt (Variables|/Game/Blueprints/BP_OpulentiumAI.BP_OpulentiumAI_C|GetHe3 _ai))))
            (:else)))))
    (:else)))