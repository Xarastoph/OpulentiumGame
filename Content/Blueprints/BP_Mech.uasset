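; BP_Mech is a selectable mech unit that turns to face targets and can transform into a deployed actor.
; RepNotifies drive the Lookat state, which starts a Pivot timeline scaled by turn rate, then gates per-tick target tracking or triggers Transform.
; Transform plays an animation, then spawns DeployedClass with proportional health and preserved selection before destroying the mech.
; TempTarget temporarily feeds BP_MechBot's follow actor, clearing on a retriggerable delay.
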(event Custom|ResetTempTarget
  (Utilities|FlowControl|RetriggerableDelay 1e+01)
  (Variables|Default|SetTempTarget 0))

(event Custom|PivotActor
  (bind _btransform (Variables|Default|GetbTransform))
  (bind _output_get (Variables|Default|SetOldRot (Transformation|GetActorRotation)))
  (Components|Timeline|SetPlayRate (Variables|Default|GetPivot) (/ 1.0 (Variables|Default|GetTurnRate)))
  (bind _time (Timeline|Pivot PlayFromStart)
    (:Update
      (if _btransform
        (Transformation|SetActorRotation (Math|Rotator|Lerp(Rotator) _output_get (stale _output_get_2) _time true) :!label _label)
        (if (Math|Boolean|ANDBoolean (>= _time 0.8) (Utilities|IsValid (Variables|Default|GetCurrentTarget)) (not (Utilities|IsValid (Utilities|Array|Get(acopy) (Variables|Default|GetWeapons)))))
          (CallFunction|FireWeapon))
        (else
          (bind _currenttarget (Variables|Default|GetCurrentTarget)
            (:then
              (bind _output_get_2 (Variables|Default|SetDesiredRot (Math|Rotator|FindLookatRotation (Transformation|GetActorLocation) (Transformation|GetActorLocation _currenttarget))))
              (goto _label))
            (:else
              (Timeline|Pivot Stop))))))
    (:Finished
      (Variables|Default|SetbLookat false)
      (if _btransform
        (CallFunction|Transform)
        (else
          (Utilities|FlowControl|Gate true) ; enters at Open
        )))))

(event Custom|Transform
  (bind _returnvalue (Transformation|GetActorTransform))
  (bind _self self)
  (bind (_location _rotation _scale) (Math|Transform|BreakTransform _returnvalue))
  (Transformation|SetActorRotation (Variables|Default|GetDesiredRot))
  (Variables|Default|SetbPlayAnim true)
  (Utilities|FlowControl|Delay (Variables|Default|GetAnimDuration))
  (bind _primaryowner (Variables|Default|GetPrimaryOwner)
    (:then
      (bind _returnvalue_2 (Game|SpawnActorfromClass (Variables|Default|GetDeployedClass) (Math|Transform|MakeTransform (+ _location (Math|Vector|MakeVector 0.0 0.0 (- (Utilities|GetClassDefaults (Variables|Default|GetDeployedClass)) (Components|Capsule|GetScaledCapsuleHalfHeight (Variables|Default|GetCapsuleComponent))))) _rotation _scale) "AlwaysSpawn" (Components|GetOwner) _primaryowner (Variables|Default|GetTeam)))
      (Variables|/Game/Blueprints/BP_OpulentiumActor.BP_OpulentiumActor_C|SetHealth _returnvalue_2 (Math|Float|Truncate (* (Variables|/Game/Blueprints/BP_OpulentiumActor.BP_OpulentiumActor_C|GetHealthMax _returnvalue_2) (/ (Math|Conversions|ToFloat(Integer) (Variables|Default|GetHealth)) (Math|Conversions|ToFloat(Integer) (Variables|Default|GetHealthMax))))))
      (if (Variables|Default|GetbSelected)
        (Default|AddSelection _primaryowner _returnvalue_2 (== _returnvalue_2 (Variables|/Game/Blueprints/BP_PlayerPrimary.BP_PlayerPrimary_C|GetSelected _primaryowner))))
      (Default|ClearGroups _primaryowner _self)
      (Actor|DestroyActor _self))
    (:else)))

(event EventOnRepCurrentTarget
  (Variables|Default|SetbLookat (or (Utilities|IsValid (Variables|Default|GetCurrentTarget)) (Variables|Default|GetbTransform)))
  (Utilities|FlowControl|Gate true) ; enters at Close
)

(event EventTick
  (params (DeltaSeconds :type Float%20%28single-precision%29))
  (|CallParentFunction DeltaSeconds)
  (Utilities|FlowControl|Gate true :!label _label
    (:Exit
      (bind _currenttarget (Variables|Default|GetCurrentTarget)
        (:then
          (Transformation|SetActorRotation (Math|Rotator|FindLookatRotation (Transformation|GetActorLocation) (Transformation|GetActorLocation _currenttarget))))
        (:else
          (goto _label Close))))))

(fn ConstructionScript
  (|CallParentFunction))

(fn OnRepBCanSelect
  (if (not (Variables|Default|GetbCanSelect))
    (Variables|Default|SetbSelected false)
    (bind _primaryowner (Variables|Default|GetPrimaryOwner)
      (:then
        (bind _asbp_mech_bot (Utilities|Casting|CastToBP_MechBot (Pawn|GetController)))
        (if (not (Variables|/Game/Blueprints/AI/BP_MechBot.BP_MechBot_C|GetbEnterTransport _asbp_mech_bot))
          (Default|ClearGroups _primaryowner self)))
      (:else))))

(fn OnRepBLookat
  (bind _blookat (Variables|Default|GetbLookat))
  (Variables|/Script/Engine.CharacterMovementComponent|SetbOrientRotationToMovement (Variables|Character|GetCharacterMovement) (not _blookat))
  (if _blookat
    (CallFunction|PivotActor)
    (elif (not (Variables|Default|GetbTransform))
      (Audio|Components|Audio|Stop (Variables|Default|GetPivot)))))

(fn TargetPos
  (params (Actor :type Actor%20Object%20Reference))
  (bind _returnvalue (Transformation|GetActorLocation Actor))
  (Utilities|Casting|CastToBP_CombatActor Actor
    (:then
      (bind _output_get (LocalVariables|SetLocalPos _returnvalue)))
    (:CastFailed
      (LocalVariables|SetLocalPos (+ (Math|Vector|MakeVector 0.0 0.0 (/ (.Z (Math|Vector|BreakVector (.BoxExtent (Collision|GetActorBounds Actor false)))) 2.0)) _returnvalue))))
  (return _output_get))

(fn OnRepBTransform
  (Variables|Default|SetbLookat (Variables|Default|GetbTransform)))

(fn OnRepCurrentPlacement
  (bind _currentplacement (Variables|Default|GetCurrentPlacement)
    (:then
      (Variables|Default|SetDesiredRot (Transformation|GetActorRotation _currentplacement)))
    (:else)))

(fn RemovefromArray
  (params (Mechs :type Array%20of%20BP%20Mech%20Object%20References) (Mech :type BP%20Mech%20Object%20Reference))
  (bind _return (LocalVariables|GetReturn))
  (for _array_element Mechs
    (Utilities|IsValid _array_element
      (:Is%20Valid
        (if (!= _array_element Mech)
          (Utilities|Array|Add _return _array_element)))))
  (return _return))

(fn OnRepTempTarget
  (bind _asbp_mech_bot (Utilities|Casting|CastToBP_MechBot (Pawn|GetController)))
  (bind _temptarget (Variables|Default|GetTempTarget)
    (:then
      (CallFunction|ResetTempTarget)
      (Variables|/Game/Blueprints/AI/BP_MechBot.BP_MechBot_C|GetFollowActor _asbp_mech_bot
        (:then)
        (:else
          (Variables|/Game/Blueprints/AI/BP_MechBot.BP_MechBot_C|SetFollowActor _asbp_mech_bot _temptarget)
          (if (Variables|/Game/Blueprints/AI/BP_MechBot.BP_MechBot_C|GetbMoveToRally _asbp_mech_bot)
            (Variables|/Game/Blueprints/AI/BP_MechBot.BP_MechBot_C|SetbMoveToRally _asbp_mech_bot false)))))
    (:else
      (if (== _temptarget (stale _output_get))
        (bind _output_get (Variables|/Game/Blueprints/AI/BP_MechBot.BP_MechBot_C|SetFollowActor _asbp_mech_bot 0))))))