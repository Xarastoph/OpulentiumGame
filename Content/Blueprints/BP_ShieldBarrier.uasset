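; BP_ShieldBarrier is a replicated shield barrier that absorbs damage, regenerates health and returns after breaking.
; TakeDamage lowers Health and clears Shields; a retriggerable delay restores Shields, letting the polling loop started at BeginPlay regenerate Health.
; RepNotifies drive state: zero Health hides ShieldMesh, disables OverlapMesh collision and sets Off.
; After a delay, clearing Off shows ShieldMesh, enables its query collision and refills Health.
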(event Custom|SetShields
  (Utilities|FlowControl|RetriggerableDelay (Variables|Default|GetRegenDelay))
  (Variables|Default|SetbShields true))

(event Custom|ResetShield
  (Utilities|FlowControl|Delay (Variables|Default|GetResetDelay))
  (Variables|Default|SetbOff false))

(event EventBeginPlay
  (Utilities|FlowControl|Delay 0.1 :!label _label)
  (if (and (< (Variables|Default|GetHealth) (Variables|Default|GetHealthMax)) (Variables|Default|GetbShields))
    (Variables|Default|SetHealth (+ (Variables|Default|GetHealth) (Variables|Default|GetHealthIncrement)))
    (goto _label)
    (else
      (goto _label))))

(fn ConstructionScript)

(fn OnRepHealth
  (if (<= (Variables|Default|GetHealth) 0.0)
    (Development|SetHiddeninGame (Variables|Default|GetShieldMesh) true true)
    (Collision|SetCollisionEnabled (Variables|Default|GetOverlapMesh) "NoCollision")
    (Variables|Default|SetbOff true)))

(fn OnRepBShields
  (if (not (Variables|Default|GetbShields))
    (CallFunction|SetShields)))

(fn TakeDamage
  (params (Damage :type Integer))
  (if (> (- (Variables|Default|GetHealth) (Math|Conversions|ToFloat(Integer) Damage)) 0.0)
    (Variables|Default|SetHealth (- (Variables|Default|GetHealth) (Math|Conversions|ToFloat(Integer) Damage)))
    (else
      (Variables|Default|SetHealth 0.0)))
  (Variables|Default|SetbShields false)
  (CallFunction|SetShields))

(fn OnRepBOff
  (bind _shieldmesh (Variables|Default|GetShieldMesh))
  (if (Variables|Default|GetbOff)
    (CallFunction|ResetShield)
    (else
      (Development|SetHiddeninGame _shieldmesh false true)
      (Collision|SetCollisionEnabled _shieldmesh "QueryOnly")
      (Variables|Default|SetHealth (Variables|Default|GetHealthMax)))))