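; BP_Builder is a production structure that builds Mech or Vehicle units for its owner and raises that unit type's population cap.
; BeginPlay spawns a rally point and updates player or AI caps, registering tier-1 AI builders; destruction reverts only player caps.
; AddToQueue and CancelUnit adjust He3 and player population around a build queue.
; With authority, BuildActor spawns the head entry's Assault, Support or Command class, passing it the rally point.
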(event Custom|BuildActor
  (bind _returnvalue (Transformation|GetActorTransform))
  (bind _buildqueue (Variables|Default|GetBuildQueue))
  (bind _item (Utilities|Array|Get(acopy) _buildqueue))
  (bind (_location _rotation _scale) (Math|Transform|BreakTransform _returnvalue))
  (bind (_cost _mode) (Utilities|Struct|BreakBuildInfo _item))
  (if (and (Ability|HasAuthority) (Utilities|Enum|Equal(Enum) (Variables|Default|GetCurrentType) "NewEnumerator3"))
    (bind _output_get (Variables|Default|SetCurrentType _mode))
    (Variables|Default|SetCurrentCost _cost)
    (bind _returnvalue_2 (Game|SpawnActorfromClass (CallFunction|GetClass _output_get) (Math|Transform|MakeTransform (+ _location (Math|Vector|RotateVector (Variables|Default|GetSpawnOffset) (Transformation|GetActorRotation))) _rotation _scale) "AlwaysSpawn" (Components|GetOwner) self (stale EventBeginPlay _primaryowner) (Variables|Default|GetRallyPoint)))
    (Utilities|IsValid _returnvalue_2
      (:Is%20Valid
        (Variables|Default|SetCurrentBuild _returnvalue_2)))))

(event EventDestroyed
  (bind _population (Variables|Default|GetPopulation))
  (|CallParentFunction)
  (bind _currentbuild (Variables|Default|GetCurrentBuild)
    (:then
      (Actor|DestroyActor _currentbuild)
      (bind _rallypoint (Variables|Default|GetRallyPoint)
        (:then
          (Actor|DestroyActor _rallypoint))
        (:else
          _)))
    (:else
      _))
  (bind _primaryowner (Variables|Default|GetPrimaryOwner)
    (:then
      (bind _playercontroller (Variables|/Game/Blueprints/BP_PlayerPrimary.BP_PlayerPrimary_C|GetPlayerController _primaryowner)
        (:then
          (switch Utilities|FlowControl|Switch|SwitchonEN_BuilderType (Variables|Default|GetBuilderType)
            (:NewEnumerator0
              (Variables|/Game/Blueprints/BP_OpulentiumPlayerController.BP_OpulentiumPlayerController_C|SetMechCap _playercontroller (- (Variables|/Game/Blueprints/BP_OpulentiumPlayerController.BP_OpulentiumPlayerController_C|GetMechCap _playercontroller) _population)))
            (:NewEnumerator1
              (Variables|/Game/Blueprints/BP_OpulentiumPlayerController.BP_OpulentiumPlayerController_C|SetVehicleCap _playercontroller (- (Variables|/Game/Blueprints/BP_OpulentiumPlayerController.BP_OpulentiumPlayerController_C|GetVehicleCap _playercontroller) _population)))))
        (:else)))
    (:else)))

(event EventSetPopulation
  (bind _self self)
  (bind _buildertype (Variables|Default|GetBuilderType))
  (bind _population (Variables|Default|GetPopulation))
  (bind _tier (Variables|Default|GetTier))
  (bind _returnvalue (== _tier 1))
  (bind _primaryowner (Variables|Default|GetPrimaryOwner)
    (:then
      (bind _playercontroller (Variables|/Game/Blueprints/BP_PlayerPrimary.BP_PlayerPrimary_C|GetPlayerController _primaryowner)
        (:then
          (switch Utilities|FlowControl|Switch|SwitchonEN_BuilderType _buildertype
            (:NewEnumerator0
              (Variables|/Game/Blueprints/BP_OpulentiumPlayerController.BP_OpulentiumPlayerController_C|SetMechCap _playercontroller (+ (Variables|/Game/Blueprints/BP_OpulentiumPlayerController.BP_OpulentiumPlayerController_C|GetMechCap _playercontroller) _population)))
            (:NewEnumerator1
              (Variables|/Game/Blueprints/BP_OpulentiumPlayerController.BP_OpulentiumPlayerController_C|SetVehicleCap _playercontroller (+ (Variables|/Game/Blueprints/BP_OpulentiumPlayerController.BP_OpulentiumPlayerController_C|GetVehicleCap _playercontroller) _population)))))
        (:else
          (bind _ai (Variables|/Game/Blueprints/BP_PlayerPrimary.BP_PlayerPrimary_C|GetAI _primaryowner)
            (:then
              (switch Utilities|FlowControl|Switch|SwitchonEN_BuilderType _buildertype
                (:NewEnumerator0
                  (Variables|/Game/Blueprints/BP_OpulentiumAI.BP_OpulentiumAI_C|SetMechCap _ai (+ (Variables|/Game/Blueprints/BP_OpulentiumAI.BP_OpulentiumAI_C|GetMechCap _ai) _population))
                  (if _returnvalue
                    (Utilities|Array|Add (.T1Facs (Utilities|Struct|BreakStructureInventory (Variables|/Game/Blueprints/BP_OpulentiumAI.BP_OpulentiumAI_C|GetStructureInventory _ai))) _self)))
                (:NewEnumerator1
                  (Variables|/Game/Blueprints/BP_OpulentiumAI.BP_OpulentiumAI_C|SetVehicleCap _ai (+ (Variables|/Game/Blueprints/BP_OpulentiumAI.BP_OpulentiumAI_C|GetVehicleCap _ai) _population))
                  (if _returnvalue
                    (Utilities|Array|Add (.T1Beacons (Utilities|Struct|BreakStructureInventory (Variables|/Game/Blueprints/BP_OpulentiumAI.BP_OpulentiumAI_C|GetStructureInventory _ai))) _self)))))
            (:else)))))
    (:else)))

(event EventBeginPlay
  (|CallParentFunction)
  (bind _primaryowner (Variables|Default|GetPrimaryOwner)
    (:then
      (bind _returnvalue (Game|SpawnActorfromClass "/Game/Blueprints/BP_RallyPoint.BP_RallyPoint_C" (Math|Conversions|ToTransform(Vector) (+ (Math|Vector|RotateVector (Variables|Default|GetRallyLocation) (Transformation|GetActorRotation)) (Transformation|GetActorLocation))) "AdjustIfPossibleButAlwaysSpawn" _primaryowner self 0))
      (Utilities|IsValid _returnvalue
        (:Is%20Valid
          (Variables|Default|SetRallyPoint _returnvalue)
          (CallFunction|SetPopulation))))
    (:else)))

(fn ConstructionScript
  (|CallParentFunction))

(fn GetClass
  (params (Type :type EN_UnitType%20Enum))
  (switch Utilities|FlowControl|Switch|SwitchonEN_UnitType Type
    (:NewEnumerator0
      (LocalVariables|SetReturnClass (Variables|Default|GetAssaultClass)))
    (:NewEnumerator1
      (bind _output_get (LocalVariables|SetReturnClass (Variables|Default|GetSupportClass))))
    (:NewEnumerator2
      (LocalVariables|SetReturnClass (Variables|Default|GetCommandClass)))
    (:NewEnumerator3
      (LocalVariables|SetReturnClass 0)))
  (return _output_get))

(fn SetBuildQueue
  (params (Index :type Integer))
  (bind _buildqueue (Variables|Default|GetBuildQueue))
  (bind _returnvalue (Utilities|Array|Length _buildqueue))
  (if (> _returnvalue 0)
    (Utilities|Array|RemoveIndex _buildqueue Index)
    (if (== Index 0)
      (bind _currentbuild (Variables|Default|GetCurrentBuild)
        (:then
          (Variables|/Game/Blueprints/BP_UnitBuild.BP_UnitBuild_C|SetbCancel _currentbuild true)
          (Actor|DestroyActor _currentbuild))
        (:else
          _))
      (if (> _returnvalue 0)
        (Variables|Default|SetCurrentType "NewEnumerator3")
        (CallFunction|BuildActor)
        (else
          (Variables|Default|SetCurrentType "NewEnumerator3"))))))

(fn CancelUnit
  (params (Index :type Integer))
  (bind _buildqueue (Variables|Default|GetBuildQueue))
  (bind _item (Utilities|Array|Get(acopy) _buildqueue Index))
  (bind (_cost _population) (Utilities|Struct|BreakBuildInfo _item))
  (bind _primaryowner (Variables|Default|GetPrimaryOwner)
    (:then
      (Default|ServerGainHe3 _primaryowner _cost)
      (bind _playercontroller (Variables|/Game/Blueprints/BP_PlayerPrimary.BP_PlayerPrimary_C|GetPlayerController _primaryowner)
        (:then
          (switch Utilities|FlowControl|Switch|SwitchonEN_BuilderType (Variables|Default|GetBuilderType)
            (:NewEnumerator0
              (Variables|/Game/Blueprints/BP_OpulentiumPlayerController.BP_OpulentiumPlayerController_C|SetMechPop _playercontroller (- (Variables|/Game/Blueprints/BP_OpulentiumPlayerController.BP_OpulentiumPlayerController_C|GetMechPop _playercontroller) _population)))
            (:NewEnumerator1
              (Variables|/Game/Blueprints/BP_OpulentiumPlayerController.BP_OpulentiumPlayerController_C|SetVehiclePop _playercontroller (- (Variables|/Game/Blueprints/BP_OpulentiumPlayerController.BP_OpulentiumPlayerController_C|GetVehiclePop _playercontroller) _population)))))
        (:else
          _)))
    (:else
      _))
  (CallFunction|SetBuildQueue Index))

(fn AddtoQueue
  (params (BuildInfo :type Build%20Info%20Structure))
  (bind (_cost _population) (Utilities|Struct|BreakBuildInfo BuildInfo))
  (bind _primaryowner (Variables|Default|GetPrimaryOwner)
    (:then
      (Default|ServerSpendHe3 _primaryowner _cost)
      (bind _playercontroller (Variables|/Game/Blueprints/BP_PlayerPrimary.BP_PlayerPrimary_C|GetPlayerController _primaryowner)
        (:then
          (switch Utilities|FlowControl|Switch|SwitchonEN_BuilderType (Variables|Default|GetBuilderType)
            (:NewEnumerator0
              (Variables|/Game/Blueprints/BP_OpulentiumPlayerController.BP_OpulentiumPlayerController_C|SetMechPop _playercontroller (+ (Variables|/Game/Blueprints/BP_OpulentiumPlayerController.BP_OpulentiumPlayerController_C|GetMechPop _playercontroller) _population)))
            (:NewEnumerator1
              (Variables|/Game/Blueprints/BP_OpulentiumPlayerController.BP_OpulentiumPlayerController_C|SetVehiclePop _playercontroller (+ _population (Variables|/Game/Blueprints/BP_OpulentiumPlayerController.BP_OpulentiumPlayerController_C|GetVehiclePop _playercontroller)))))
          (bind _returnvalue (Utilities|Array|Add (Variables|Default|GetBuildQueue) BuildInfo))
          (if (== _returnvalue 0)
            (CallFunction|BuildActor)))
        (:else)))
    (:else)))