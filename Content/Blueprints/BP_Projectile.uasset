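; Projectile actor that damages enemy-team BP_OpulentiumActors on impact and spawns a hit effect actor before destroying itself.
; Server-side capsule overlaps and per-tick line traces from the previous location share one hit path, filtering out owners and a brief post-spawn invulnerability.
; On destruction, a nonzero Radius triggers a sphere trace applying distance-falloff damage to enemy pawns.
; Replicated HitActor fractures struck BP_Destructibles through its OnRep.
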(event OnComponentBeginOverlap(Capsule)
  (params (OtherActor :type Actor%20Object%20Reference) (OtherComp :type Primitive%20Component%20Object%20Reference) (OtherBodyIndex :type Integer) (bFromSweep :type Boolean) (SweepResult :type Hit%20Result%20Structure%20%28by%20ref%29))
  (Networking|SwitchHasAuthority
    (:Authority
      (Utilities|IsValid OtherActor
        (:Is%20Valid
          (bind _output_get (Variables|Default|SetHitActor OtherActor))
          (if (and (CallFunction|NotOwners _output_get) (not (Variables|Default|GetbInvulnerable)))
            (bind _asbp_opulentium_actor (Utilities|Casting|CastToBP_OpulentiumActor OtherActor)
              (:then
                (if (!= (Variables|/Game/Blueprints/BP_OpulentiumActor.BP_OpulentiumActor_C|GetTeam _asbp_opulentium_actor) (Variables|Default|GetTeam))
                  (Default|TakeDamage _asbp_opulentium_actor (stale EventBeginPlay _output_get))))
              (:CastFailed
                _))
            (Game|SpawnActorfromClass (Variables|Default|GetHitClass) (Transformation|GetActorTransform) "AlwaysSpawn" 0 0)
            (Actor|DestroyActor)))))))

(event EventDestroyed
  (bind _returnvalue (Transformation|GetActorLocation))
  (bind _radius (Variables|Default|GetRadius))
  (bind _trackactor (Variables|Default|GetTrackActor)
    (:then
      (Actor|DestroyActor _trackactor))
    (:else
      _))
  (if (!= _radius 0.0)
    (bind _outhits (Collision|MultiSphereTraceForObjects _returnvalue (+ _returnvalue "0, 0,4.000000") _radius (Utilities|Array|MakeArray "ObjectTypeQuery3") false 0 "None"))
    (for _array_element _outhits
      (if (and (Utilities|IsValid (.HitActor (Collision|BreakHitResult _array_element))) (not (Utilities|Array|ContainsItem (Variables|Default|GetExplodedActors) (.HitActor (Collision|BreakHitResult _array_element)))))
        (bind _asbp_opulentium_actor (Utilities|Casting|CastToBP_OpulentiumActor (.HitActor (Collision|BreakHitResult _array_element))))
        (if (!= (Variables|/Game/Blueprints/BP_OpulentiumActor.BP_OpulentiumActor_C|GetTeam _asbp_opulentium_actor) (Variables|Default|GetTeam))
          (Default|TakeDamage _asbp_opulentium_actor (Math|Float|Truncate (* (Variables|Default|GetDamageMax) (- 1.0 (/ (Transformation|GetDistanceTo (.HitActor (Collision|BreakHitResult _array_element)) self) (Variables|Default|GetRadius)))))))
        (Utilities|Array|Add (Variables|Default|GetExplodedActors) (.HitActor (Collision|BreakHitResult _array_element)))))))

(event EventBeginPlay
  (bind _output_get (Variables|Default|SetDamageMax (Variables|Default|GetDamage)))
  (Audio|Components|Audio|Play (Variables|Default|GetFireSound) 0.1)
  (bind _output_get_2 (Variables|Default|SetPrevLoc (Transformation|GetActorLocation)))
  (Utilities|FlowControl|Delay 0.05)
  (Variables|Default|SetbInvulnerable false))

(event EventTick
  (params (DeltaSeconds :type Float%20%28single-precision%29))
  (bind _returnvalue (Transformation|GetActorLocation))
  (Networking|SwitchHasAuthority
    (:Authority
      (bind (_outhit _returnvalue_2) (Collision|LineTraceByChannel (stale EventBeginPlay _output_get_2) _returnvalue "TraceTypeQuery1" false (CallFunction|IgnoreActors) "None"))
      (Variables|Default|SetPrevLoc _returnvalue)
      (if _returnvalue_2
        (Utilities|IsValid (.HitActor (Collision|BreakHitResult _outhit))
          (:Is%20Valid
            (Variables|Default|SetHitActor (.HitActor (Collision|BreakHitResult _outhit)))
            (if (and (CallFunction|NotOwners (stale OnComponentBeginOverlap(Capsule) _output_get)) (not (Variables|Default|GetbInvulnerable)))
              (bind _asbp_opulentium_actor (Utilities|Casting|CastToBP_OpulentiumActor (stale OnComponentBeginOverlap(Capsule) OtherActor))
                (:then
                  (if (!= (Variables|/Game/Blueprints/BP_OpulentiumActor.BP_OpulentiumActor_C|GetTeam _asbp_opulentium_actor) (Variables|Default|GetTeam))
                    (Default|TakeDamage _asbp_opulentium_actor (stale EventBeginPlay _output_get))))
                (:CastFailed
                  _))
              (Game|SpawnActorfromClass (Variables|Default|GetHitClass) (Transformation|GetActorTransform) "AlwaysSpawn" 0 0)
              (Actor|DestroyActor))))))))

(fn ConstructionScript)

(fn IgnoreActors
  (bind _returnactors (LocalVariables|GetReturnActors))
  (bind _outactors (Actor|GetAllActorsOfClass "/Game/Environment/Objects/TerritoryVolume/BP_TerritoryVolume.BP_TerritoryVolume_C"))
  (bind _outactors_2 (Actor|GetAllActorsOfClass "/Game/Blueprints/BP_Placement.BP_Placement_C"))
  (Utilities|Array|AppendArray _returnactors _outactors)
  (Utilities|Array|AppendArray _returnactors _outactors_2)
  (Utilities|Array|Add _returnactors (Components|GetOwner))
  (return _returnactors))

(fn NotOwners
  (params (Actor :type Actor%20Object%20Reference))
  (bind _returnvalue (Components|GetOwner))
  (Utilities|IsValid Actor
    (:Is%20Valid
      (if (== Actor _returnvalue)
        _
        (else
          (bind _asbp_weapon (Utilities|Casting|CastToBP_Weapon _returnvalue)
            (:then
              (bind _combatowner (Variables|/Game/Blueprints/BP_Weapon.BP_Weapon_C|GetCombatOwner _asbp_weapon)
                (:then
                  (if (== _combatowner Actor)
                    _
                    (else
                      (return true))))
                (:else
                  (return true))))
            (:CastFailed
              (return true))))))
    (:Is%20Not%20Valid
      _))
  (return false))

(fn Fracture
  (params (Destructible :type BP%20Destructible%20Object%20Reference))
  (Utilities|IsValid Destructible
    (:Is%20Valid
      (Game|Damage|ApplyDamage (Variables|/Game/Blueprints/BP_Destructible.BP_Destructible_C|GetDestructible Destructible) 1.0 (Transformation|GetActorLocation) (Transformation|GetVelocity) (* (Variables|Default|GetDamage) 1e+02)))))

(fn OnRepHitActor
  (bind _hitactor (Variables|Default|GetHitActor)
    (:then
      (bind _asbp_destructible (Utilities|Casting|CastToBP_Destructible _hitactor))
      (CallFunction|Fracture _asbp_destructible))
    (:else)))