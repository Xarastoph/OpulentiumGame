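; BP_WaveSpawn is a wave spawn point that creates team-tagged enemy pawns on the server when SpawnWave fires.
; After a delay, it spawns WaveIntensity instances of SpawnClass at random horizontal offsets around itself.
; Each pawn ends up possessed by a wave-flagged BP_SecurityBot controller, replacing any other controller.
; It increments BP_WaveBoss's WaveTotal per spawn, then clears its FirstWave flag and advances its own WaveNumber.
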(event EventSpawnWave
  (bind _returnvalue (Math|Random|RandomUnitVector))
  (bind _waveintensity (Variables|Default|GetWaveIntensity))
  (bind (_x _y) (Math|Vector|BreakVector _returnvalue))
  (Networking|SwitchHasAuthority
    (:Authority
      (if (> _waveintensity 0)
        (Utilities|FlowControl|Delay 1e+01)
        (for _index (range 1 _waveintensity)
          (bind _returnvalue_2 (Game|SpawnActorfromClass (Variables|Default|GetSpawnClass) (Math|Conversions|ToTransform(Vector) (+ (Transformation|GetActorLocation) (* (Math|Vector|MakeVector _x _y 0.0) 256.0))) "AdjustIfPossibleButAlwaysSpawn" 0 0))
          (Variables|/Game/Blueprints/BP_OpulentiumActor.BP_OpulentiumActor_C|SetTeam _returnvalue_2 256)
          (Utilities|IsValid (Pawn|GetController _returnvalue_2)
            (:Is%20Valid
              (bind _asbp_security_bot (Utilities|Casting|CastToBP_SecurityBot (Pawn|GetController _returnvalue_2))
                (:then
                  (Variables|/Game/Factions/Security/Bot/BP_SecurityBot.BP_SecurityBot_C|SetbWave _asbp_security_bot true))
                (:CastFailed
                  (Actor|DestroyActor (Pawn|GetController _returnvalue_2))
                  (bind _returnvalue_3 (Game|SpawnActorfromClass "/Game/Factions/Security/Bot/BP_SecurityBot.BP_SecurityBot_C" (Transformation|GetActorTransform _returnvalue_2) "AlwaysSpawn" 0 0 :!label _label))
                  (Variables|/Game/Factions/Security/Bot/BP_SecurityBot.BP_SecurityBot_C|SetbWave _returnvalue_3 true)
                  (Pawn|Possess _returnvalue_3 _returnvalue_2))))
            (:Is%20Not%20Valid
              (goto _label)))
          (bind _outactors (Actor|GetAllActorsOfClass "/Game/Blueprints/BP_WaveBoss.BP_WaveBoss_C"))
          (Math|Integer|IncrementInt (Variables|/Game/Blueprints/BP_WaveBoss.BP_WaveBoss_C|GetWaveTotal (Utilities|Array|Get(acopy) _outactors))))
        (bind _outactors_2 (Actor|GetAllActorsOfClass "/Game/Blueprints/BP_WaveBoss.BP_WaveBoss_C"))
        (Variables|/Game/Blueprints/BP_WaveBoss.BP_WaveBoss_C|SetbFirstWave (Utilities|Array|Get(acopy) _outactors_2) false)
        (Math|Integer|IncrementInt (Variables|Default|GetWaveNumber))))))

(fn ConstructionScript)