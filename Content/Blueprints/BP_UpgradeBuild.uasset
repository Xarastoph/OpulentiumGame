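; Timed construction placeholder for a structure upgrade, showing progress through a dynamic material and the owning player's upgrade menu.
; Tick accumulates time until BuildTime, when the authority spawns UpgradeClass, registers it on a parent BP_Conduit and destroys this actor.
; Cancelling refunds He3 up to the cap and removes the icon height offset.
; Client success and cancel events update the upgrade tree node and hide progress text on remotes.
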(event Custom|Server_SetCancel
  (Variables|Default|SetbCancel true))

(event Custom|Client_Cancel
  (Networking|SwitchHasAuthority
    (:Remote
      (bind _parentstructure (Variables|Default|GetParentStructure)
        (:then
          (Variables|/Game/Blueprints/BP_OpulentiumActor.BP_OpulentiumActor_C|SetIconOffset _parentstructure (- (Variables|Default|GetHeight) (Variables|/Game/Blueprints/BP_OpulentiumActor.BP_OpulentiumActor_C|GetIconOffset _parentstructure)))
          (bind _primaryowner (Variables|Default|GetPrimaryOwner)
            (:then
              (bind _upgrademenu (Variables|/Game/Blueprints/BP_PlayerPrimary.BP_PlayerPrimary_C|GetUpgradeMenu _primaryowner)
                (:then
                  (if (== (Variables|/Game/Blueprints/Widget/BP_UpgradeMenu.BP_UpgradeMenu_C|GetStructure _upgrademenu) (Variables|Default|GetParentStructure))
                    (Widget|SetVisibility (Variables|/Game/Blueprints/Widget/BP_UpgradeMenu.BP_UpgradeMenu_C|GetProgressText _upgrademenu) "Hidden")))
                (:else
                  _))
              (Variables|Default|SetbCancel true)
              (CallFunction|SetNodeDone))
            (:else)))
        (:else)))))

(event Custom|Client_Success
  (Networking|SwitchHasAuthority
    (:Remote
      (Variables|Default|SetbCancel false)
      (bind _primaryowner (Variables|Default|GetPrimaryOwner)
        (:then
          (bind _upgrademenu (Variables|/Game/Blueprints/BP_PlayerPrimary.BP_PlayerPrimary_C|GetUpgradeMenu _primaryowner)
            (:then
              (if (== (Variables|/Game/Blueprints/Widget/BP_UpgradeMenu.BP_UpgradeMenu_C|GetStructure _upgrademenu) (Variables|Default|GetParentStructure))
                (Widget|SetVisibility (Variables|/Game/Blueprints/Widget/BP_UpgradeMenu.BP_UpgradeMenu_C|GetProgressText _upgrademenu) "Hidden")))
            (:else
              _))
          (CallFunction|SetNodeDone))
        (:else)))))

(event EventBeginPlay
  (bind _returnvalue (Rendering|Material|CreateDynamicMaterialInstance (Variables|Default|GetStaticMesh) 0 "/Game/Environment/Materials/Static/GreenStaticPanner_Inst.GreenStaticPanner_Inst" :!class /Script/Engine.PrimitiveComponent))
  (bind _asbp_opulentium_player_controller (Utilities|Casting|CastToBP_OpulentiumPlayerController (Components|GetOwner)))
  (bind _output_get (Variables|Default|SetPrimaryOwner (Variables|/Game/Blueprints/BP_OpulentiumPlayerController.BP_OpulentiumPlayerController_C|GetPrimaryOwner _asbp_opulentium_player_controller)))
  (Utilities|FlowControl|Delay 0.05)
  (bind _parentstructure (Variables|Default|GetParentStructure)
    (:then
      (Variables|/Game/Blueprints/BP_OpulentiumActor.BP_OpulentiumActor_C|SetIconOffset _parentstructure (+ (Variables|Default|GetHeight) (Variables|/Game/Blueprints/BP_OpulentiumActor.BP_OpulentiumActor_C|GetIconOffset _parentstructure))))
    (:else)))

(event EventTick
  (params (DeltaSeconds :type Float%20%28single-precision%29))
  (bind _output_get (Variables|Default|SetDTime (+ DeltaSeconds (Variables|Default|GetDTime))))
  (if (< (/ _output_get (Variables|Default|GetBuildTime)) 1.0)
    (if (Variables|Default|GetbCancel)
      (CallFunction|Refund)
      (bind _parentstructure (Variables|Default|GetParentStructure)
        (:then
          (Variables|/Game/Blueprints/BP_OpulentiumActor.BP_OpulentiumActor_C|SetIconOffset _parentstructure (- (Variables|/Game/Blueprints/BP_OpulentiumActor.BP_OpulentiumActor_C|GetIconOffset _parentstructure) (Variables|Default|GetHeight)))
          (CallFunction|ClientCancel))
        (:else
          _))
      (bind _upgrademenu (Variables|/Game/Blueprints/BP_PlayerPrimary.BP_PlayerPrimary_C|GetUpgradeMenu (stale EventBeginPlay _output_get) :!label _label)
        (:then
          (if (== (Variables|/Game/Blueprints/Widget/BP_UpgradeMenu.BP_UpgradeMenu_C|GetStructure _upgrademenu) (Variables|Default|GetParentStructure))
            (Widget|SetVisibility (Variables|/Game/Blueprints/Widget/BP_UpgradeMenu.BP_UpgradeMenu_C|GetProgressText _upgrademenu) "Hidden")))
        (:else
          _))
      (CallFunction|SetNodeDone)
      (if (Variables|Default|GetbCancel)
        _
        (else
          (CallFunction|ClientSuccess)))
      (Actor|DestroyActor)
      (else
        (Rendering|Material|SetScalarParameterValue (stale EventBeginPlay _returnvalue) "Time" (/ _output_get (Variables|Default|GetBuildTime)) :!class /Script/Engine.MaterialInstanceDynamic)
        (bind _primaryowner (Variables|Default|GetPrimaryOwner)
          (:then
            (bind _upgrademenu_2 (Variables|/Game/Blueprints/BP_PlayerPrimary.BP_PlayerPrimary_C|GetUpgradeMenu _primaryowner)
              (:then
                (if (== (Variables|/Game/Blueprints/Widget/BP_UpgradeMenu.BP_UpgradeMenu_C|GetStructure _upgrademenu_2) (Variables|Default|GetParentStructure))
                  (Variables|/Game/Blueprints/BP_PlayerPrimary.BP_PlayerPrimary_C|SetUpgradeProgress _primaryowner (/ _output_get (Variables|Default|GetBuildTime)))))
              (:else)))
          (:else))))
    (else
      (Networking|SwitchHasAuthority
        (:Authority
          (bind _returnvalue (Game|SpawnActorfromClass (Variables|Default|GetUpgradeClass) (Transformation|GetActorTransform) "AlwaysSpawn" (Components|GetOwner) 0))
          (Variables|/Game/Blueprints/BP_StructureUpgrade.BP_StructureUpgrade_C|SetParentStructure _returnvalue (Variables|Default|GetParentStructure))
          (CallFunction|SetUpgrade _returnvalue)
          (Variables|/Game/Blueprints/BP_StructureUpgrade.BP_StructureUpgrade_C|SetTeam _returnvalue (Variables|Default|GetTeam))
          (goto _label))))))

(fn ConstructionScript)

(fn Refund
  (bind _buildcost (Variables|Default|GetBuildCost))
  (bind _primaryowner (Variables|Default|GetPrimaryOwner)
    (:then
      (bind _playercontroller (Variables|/Game/Blueprints/BP_PlayerPrimary.BP_PlayerPrimary_C|GetPlayerController _primaryowner)
        (:then
          (if (< (Variables|/Game/Blueprints/BP_OpulentiumPlayerController.BP_OpulentiumPlayerController_C|GetHe3 _playercontroller) (Variables|/Game/Blueprints/BP_OpulentiumPlayerController.BP_OpulentiumPlayerController_C|GetHe3Cap _playercontroller))
            (if (<= (+ (Variables|/Game/Blueprints/BP_OpulentiumPlayerController.BP_OpulentiumPlayerController_C|GetHe3 _playercontroller) _buildcost) (Variables|/Game/Blueprints/BP_OpulentiumPlayerController.BP_OpulentiumPlayerController_C|GetHe3Cap _playercontroller))
              (Default|ServerGainHe3 _primaryowner _buildcost)
              (else
                (Default|ServerGainHe3 _primaryowner (- (Variables|/Game/Blueprints/BP_OpulentiumPlayerController.BP_OpulentiumPlayerController_C|GetHe3Cap _playercontroller) (Variables|/Game/Blueprints/BP_OpulentiumPlayerController.BP_OpulentiumPlayerController_C|GetHe3 _playercontroller)))))))
        (:else)))
    (:else)))

(fn SetUpgrade
  (params (Upgrade :type BP%20Structure%20Upgrade%20Object%20Reference))
  (bind _parentstructure (Variables|Default|GetParentStructure)
    (:then
      (bind _asbp_conduit (Utilities|Casting|CastToBP_Conduit _parentstructure))
      (Variables|/Game/Blueprints/BP_Conduit.BP_Conduit_C|SetCurrentUpgrade _asbp_conduit Upgrade))
    (:else)))

(fn SetNodeDone
  (bind _primaryowner (Variables|Default|GetPrimaryOwner)
    (:then
      (bind _upgrademenu (Variables|/Game/Blueprints/BP_PlayerPrimary.BP_PlayerPrimary_C|GetUpgradeMenu _primaryowner)
        (:then
          (bind _currenttree (Variables|/Game/Blueprints/Widget/BP_UpgradeMenu.BP_UpgradeMenu_C|GetCurrentTree _upgrademenu)
            (:then
              (bind _array_element (Utilities|Array|ForEachLoopwithBreak (Variables|/Game/Blueprints/Widget/BP_UpgradeTree.BP_UpgradeTree_C|GetNodes _currenttree) :!label _label)
                (:LoopBody
                  (if (== (Variables|/Game/Blueprints/Widget/BP_UpgradeNode.BP_UpgradeNode_C|GetUpgradeClass _array_element) (Variables|Default|GetUpgradeClass))
                    (Variables|/Game/Blueprints/Widget/BP_UpgradeNode.BP_UpgradeNode_C|SetbDone _array_element (not (Variables|Default|GetbCancel)))
                    (Variables|/Game/Blueprints/Widget/BP_UpgradeNode.BP_UpgradeNode_C|SetbInProgress _array_element false)
                    (goto _label Break)))
                (:Completed
                  (Default|UpdateTree _currenttree)
                  (Variables|/Game/Blueprints/BP_PlayerPrimary.BP_PlayerPrimary_C|SetUpgradeProgress _primaryowner 0.0))))
            (:else)))
        (:else)))
    (:else)))