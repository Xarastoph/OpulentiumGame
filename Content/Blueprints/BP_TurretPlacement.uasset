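; Turret placement actor that follows the owning player's aim while locating and flags whether the spot is valid.
; Each tick it moves to the vision trace point plus a relative offset, snaps to the surface and, for nonzero offsets, orients along that offset.
; A sphere trace clears CanPlace on hitting pawns or vehicles other than placement actors.
; On destruction it releases itself as the TurretMech's current placement.
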(event EventTick
  (params (DeltaSeconds :type Float%20%28single-precision%29))
  (bind _relative (Variables|Default|GetRelative))
  ;[1 1 1] Set Location
  (if (Variables|Default|GetbLocating)
    (bind _asbp_player_primary (Utilities|Casting|CastToBP_PlayerPrimary (Components|GetOwner)))
    (Transformation|SetActorLocation (+ (.Location (Collision|BreakHitResult (Default|VisionTrace _asbp_player_primary))) (Variables|Default|GetRelative)) false false)
    (bind (_outloc _outrot) (CallFunction|SurfaceSnap 512.0))
    (Transformation|SetActorLocation _outloc false false)
    (if (not (Math|Vector|Equal(Vector) _relative "0, 0, 0" 0.0001))
      (Transformation|SetActorRotation (Math|Rotator|CombineRotators _outrot (Math|Rotator|MakeRotfromX _relative))))
    ;[1 1 1] Set Can Place
    (bind (_outhits _returnvalue) (Collision|MultiSphereTraceForObjects (+ (.Location (Collision|BreakHitResult (Default|VisionTrace _asbp_player_primary))) (Variables|Default|GetRelative)) (+ (+ (.Location (Collision|BreakHitResult (Default|VisionTrace _asbp_player_primary))) (Variables|Default|GetRelative)) "0, 0,4.000000") 128.0 (Utilities|Array|MakeArray "ObjectTypeQuery3" "ObjectTypeQuery5") false 0 "None"))
    (Variables|Default|SetbCanPlace true)
    (if _returnvalue
      (for _array_element _outhits
        (if (not (or (== (Utilities|GetClass (.HitActor (Collision|BreakHitResult _array_element))) "/Game/Blueprints/BP_Placement.BP_Placement_C") (Utilities|ClassIsChildOf (Utilities|GetClass (.HitActor (Collision|BreakHitResult _array_element))) "/Game/Blueprints/BP_Placement.BP_Placement_C")))
          (Variables|Default|SetbCanPlace false))))))

(event EventDestroyed
  ;[1 1 1] Destroyed
  (bind _turretmech (Variables|Default|GetTurretMech)
    (:then
      (bind _currentplacement (Variables|/Game/Blueprints/BP_Mech.BP_Mech_C|GetCurrentPlacement _turretmech)
        (:then
          (if (== _currentplacement self)
            (Variables|/Game/Blueprints/BP_Mech.BP_Mech_C|SetCurrentPlacement _turretmech 0)))
        (:else)))
    (:else)))

(fn ConstructionScript
  (|CallParentFunction))