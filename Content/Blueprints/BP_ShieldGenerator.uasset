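; BP_ShieldGenerator is an actor that creates and owns the lifetime of a team shield barrier.
; On BeginPlay, only the authority spawns a BP_ShieldBarrier at the generator's transform, passes it the generator's Team and stores it as Shield.
; When the generator is destroyed, it destroys that barrier if it is still valid.
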(event EventBeginPlay
  (|CallParentFunction)
  (Networking|SwitchHasAuthority
    (:Authority
      (bind _returnvalue (Game|SpawnActorfromClass "/Game/Blueprints/BP_ShieldBarrier.BP_ShieldBarrier_C" (Transformation|GetActorTransform) "AlwaysSpawn" (Components|GetOwner) 0))
      (Variables|/Game/Blueprints/BP_ShieldBarrier.BP_ShieldBarrier_C|SetTeam _returnvalue (Variables|Default|GetTeam))
      (Variables|Default|SetShield _returnvalue))))

(event EventDestroyed
  (|CallParentFunction)
  (bind _shield (Variables|Default|GetShield)
    (:then
      (Actor|DestroyActor _shield))
    (:else)))

(fn ConstructionScript
  (|CallParentFunction))