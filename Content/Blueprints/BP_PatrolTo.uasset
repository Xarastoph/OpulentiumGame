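; BP_PatrolTo is a player-owned patrol waypoint marker showing a camera-facing order number.
; Tick snaps it to the player's surface trace while locating and, through a gate, stretches and aims a Branch link to the next waypoint.
; RepNotifies update the number, visibility with trace collision, and selection brightness on dynamic materials, with selection also opening the gate.
; MechTest destroys the whole containing route once the marker has no mechs.
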(event Custom|ToggleGate
  (params (bOpen :type Boolean))
  (bind _self self)
  (bind _branch (Variables|Default|GetBranch))
  (if bOpen
    (Utilities|FlowControl|Gate false) ; enters at Open
    (else
      (Utilities|FlowControl|Gate false) ; enters at Close
    )))

(event EventBeginPlay
  (bind _skeletalmesh (Variables|Default|GetSkeletalMesh))
  (bind _materials (Variables|Default|GetMaterials))
  (bind _returnvalue (Rendering|Material|CreateDynamicMaterialInstance _skeletalmesh 6 "/Game/Environment/Objects/PatrolTo/Materials/PatrolTo_L1Mat_Inst.PatrolTo_L1Mat_Inst" :!class /Script/Engine.PrimitiveComponent))
  (bind _returnvalue_2 (Rendering|Material|CreateDynamicMaterialInstance _skeletalmesh 7 "/Game/Environment/Objects/PatrolTo/Materials/PatrolTo_L2Mat_Inst.PatrolTo_L2Mat_Inst" :!class /Script/Engine.PrimitiveComponent))
  (bind _returnvalue_3 (Rendering|Material|CreateDynamicMaterialInstance _skeletalmesh 8 "/Game/Environment/Objects/PatrolTo/Materials/PatrolTo_L3Mat_Inst.PatrolTo_L3Mat_Inst" :!class /Script/Engine.PrimitiveComponent))
  (bind _returnvalue_4 (Rendering|Material|CreateDynamicMaterialInstance _skeletalmesh 9 "/Game/Environment/Objects/PatrolTo/Materials/PatrolTo_L4Mat_Inst.PatrolTo_L4Mat_Inst" :!class /Script/Engine.PrimitiveComponent))
  (bind _returnvalue_5 (Rendering|Material|CreateDynamicMaterialInstance _skeletalmesh 10 "/Game/Environment/Objects/PatrolTo/Materials/PatrolTo_L5Mat_Inst.PatrolTo_L5Mat_Inst" :!class /Script/Engine.PrimitiveComponent))
  (bind _returnvalue_6 (Rendering|Material|CreateDynamicMaterialInstance _skeletalmesh 11 "/Game/Environment/Objects/PatrolTo/Materials/PatrolTo_L6Mat_Inst.PatrolTo_L6Mat_Inst" :!class /Script/Engine.PrimitiveComponent))
  (bind _returnvalue_7 (Rendering|Material|CreateDynamicMaterialInstance _skeletalmesh 12 "/Game/Environment/Objects/PatrolTo/Materials/PatrolTo_ConeMat_Inst.PatrolTo_ConeMat_Inst" :!class /Script/Engine.PrimitiveComponent))
  (bind _returnvalue_8 (Rendering|Material|CreateDynamicMaterialInstance _skeletalmesh 13 "/Game/Environment/Objects/PatrolTo/Materials/PatrolTo_LimbMat_Inst.PatrolTo_LimbMat_Inst" :!class /Script/Engine.PrimitiveComponent))
  (Utilities|Array|Add _materials _returnvalue)
  (Utilities|Array|Add _materials _returnvalue_2)
  (Utilities|Array|Add _materials _returnvalue_3)
  (Utilities|Array|Add _materials _returnvalue_4)
  (Utilities|Array|Add _materials _returnvalue_5)
  (Utilities|Array|Add _materials _returnvalue_6)
  (Utilities|Array|Add _materials _returnvalue_7)
  (Utilities|Array|Add _materials _returnvalue_8)
  (bind _asbp_player_primary (Utilities|Casting|CastToBP_PlayerPrimary (Components|GetOwner)))
  (Variables|Default|SetPrimaryOwner _asbp_player_primary)
  (Rendering|Components|TextRender|SetText (Variables|Default|GetOrderNum) (Utilities|Text|ToText(Integer) (Variables|Default|GetOrder)))
  (Variables|Default|SetbSelected true))

(event EventTick
  (params (DeltaSeconds :type Float%20%28single-precision%29))
  (bind _self self)
  (bind _ordernum (Variables|Default|GetOrderNum))
  (bind _branch (Variables|Default|GetBranch))
  (bind _primaryowner (Variables|Default|GetPrimaryOwner)
    (:then
      (Transformation|SetWorldRotation _ordernum (Math|Rotator|FindLookatRotation (Transformation|GetWorldLocation _ordernum) (Transformation|GetWorldLocation (Variables|/Game/Blueprints/BP_PlayerPrimary.BP_PlayerPrimary_C|GetCamera _primaryowner))) false false)
      (if (Variables|Default|GetbLocating)
        (Transformation|SetActorLocation (.HitLocation (Default|SurfaceTrace _primaryowner)) false false))
      (Utilities|FlowControl|Gate false
        (:Exit
          (bind _nextpatrol (Variables|Default|GetNextPatrol)
            (:then
              (Development|SetHiddeninGame _branch false false)
              (SplineMesh|SetEndPosition _branch (Math|Vector|MakeVector (Transformation|GetDistanceTo _nextpatrol _self) 0.0 0.0))
              (SplineMesh|SetEndTangent _branch (Math|Vector|MakeVector (Transformation|GetDistanceTo _nextpatrol _self) 0.0 0.0) :!class /Script/Engine.SplineMeshComponent)
              (SplineMesh|SetStartTangent _branch (Math|Vector|MakeVector (Transformation|GetDistanceTo _nextpatrol _self) 0.0 0.0) :!class /Script/Engine.SplineMeshComponent)
              (Transformation|SetWorldRotation _branch (Math|Rotator|FindLookatRotation (Transformation|GetActorLocation _self) (Transformation|GetActorLocation _nextpatrol)) false false))
            (:else
              (Development|SetHiddeninGame _branch true false)
              (CallFunction|ToggleGate (Variables|Default|GetbLocating)))))))
    (:else)))

(fn ConstructionScript)

(fn OnRepBSelected
  (bind _bselected (Variables|Default|GetbSelected))
  (for _array_element (Variables|Default|GetMaterials)
    (Rendering|Material|SetScalarParameterValue _array_element "Brightness" (+ (* (Math|Conversions|ToFloat(Boolean) _bselected) 2.0) 1.0) :!class /Script/Engine.MaterialInstanceDynamic)
    (if _bselected
      (CallFunction|ToggleGate true))))

(fn OnRepBShow
  (bind _tracecomp (Variables|Default|GetTraceComp))
  (bind _bshow (Variables|Default|GetbShow))
  (Rendering|SetActorHiddenInGame (not _bshow))
  (if _bshow
    (Collision|SetCollisionEnabled _tracecomp "QueryOnly")
    (else
      (Collision|SetCollisionEnabled _tracecomp "NoCollision"))))

(fn OnRepOrder
  (Rendering|Components|TextRender|SetText (Variables|Default|GetOrderNum) (Utilities|Text|ToText(Integer) (Variables|Default|GetOrder))))

(fn MechTest
  (bind _self self)
  (if (not (> (Utilities|Array|Length (Variables|Default|GetMechs)) 0))
    (bind _primaryowner (Variables|Default|GetPrimaryOwner)
      (:then
        (bind (_array_element _array_index) (Utilities|Array|ForEachLoopwithBreak (Variables|/Game/Blueprints/BP_PlayerPrimary.BP_PlayerPrimary_C|GetPatrolRoutes _primaryowner) :!label _label)
          (:LoopBody
            (if (Utilities|Array|ContainsItem (Utilities|Struct|BreakPatrollnfo _array_element) _self)
              (for _array_element_2 (Utilities|Struct|BreakPatrollnfo _array_element)
                (if (and (!= _array_element_2 _self) (Utilities|IsValid _array_element_2))
                  (Actor|DestroyActor _array_element_2)))
              (Utilities|Array|RemoveIndex (Variables|/Game/Blueprints/BP_PlayerPrimary.BP_PlayerPrimary_C|GetPatrolRoutes _primaryowner) _array_index)
              (goto _label Break)))
          (:Completed
            (Actor|DestroyActor))))
      (:else))))