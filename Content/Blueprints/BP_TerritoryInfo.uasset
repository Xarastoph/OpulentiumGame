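; BP_TerritoryInfo is an info object that registers itself with a Territory and a Primary when play begins.
; If each reference is valid, it adds itself to that object's info array and stores the returned index.
; A replicated CommandCentre reference updates a HasCommandCentre flag through its OnRep function, based on whether the reference is valid.
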(event EventBeginPlay
  (bind _self self)
  (bind _territory (Variables|Default|GetTerritory)
    (:then
      (bind _returnvalue (Utilities|Array|Add (Variables|/Game/Environment/Objects/TerritoryVolume/BP_TerritoryVolume.BP_TerritoryVolume_C|GetTerritoryInfos _territory) _self))
      (Variables|Default|SetIndexTerritory _returnvalue))
    (:else
      _))
  (bind _primary (Variables|Default|GetPrimary)
    (:then
      (bind _returnvalue_2 (Utilities|Array|Add (Variables|/Game/Blueprints/BP_PlayerPrimary.BP_PlayerPrimary_C|GetTerritoryInfo _primary) _self))
      (Variables|Default|SetIndexPrimary _returnvalue_2))
    (:else)))

(fn ConstructionScript)

(fn OnRepCommandCentre
  (Variables|Default|SetbHasCommandCentre (Utilities|IsValid (Variables|Default|GetCommandCentre))))