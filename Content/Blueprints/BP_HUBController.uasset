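; BP_HUBController is the player controller for the menu hub, handling the front-end UI and lobby hosting or joining.
; On BeginPlay it shows the cursor, displays BP_MainMenu as the active widget and pre-creates BP_DirectJoin without showing it.
; SetLoading adds a new loading screen to the viewport.
; Server_HostLobby and Server_JoinLobby forward to BP_OpulentiumInstance, passing the controller itself.
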(event Custom|Server_JoinLobby
  (bind _asbp_opulentium_instance (Utilities|Casting|CastToBP_OpulentiumInstance (Game|GetGameInstance)))
  (Default|JoinLobby _asbp_opulentium_instance self))

(event Custom|Server_HostLobby
  (bind _asbp_opulentium_instance (Utilities|Casting|CastToBP_OpulentiumInstance (Game|GetGameInstance)))
  (Default|HostLobby _asbp_opulentium_instance self))

(event Custom|SetLoading
  (bind _returnvalue (UserInterface|CreateWidget "/Game/Blueprints/Widget/BP_LoadScreen.BP_LoadScreen_C" self))
  (UserInterface|Viewport|AddtoViewport _returnvalue 0))

(event Custom|SpawnWidgets
  (bind _self self)
  (Variables|/Script/Engine.PlayerController|SetbShowMouseCursor _self true)
  (bind _returnvalue (UserInterface|CreateWidget "/Game/Blueprints/Widget/BP_MainMenu.BP_MainMenu_C" _self))
  (bind _output_get (Variables|Default|SetMainMenu _returnvalue))
  (UserInterface|Viewport|AddtoViewport _output_get 0)
  (Variables|Default|SetActiveWidget _output_get)
  (bind _returnvalue_2 (UserInterface|CreateWidget "/Game/Blueprints/Widget/BP_DirectJoin.BP_DirectJoin_C" _self))
  (Variables|Default|SetJoinGame _returnvalue_2))

(event EventBeginPlay
  (CallFunction|SpawnWidgets))

(fn ConstructionScript)