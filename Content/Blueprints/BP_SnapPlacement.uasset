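; BP_SnapPlacement is a structure placement actor that follows the owner's vision trace and snaps onto valid build spots.
; BeginPlay caches every He3 deposit and power node, and Tick passes them with the trace hit to SwitchCanPlace.
; If the player's He3 covers the cost, it snaps to the first unused spot within range and sets CanPlace.
; Extractors search deposits, while other structures search power nodes.
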(event EventBeginPlay
  ;[1 1 1] Tick
  (|CallParentFunction)
  (bind _outactors (Actor|GetAllActorsOfClass "/Game/Environment/Objects/He3Deposit/BP_He3Deposit.BP_He3Deposit_C"))
  (bind _outactors_2 (Actor|GetAllActorsOfClass "/Game/Environment/Objects/PowerNode/BP_PowerNode.BP_PowerNode_C")))

(event EventTick
  (params (DeltaSeconds :type Float%20%28single-precision%29))
  (bind _primaryowner (Variables|Default|GetPrimaryOwner))
  (bind _hitresult (Default|VisionTrace _primaryowner))
  (bind _location (Collision|BreakHitResult _hitresult))
  ;[1 1 1] Tick
  (if (Variables|Default|GetbCanPlace)
    _
    (else
      (Transformation|SetActorLocation _location false false)))
  (Utilities|SwitchCanPlace (stale EventBeginPlay _outactors) (stale EventBeginPlay _outactors_2) _location
    (:True
      (Transformation|SetActorLocation (Variables|Default|GetSnapLocation) false false))))

(fn ConstructionScript)