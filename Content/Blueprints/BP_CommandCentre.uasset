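; Command centre structure that claims its territory at tier 1 and serves as a team respawn option.
; On BeginPlay it raises the owning player's or AI's structure caps and refreshes the upgrade tree locally and via client event.
; It adds self or ally buttons to teammates' respawn menus, removing them and clearing the territory reference when destroyed.
; A radius mesh scales with CommandRadius, with replicated visibility following selection or placement.
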(event Custom|Client_UpdateTree
  ;[1 1 1] Destroyed
  (CallFunction|UpdateTree))

(event Custom|AddButtons
  (bind _self self)
  (bind _outactors (Actor|GetAllActorsOfClass "/Game/Blueprints/BP_PlayerPrimary.BP_PlayerPrimary_C"))
  (for _array_element _outactors
    (bind _playercontroller (Variables|/Game/Blueprints/BP_PlayerPrimary.BP_PlayerPrimary_C|GetPlayerController _array_element)
      (:then
        (bind _respawnmenu (Variables|/Game/Blueprints/BP_PlayerPrimary.BP_PlayerPrimary_C|GetRespawnMenu _array_element)
          (:then
            (if (== (Variables|/Game/Blueprints/BP_OpulentiumActor.BP_OpulentiumActor_C|GetTeam _array_element) (Variables|Default|GetTeam))
              (if (== _playercontroller (Components|GetOwner))
                (bind _returnvalue (UserInterface|CreateWidget "/Game/Blueprints/Widget/BP_HomeSelf.BP_HomeSelf_C" _playercontroller))
                (Utilities|Array|Add (Variables|/Game/Blueprints/Widget/BP_RespawnMenu.BP_RespawnMenu_C|GetButtons _respawnmenu) _returnvalue)
                (Variables|/Game/Blueprints/Widget/BP_HomeButton.BP_HomeButton_C|SetCommand _returnvalue _self)
                (if (Variables|/Game/Blueprints/BP_PlayerPrimary.BP_PlayerPrimary_C|GetbRespawn _array_element)
                  (UserInterface|Viewport|AddtoViewport _returnvalue 0))
                (else
                  (bind _returnvalue_2 (UserInterface|CreateWidget "/Game/Blueprints/Widget/BP_HomeAlly.BP_HomeAlly_C" _playercontroller))
                  (Utilities|Array|Add (Variables|/Game/Blueprints/Widget/BP_RespawnMenu.BP_RespawnMenu_C|GetButtons _respawnmenu) _returnvalue_2)
                  (Variables|/Game/Blueprints/Widget/BP_HomeButton.BP_HomeButton_C|SetCommand _returnvalue_2 _self)
                  (if (Variables|/Game/Blueprints/BP_PlayerPrimary.BP_PlayerPrimary_C|GetbRespawn _array_element)
                    (UserInterface|Viewport|AddtoViewport _returnvalue_2 0))))))
          (:else)))
      (:else))))

(event Custom|SetTerritoryTier
  (Variables|/Game/Blueprints/BP_TerritoryInfo.BP_TerritoryInfo_C|SetTier (.Result (CallFunction|GetTerritoryInfo (.Territory (CallFunction|GetTerritory)))) 1))

(event EventDestroyed
  ;[1 1 1] Destroyed
  (Variables|/Game/Blueprints/BP_TerritoryInfo.BP_TerritoryInfo_C|SetCommandCentre (.Result (CallFunction|GetTerritoryInfo (.Territory (CallFunction|GetTerritory)))) 0)
  (bind _outactors (Actor|GetAllActorsOfClass "/Game/Blueprints/BP_PlayerPrimary.BP_PlayerPrimary_C"))
  (for _array_element _outactors
    (bind _respawnmenu (Variables|/Game/Blueprints/BP_PlayerPrimary.BP_PlayerPrimary_C|GetRespawnMenu _array_element)
      (:then
        (bind _array_element_2 (Utilities|Array|ForEachLoopwithBreak (Variables|/Game/Blueprints/Widget/BP_RespawnMenu.BP_RespawnMenu_C|GetButtons _respawnmenu) :!label _label)
          (:LoopBody
            (if (== (Variables|/Game/Blueprints/Widget/BP_HomeButton.BP_HomeButton_C|GetCommand _array_element_2) self)
              (Widget|RemovefromParent _array_element_2)
              (Utilities|Array|RemoveItem (Variables|/Game/Blueprints/Widget/BP_RespawnMenu.BP_RespawnMenu_C|GetButtons _respawnmenu) _array_element_2)
              (goto _label Break)))))
      (:else)))
  (CallFunction|UpdateTree)
  (CallFunction|ClientUpdateTree))

(event EventBeginPlay
  (bind _commandradius (Variables|Default|GetCommandRadius))
  (bind _returnvalue (/ _commandradius 1e+02))
  (|CallParentFunction)
  (Transformation|SetWorldScale3D (Variables|Default|GetCCRadius) (Math|Vector|MakeVector _returnvalue _returnvalue 2.0))
  (bind _primaryowner (Variables|Default|GetPrimaryOwner)
    (:then
      (bind _ai (Variables|/Game/Blueprints/BP_PlayerPrimary.BP_PlayerPrimary_C|GetAI _primaryowner)
        (:then
          (Utilities|Array|Add (Utilities|Struct|BreakStructureInventory (Variables|/Game/Blueprints/BP_OpulentiumAI.BP_OpulentiumAI_C|GetStructureInventory _ai)) self))
        (:else
          _))
      (CallFunction|UpdatePopulation)
      (bind _currentplacement (Variables|/Game/Blueprints/BP_PlayerPrimary.BP_PlayerPrimary_C|GetCurrentPlacement _primaryowner)
        (:then
          (Variables|Default|SetbShowRadius (Variables|/Game/Blueprints/BP_Placement.BP_Placement_C|GetbShowRadius _currentplacement)))
        (:else
          _))
      (CallFunction|AddButtons)
      (CallFunction|SetTerritoryTier)
      (CallFunction|UpdateTree)
      (CallFunction|ClientUpdateTree))
    (:else)))

(event EventOnRepBSelected
  ;[1 1 1] Destroyed
  (|CallParentFunction)
  (Variables|Default|SetbShowRadius (Variables|Default|GetbSelected)))

(fn ConstructionScript
  (|CallParentFunction))

(fn OnRepBShowRadius
  (Development|SetHiddeninGame (Variables|Default|GetCCRadius) (not (Variables|Default|GetbShowRadius)) false))

(fn UpdateTree
  (bind _primaryowner (Variables|Default|GetPrimaryOwner)
    (:then
      (bind _upgrademenu (Variables|/Game/Blueprints/BP_PlayerPrimary.BP_PlayerPrimary_C|GetUpgradeMenu _primaryowner)
        (:then
          (bind _currenttree (Variables|/Game/Blueprints/Widget/BP_UpgradeMenu.BP_UpgradeMenu_C|GetCurrentTree _upgrademenu)
            (:then
              (Default|UpdateTree _currenttree))
            (:else)))
        (:else)))
    (:else)))

(fn OnRepCommandRadius
  (bind _commandradius (Variables|Default|GetCommandRadius))
  (bind _returnvalue (/ _commandradius 1e+02))
  (Transformation|SetWorldScale3D (Variables|Default|GetCCRadius) (Math|Vector|MakeVector _returnvalue _returnvalue 2.0)))

(fn UpdatePopulation
  (Variables|/Game/Blueprints/BP_TerritoryInfo.BP_TerritoryInfo_C|SetCommandCentre (.Result (CallFunction|GetTerritoryInfo (.Territory (CallFunction|GetTerritory)))) self)
  (bind _primaryowner (Variables|Default|GetPrimaryOwner)
    (:then
      (bind _playercontroller (Variables|/Game/Blueprints/BP_PlayerPrimary.BP_PlayerPrimary_C|GetPlayerController _primaryowner)
        (:then
          (bind _structout (Utilities|Struct|SetmembersinStructureCap (Variables|/Game/Blueprints/BP_OpulentiumPlayerController.BP_OpulentiumPlayerController_C|GetStructureCap _playercontroller) (+ (.T1FacCap (Utilities|Struct|BreakStructureCap (Variables|/Game/Blueprints/BP_OpulentiumPlayerController.BP_OpulentiumPlayerController_C|GetStructureCap _playercontroller))) 2) (+ (.ContainerCap (Utilities|Struct|BreakStructureCap (Variables|/Game/Blueprints/BP_OpulentiumPlayerController.BP_OpulentiumPlayerController_C|GetStructureCap _playercontroller))) 2) (+ (.T1BeaconCap (Utilities|Struct|BreakStructureCap (Variables|/Game/Blueprints/BP_OpulentiumPlayerController.BP_OpulentiumPlayerController_C|GetStructureCap _playercontroller))) 1)))
          (Variables|/Game/Blueprints/BP_OpulentiumPlayerController.BP_OpulentiumPlayerController_C|SetStructureCap _playercontroller _structout))
        (:else
          (bind _ai (Variables|/Game/Blueprints/BP_PlayerPrimary.BP_PlayerPrimary_C|GetAI _primaryowner)
            (:then
              (bind _structout_2 (Utilities|Struct|SetmembersinStructureCap (Variables|/Game/Blueprints/BP_OpulentiumAI.BP_OpulentiumAI_C|GetStructureCap _ai) (+ (.T1FacCap (Utilities|Struct|BreakStructureCap (Variables|/Game/Blueprints/BP_OpulentiumAI.BP_OpulentiumAI_C|GetStructureCap _ai))) 2) (+ (.ContainerCap (Utilities|Struct|BreakStructureCap (Variables|/Game/Blueprints/BP_OpulentiumAI.BP_OpulentiumAI_C|GetStructureCap _ai))) 2) (+ (.T1BeaconCap (Utilities|Struct|BreakStructureCap (Variables|/Game/Blueprints/BP_OpulentiumAI.BP_OpulentiumAI_C|GetStructureCap _ai))) 1)))
              (Variables|/Game/Blueprints/BP_OpulentiumAI.BP_OpulentiumAI_C|SetStructureCap _ai _structout_2)
              (Default|StatusCheck _ai))
            (:else)))))
    (:else)))