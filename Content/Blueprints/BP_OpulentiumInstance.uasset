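; BP_OpulentiumInstance handles LAN session hosting, joining and level travel for the game's lobby.
; HostLobby server-travels to LobbyMap01 when its session search succeeds, otherwise creates a session and opens that map as a listen server.
; JoinLobby shows loading on the hub controller and joins the first session found.
; Server_OpenLevel records each lobby controller's lobby-to-player ID pairing and shows its loading screen before issuing servertravel.
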(event Custom|HostLobby
  (params (Host :type Player%20Controller%20Object%20Reference))
  (|FindSessions Host 1 true
    (:OnSuccess
      (Development|ExecuteConsoleCommand "servertravel LobbyMap01" Host))
    (:OnFailure
      (|Session Host 8 true
        (:OnSuccess
          (Game|OpenLevel(byName) "LobbyMap01" true "listen"))))))

(event Custom|JoinLobby
  (params (Player :type Player%20Controller%20Object%20Reference))
  (bind _results (|FindSessions Player 1 true)
    (:then
      (bind _asbp_hubcontroller (Utilities|Casting|CastToBP_HUBController Player))
      (Default|SetLoading _asbp_hubcontroller))
    (:OnSuccess
      (|JoinSession Player (Utilities|Array|Get(acopy) _results)))))

(event Custom|Server_OpenLevel
  (params (Level :type Name))
  (bind _returnvalue (Utilities|String|ToString(Name) Level))
  (bind _returnvalue_2 (Utilities|String|Append "servertravel " _returnvalue))
  (Development|PrintString _returnvalue_2)
  (CallFunction|PopulateIDInfo)
  (Development|ExecuteConsoleCommand _returnvalue_2 (Game|GetPlayerController 0)))

(fn PopulateIDInfo
  (bind _outactors (Actor|GetAllActorsOfClass "/Game/Blueprints/Widget/BP_LobbyController.BP_LobbyController_C"))
  (for _array_element _outactors
    (bind _playerstate (Variables|/Script/Engine.Controller|GetPlayerState _array_element)
      (:then
        (Utilities|Array|Add (Variables|Default|GetPlayerIDs) (Utilities|Struct|MakePlayerIDInfo (Variables|/Game/Blueprints/Widget/BP_LobbyController.BP_LobbyController_C|GetID _array_element) (Variables|/Script/Engine.PlayerState|GetPlayerId _playerstate)))
        (Default|ShowLoad _array_element))
      (:else))))