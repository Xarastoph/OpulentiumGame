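; BP_Conduit is a player-owned structure that claims a nearby power node and provides an upgrade tree UI.
; On BeginPlay it creates the tree widget for its owning player controller, links it back to itself, then after a brief delay marks the first BP_PowerNode found in range as used.
; ShowTree displays the widget around screen center.
; On destruction it frees the node and destroys its current upgrade and build actors.
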(event EventBeginPlay
  (bind _self self)
  (|CallParentFunction)
  (bind _asbp_opulentium_player_controller (Utilities|Casting|CastToBP_OpulentiumPlayerController (Components|GetOwner))
    (:then
      (bind _returnvalue (UserInterface|CreateWidget (Variables|Default|GetUpgradeTreeClass) _asbp_opulentium_player_controller))
      (Utilities|IsValid _returnvalue
        (:Is%20Valid
          (Variables|Default|SetUpgradeTree _returnvalue)
          (Variables|/Game/Blueprints/Widget/BP_UpgradeTree.BP_UpgradeTree_C|SetStructure _returnvalue _self))
        (:Is%20Not%20Valid
          _)))
    (:CastFailed
      _))
  (Utilities|FlowControl|Delay 0.01)
  (CallFunction|SetNode _self))

(event EventShowTree
  (bind _upgradetree (Variables|Default|GetUpgradeTree)
    (:then
      (UserInterface|Viewport|AddtoViewport _upgradetree 1)
      (Class|Widget|SetRenderTransform _upgradetree (Utilities|Struct|MakeWidgetTransform "(X=-440.000000,Y=-136.000000)"))
      (Class|UserWidget|SetDesiredSizeinViewport _upgradetree "(X=678.000000,Y=371.000000)")
      (Class|UserWidget|SetAnchorsinViewport _upgradetree (Utilities|Struct|MakeAnchors "(X=0.500000,Y=0.500000)" "(X=0.500000,Y=0.500000)")))
    (:else)))

(event EventDestroyed
  (bind _node (Variables|Default|GetNode)
    (:then
      (Variables|/Game/Environment/Objects/PowerNode/BP_PowerNode.BP_PowerNode_C|SetbUsed _node false))
    (:else
      _))
  (bind _currentupgrade (Variables|Default|GetCurrentUpgrade)
    (:then
      (Actor|DestroyActor _currentupgrade))
    (:else
      _))
  (bind _currentbuild (Variables|Default|GetCurrentBuild)
    (:then
      (Actor|DestroyActor _currentbuild))
    (:else)))

(fn ConstructionScript)

(fn SetNode
  (bind _outactors (Actor|GetAllActorsOfClass "/Game/Environment/Objects/PowerNode/BP_PowerNode.BP_PowerNode_C"))
  (bind _array_element (Utilities|Array|ForEachLoopwithBreak _outactors :!label _label)
    (:LoopBody
      (if (<= (Transformation|GetDistanceTo _array_element self) 256.0)
        (Variables|Default|SetNode _array_element)
        (Variables|/Game/Environment/Objects/PowerNode/BP_PowerNode.BP_PowerNode_C|SetbUsed _array_element true)
        (goto _label Break)))))