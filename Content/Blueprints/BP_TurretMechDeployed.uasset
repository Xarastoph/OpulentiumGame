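; Deployed turret mech Blueprint that aims at its current target and directs its weapons at it.
; SetTarget calls its parent, then steps yaw and pitch at TurnRate, snapping when close, with yaw offset 180 degrees.
; CanFire requires both axes aligned.
; FireWeapon and ProxyRepFire pass the target to all weapons or clear it, and the CurrentTarget rep-notify drops CanFire when the target is invalid.
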(event EventOnRepCurrentTarget
  ;[1 1 1] SetAnimValues
  (Variables|Default|GetCurrentTarget
    (:then)
    (:else
      (Variables|Default|SetbCanFire false))))

(event EventFireWeapon
  (bind _currenttarget (Variables|Default|GetCurrentTarget))
  (bind _weapons (Variables|Default|GetWeapons))
  ;[1 1 1] SetAnimValues
  (if (and (Utilities|IsValid _currenttarget) (Variables|Default|GetbCanFire))
    (for _array_element _weapons
      (Utilities|IsValid _array_element
        (:Is%20Valid
          (Variables|/Game/Blueprints/BP_Weapon.BP_Weapon_C|SetTarget _array_element _currenttarget))))
    (else
      (for _array_element_2 _weapons
        (Utilities|IsValid _array_element_2
          (:Is%20Valid
            (Variables|/Game/Blueprints/BP_Weapon.BP_Weapon_C|SetTarget _array_element_2 0)))))))

(event EventSetTarget
  (params (DTime :type Float%20%28single-precision%29))
  ;[1 1 1] SetAnimValues
  (|CallParentFunction DTime)
  (bind _byaw (CallFunction|SetYaw DTime))
  (CallFunction|SetPitch _byaw DTime))

(event EventProxyRepFire
  (bind _currenttarget (Variables|Default|GetCurrentTarget))
  (bind _weapons (Variables|Default|GetWeapons))
  ;[1 1 1] SetAnimValues
  (if (and (Utilities|IsValid _currenttarget) (Variables|Default|GetbCanFire))
    (for _array_element _weapons
      (Utilities|IsValid _array_element
        (:Is%20Valid
          (Variables|/Game/Blueprints/BP_Weapon.BP_Weapon_C|SetTarget _array_element _currenttarget))))
    (else
      (for _array_element_2 _weapons
        (Utilities|IsValid _array_element_2
          (:Is%20Valid
            (Variables|/Game/Blueprints/BP_Weapon.BP_Weapon_C|SetTarget _array_element_2 0)))))))

(fn ConstructionScript)

(fn SetYaw
  (params (DTime :type Float%20%28single-precision%29))
  (bind _turnrate (Variables|Default|GetTurnRate))
  (bind _returnvalue (* DTime _turnrate))
  (bind _currenttarget (Variables|Default|GetCurrentTarget)
    (:then
      (if (< _returnvalue (Math|Float|Absolute(Float) (- (Math|Float|Absolute(Float) (.Yaw (Math|Rotator|BreakRotator (Math|Rotator|Delta(Rotator) (CallFunction|GetTurretRotation) (Math|Rotator|FindLookatRotation (Transformation|GetActorLocation) (Transformation|GetActorLocation _currenttarget)))))) 1.8e+02)))
        (Variables|Default|SetTurretYaw (+ (* _returnvalue (Math|Float|Sign(Float) (.Yaw (Math|Rotator|BreakRotator (Math|Rotator|Delta(Rotator) (CallFunction|GetTurretRotation) (Math|Rotator|FindLookatRotation (Transformation|GetActorLocation) (Transformation|GetActorLocation _currenttarget))))))) (stale _output_get)))
        (else
          (bind _output_get (Variables|Default|SetTurretYaw (+ (.Yaw (Math|Rotator|BreakRotator (Math|Rotator|FindLookatRotation (Transformation|GetActorLocation) (Transformation|GetActorLocation _currenttarget)))) 1.8e+02)))
          (return true))))
    (:else
      _))
  (return false))

(fn GetTurretRotation
  (return (Math|Rotator|MakeRotator 0.0 (Variables|Default|GetTurretPitch) (Variables|Default|GetTurretYaw))))

(fn SetPitch
  (params (bYaw :type Boolean) (DTime :type Float%20%28single-precision%29))
  (bind _turnrate (Variables|Default|GetTurnRate))
  (bind _returnvalue (* DTime _turnrate))
  (bind _currenttarget (Variables|Default|GetCurrentTarget)
    (:then
      (if (< _returnvalue (Math|Float|Absolute(Float) (.Pitch (Math|Rotator|BreakRotator (Math|Rotator|Delta(Rotator) (CallFunction|GetTurretRotation) (Math|Rotator|FindLookatRotation (Transformation|GetActorLocation) (Transformation|GetActorLocation _currenttarget)))))))
        (Variables|Default|SetTurretPitch (+ (* _returnvalue (Math|Float|Sign(Float) (.Pitch (Math|Rotator|BreakRotator (Math|Rotator|Delta(Rotator) (CallFunction|GetTurretRotation) (Math|Rotator|FindLookatRotation (Transformation|GetActorLocation) (Transformation|GetActorLocation _currenttarget))))))) (stale _output_get_2)))
        (bind _output_get (LocalVariables|SetbPitch false))
        (else
          (bind _output_get_2 (Variables|Default|SetTurretPitch (.Pitch (Math|Rotator|BreakRotator (Math|Rotator|FindLookatRotation (Transformation|GetActorLocation) (Transformation|GetActorLocation _currenttarget))))))
          (LocalVariables|SetbPitch true)))
      (if (Math|Boolean|NotEqual(Boolean) (stale _output_get_3) (and _output_get bYaw))
        (bind _output_get_3 (Variables|Default|SetbCanFire (and _output_get bYaw)))))
    (:else)))

(fn OnRepBFireWeapon)