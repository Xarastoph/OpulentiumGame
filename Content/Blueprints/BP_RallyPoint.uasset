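; BP_RallyPoint is a rally point flag tied to a Builder and owned by the player (BP_PlayerPrimary).
; Each tick it turns on yaw only to face the player.
; While Locating, it snaps just above the player's vision trace hit to preview placement.
; Otherwise it hides on a short timer, but reappears while the player looks at its Builder or that Builder is selected.
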(event Custom|Hide
  ;[1 1 1] HideSelf
  (Rendering|SetActorHiddenInGame true))

(event EventBeginPlay
  ;[1 1 1] Begin Play
  (bind _asbp_player_primary (Utilities|Casting|CastToBP_PlayerPrimary (Components|GetOwner)))
  (bind _output_get (Variables|Default|SetPrimaryOwner _asbp_player_primary)))

(event EventTick
  (params (DeltaSeconds :type Float%20%28single-precision%29))
  (bind _builder (Variables|Default|GetBuilder))
  ;[1 1 1] Flag Lookat
  (Transformation|SetWorldRotation (Math|Rotator|MakeRotator 0.0 0.0 (.Yaw (Math|Rotator|BreakRotator (Math|Rotator|FindLookatRotation (Transformation|GetActorLocation self) (Transformation|GetWorldLocation (stale EventBeginPlay _output_get)))))) false false)
  ;[1 1 1] Locating
  (if (Variables|Default|GetbLocating)
    (Transformation|SetActorLocation (+ (.Location (Collision|BreakHitResult (Default|VisionTrace (Variables|Default|GetPrimaryOwner)))) "0, 0,4.000000") false false)
    (Rendering|SetActorHiddenInGame false :!label _label)
    (Class|KismetSystemLibrary|ClearTimerHandle (stale _returnvalue))
    (else
      ;[1 1 1] Hide Test
      (if (Utilities|Time|IsTimerActivebyHandle (stale _returnvalue))
        _
        (else
          (bind _returnvalue (Utilities|Time|SetTimerbyEvent (delegate Custom|Hide) 3.0))))
      (bind _primaryowner (Variables|Default|GetPrimaryOwner)
        (:then
          (bind _lookatobject (Variables|/Game/Blueprints/BP_PlayerPrimary.BP_PlayerPrimary_C|GetLookatObject _primaryowner)
            (:then
              (bind _asbp_builder (Utilities|Casting|CastToBP_Builder _lookatobject)
                (:then
                  (if (== _asbp_builder _builder)
                    (goto _label)
                    (else
                      _)))
                (:CastFailed
                  _)))
            (:else
              _))
          (if (Variables|/Game/Blueprints/BP_OpulentiumActor.BP_OpulentiumActor_C|GetbSelected _builder)
            (goto _label)))
        (:else)))))

(fn ConstructionScript)