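; BP_Icons is a selection and highlight indicator that shows a bounding box for a Parent object.
; RepNotifies on its show and selected states toggle the box and custom depth rendering on the parent's mesh, turning the box green when selected and white otherwise.
; Deselection clears the show state unless the parent is still the primary owner's look-at object.
; Health and max health notifies are empty.
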(fn ConstructionScript)

(fn OnRepBShowBox
  (bind _bshowbox (Variables|Default|GetbShowBox))
  (bind _bselected (Variables|Default|GetbSelected))
  (bind _returnvalue (or _bshowbox _bselected))
  (Development|SetHiddeninGame (Variables|Default|GetBoundingBox) (not _returnvalue) false)
  (bind _parent (Variables|Default|GetParent)
    (:then
      (Rendering|SetRenderCustomDepth (Variables|/Script/Engine.Character|GetMesh _parent) _returnvalue))
    (:else)))

(fn OnRepBSelected
  (bind _boundingbox (Variables|Default|GetBoundingBox))
  (if (Variables|Default|GetbSelected)
    (Rendering|Material|SetMaterial _boundingbox 0 "/Game/Environment/Materials/Glow/GreenMat.GreenMat")
    (Development|SetHiddeninGame _boundingbox false false)
    (bind _parent (Variables|Default|GetParent)
      (:then
        (Rendering|SetRenderCustomDepth (Variables|/Script/Engine.Character|GetMesh _parent) true))
      (:else))
    (else
      (Rendering|Material|SetMaterial _boundingbox 0 "/Game/Environment/Materials/Glow/WhiteMat.WhiteMat")
      (bind _primaryowner (Variables|Default|GetPrimaryOwner)
        (:then
          (if (and (not (== (Variables|Default|GetParent) (Variables|/Game/Blueprints/BP_PlayerPrimary.BP_PlayerPrimary_C|GetLookatObject _primaryowner))) (stale _output_get))
            (bind _output_get (Variables|Default|SetbShowBox false))))
        (:else)))))

(fn OnRepHealth)

(fn OnRepHealthMax)