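; Owned, selectable game actor with replicated health that notifies its PrimaryOwner on spawn and clears its groups before destruction.
; Authority-side damage clamps health and triggers a sphere trace that sets nearby mechs' temporary target to the attacker, throttled by a retriggerable cooldown.
; Rep-notifies drive death, cooldown reset and custom-depth outlines for selection or owner look-at.
; Helpers provide a radar sphere test and find territory volumes and their per-owner info.
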(event Custom|Death
  (bind _primaryowner (Variables|Default|GetPrimaryOwner)
    (:then
      (Default|ClearGroups _primaryowner self))
    (:else
      _))
  (Actor|DestroyActor))

(event Custom|NotifyAttack
  (params (Instigator :type BP%20Opulentium%20Actor%20Object%20Reference))
  (bind _returnvalue (Transformation|GetActorLocation))
  (if (Variables|Default|GetbNotifyAttack)
    (Variables|Default|SetbNotifyAttack false)
    (bind _outhits (Collision|MultiSphereTraceForObjects _returnvalue (+ _returnvalue "0, 0,4.000000") 2048.0 (Utilities|Array|MakeArray "ObjectTypeQuery3") false 0 "None" false))
    (for _array_element _outhits
      (bind _asbp_mech (Utilities|Casting|CastToBP_Mech (.HitActor (Collision|BreakHitResult _array_element))))
      (Variables|/Game/Blueprints/BP_Mech.BP_Mech_C|SetTempTarget _asbp_mech Instigator))))

(event Custom|ResetNotifyAttack
  (Utilities|FlowControl|RetriggerableDelay 1e+01)
  (Variables|Default|SetbNotifyAttack true))

(event EventBeginPlay
  (bind _spawntext (Variables|Default|GetSpawnText))
  (bind _primaryowner (Variables|Default|GetPrimaryOwner)
    (:then
      (if (Utilities|Enum|NotEqual(Enum) _spawntext "")
        (Default|AddNotification _primaryowner (Utilities|Struct|MakeNotificationInfo (Variables|Default|GetHUDIcon) _spawntext)))
      (bind _ai (Variables|/Game/Blueprints/BP_PlayerPrimary.BP_PlayerPrimary_C|GetAI _primaryowner)
        (:then
          (Utilities|FlowControl|Delay 0.5)
          (Default|QuickStatusCheck _ai))
        (:else)))
    (:else)))

(fn ConstructionScript)

(fn TakeDamage
  (params (Damage :type Integer) (Instigator :type BP%20Opulentium%20Actor%20Object%20Reference))
  (Networking|SwitchHasAuthority
    (:Authority
      (Variables|Default|SetHealth (Math|Integer|Clamp(Integer) (- (Variables|Default|GetHealth) Damage) 0 (Variables|Default|GetHealthMax)))
      (CallFunction|NotifyAttack Instigator))))

(fn OnRepHealth
  (if (<= (Variables|Default|GetHealth) 0)
    (CallFunction|Death)))

(fn OnRepBSelected
  (bind _bselected (Variables|Default|GetbSelected))
  (Rendering|SetCustomDepthStencilValue (Variables|Character|GetMesh) (+ 252 (Math|Conversions|ToInteger(Boolean) _bselected)))
  (if _bselected
    (Variables|Default|SetbShowBox true :!label _label)
    (else
      (bind _primaryowner (Variables|Default|GetPrimaryOwner)
        (:then
          (bind _lookatobject (Variables|/Game/Blueprints/BP_PlayerPrimary.BP_PlayerPrimary_C|GetLookatObject _primaryowner)
            (:then
              (if (!= _lookatobject self)
                _
                (else
                  (goto _label))))
            (:else
              _)))
        (:else
          _))
      (Variables|Default|SetbShowBox false))))

(fn OnRepBShowBox
  (Rendering|SetRenderCustomDepth (Variables|Character|GetMesh) (Variables|Default|GetbShowBox)))

(fn EnemyRadarTest
  (params (Primary :type BP%20Player%20Primary%20Object%20Reference))
  (bind _returnvalue (Transformation|GetActorLocation Primary))
  (bind _outhits (Collision|MultiSphereTraceForObjects _returnvalue (+ _returnvalue "0, 0,4.000000") 7.2e+03 (Utilities|Array|MakeArray "ObjectTypeQuery3") false 0 "None"))
  (bind _array_element (Utilities|Array|ForEachLoopwithBreak _outhits :!label _label)
    (:LoopBody
      (Utilities|IsValid (.HitActor (Collision|BreakHitResult _array_element))
        (:Is%20Valid
          (if (or (== (Components|GetOwner (.HitActor (Collision|BreakHitResult _array_element))) (Variables|/Game/Blueprints/BP_PlayerPrimary.BP_PlayerPrimary_C|GetPlayerController Primary)) (== (.HitActor (Collision|BreakHitResult _array_element)) Primary))
            (bind _output_get (LocalVariables|SetbValid false))
            (goto _label Break)))))
    (:Completed
      (return _output_get))))

(fn GetTerritory
  (bind _returnvalue (Transformation|GetActorLocation))
  (bind _outhit (Collision|LineTraceForObjects _returnvalue (+ _returnvalue "0, 0,10000.000000") (Utilities|Array|MakeArray "ObjectTypeQuery7") false 0 "None"))
  (bind _asbp_territory_volume (Utilities|Casting|CastToBP_TerritoryVolume (.HitActor (Collision|BreakHitResult _outhit)))
    (:then
      (return _asbp_territory_volume true))
    (:CastFailed
      (return 0 false))))

(fn GetTerritoryInfo
  (params (Territory :type BP%20Territory%20Volume%20Object%20Reference))
  (bind _array_element (Utilities|Array|ForEachLoopwithBreak (Variables|/Game/Environment/Objects/TerritoryVolume/BP_TerritoryVolume.BP_TerritoryVolume_C|GetTerritoryInfos Territory) :!label _label)
    (:LoopBody
      (if (or (== (Variables|/Game/Blueprints/BP_TerritoryInfo.BP_TerritoryInfo_C|GetPrimary _array_element) (Variables|Default|GetPrimaryOwner)) (== (Variables|/Game/Blueprints/BP_TerritoryInfo.BP_TerritoryInfo_C|GetPrimary _array_element) self))
        (bind _output_get (LocalVariables|SetInfo _array_element))
        (goto _label Break)))
    (:Completed
      (return _output_get (Utilities|IsValid _output_get)))))

(fn OnRepBNotifyAttack
  (if (not (Variables|Default|GetbNotifyAttack))
    (CallFunction|ResetNotifyAttack)))