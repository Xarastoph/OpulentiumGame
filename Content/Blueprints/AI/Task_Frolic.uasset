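; Behavior tree task that makes a BP_MechBot-controlled pawn frolic by moving it to a random spot around its focus.
; It centers on the blackboard FocusActor's location when valid, otherwise on the Focus vector.
; A flattened random direction scaled between Radius and a quarter of it offsets the destination.
; AIMoveTo drives the pawn, and the task reports success whether the move succeeds or fails.
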(event EventReceiveExecute
  (params (OwnerActor :type Actor%20Object%20Reference))
  (bind _returnvalue (Math|Random|RandomUnitVector))
  (bind _focusactor (Variables|Default|GetFocusActor))
  (bind _radius (Variables|Default|GetRadius))
  (bind _returnvalue_2 (Class|BTFunctionLibrary|GetBlackboardValueasObject _focusactor))
  (bind (_x _y) (Math|Vector|BreakVector _returnvalue))
  (bind _returnvalue_3 (/ _radius 4.0))
  (bind _returnvalue_4 (Math|Vector|MakeVector _x _y 0.0))
  (bind _returnvalue_5 (Math|Random|RandomFloatinRange _radius _returnvalue_3))
  (bind _returnvalue_6 (* _returnvalue_4 _returnvalue_5))
  ;[1 1 1] Frolic
  (bind _asbp_mech_bot (Utilities|Casting|CastToBP_MechBot OwnerActor))
  (Utilities|IsValid _returnvalue_2
    (:Is%20Valid
      (bind _asactor (Utilities|Casting|CastToActor _returnvalue_2))
      (AI|AIMoveTo (Pawn|GetControlledPawn _asbp_mech_bot) (+ (Transformation|GetActorLocation _asactor) _returnvalue_6) 0 32.0 false
        (:OnSuccess
          _)
        (:OnFail
          _)))
    (:Is%20Not%20Valid
      (AI|AIMoveTo (Pawn|GetControlledPawn _asbp_mech_bot) (+ (Class|BTFunctionLibrary|GetBlackboardValueasVector (Variables|Default|GetFocus)) _returnvalue_6) 0 5.0 false
        (:OnSuccess
          _)
        (:OnFail
          _))))
  (AI|BehaviorTree|FinishExecute true))