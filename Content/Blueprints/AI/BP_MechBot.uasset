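; AI controller for mech units that runs the Mech behavior tree and holds their move, patrol, rally, follow and transport orders.
; RepNotify handlers on the order flags clear conflicting orders, destroy the mech's current placement and handle transport seats.
; Queued moves use an order-numbered chain that renumbers when Moving turns off, with SetMoving re-raised after a short delay.
; Ending a patrol removes the mech from its patrol points and clears the chain.
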(event Custom|DestroyPlacement
  (bind _mech (Variables|Default|GetMech)
    (:then
      (bind _currentplacement (Variables|/Game/Blueprints/BP_Mech.BP_Mech_C|GetCurrentPlacement _mech)
        (:then
          (Actor|DestroyActor _currentplacement))
        (:else)))
    (:else)))

(event Custom|ResetMoving
  ;[1 1 1] Begin Play
  (Utilities|FlowControl|Delay 0.1)
  (Variables|Default|SetbSetMoving true))

(event EventBeginPlay
  ;[1 1 1] Begin Play
  (Utilities|FlowControl|Delay 0.1)
  (Class|AIController|UseBlackboard "/Game/Blueprints/AI/Mech_Blackboard.Mech_Blackboard")
  (AI|RunBehaviorTree "/Game/Blueprints/AI/BT_Mech.BT_Mech")
  (bind _asbp_mech (Utilities|Casting|CastToBP_Mech (Pawn|GetControlledPawn)))
  (Variables|Default|SetMech _asbp_mech))

(fn ConstructionScript)

(fn PurgeMovetoChain
  (Utilities|Array|Clear (Variables|Default|GetMoveToChain)))

(fn NegateOrder
  (bind _movetochain (Variables|Default|GetMoveToChain))
  (bind (_array_element _array_index) (Utilities|Array|ForEachLoopwithBreak _movetochain :!label _label)
    (:LoopBody
      (if (== (Utilities|Struct|BreakMoveToInfo _array_element) (CallFunction|GetCurrentMoveto))
        (Utilities|Array|RemoveIndex _movetochain _array_index)
        (goto _label Break)))
    (:Completed
      (for (_array_element_2 _array_index_2) _movetochain
        (Utilities|Array|SetArrayElem _movetochain _array_index_2 (Utilities|Struct|MakeMoveToInfo (.MoveTo (Utilities|Struct|BreakMoveToInfo _array_element_2)) (- (.Order (Utilities|Struct|BreakMoveToInfo _array_element_2)) 1)) true))
      (Variables|Default|SetCurrentMoveTo 0))))

(fn SetNextMoveto
  (bind _current (CallFunction|GetCurrentMoveto))
  (Utilities|IsValid _current
    (:Is%20Valid
      (Variables|Default|SetCurrentMoveTo _current)
      (Variables|Default|SetbMoving true))
    (:Is%20Not%20Valid
      (CallFunction|PurgeMovetoChain))))

(fn GetCurrentMoveto
  (bind _array_element (Utilities|Array|ForEachLoopwithBreak (Variables|Default|GetMoveToChain) :!label _label)
    (:LoopBody
      (if (== (.Order (Utilities|Struct|BreakMoveToInfo _array_element)) 1)
        (bind _output_get (LocalVariables|SetMoveTo (.MoveTo (Utilities|Struct|BreakMoveToInfo _array_element))))
        (goto _label Break)))
    (:Completed
      (return _output_get))))

(fn OnRepBMoving
  (if (Variables|Default|GetbMoving)
    (Variables|Default|SetbMoveToRally false)
    (Variables|Default|SetbFollowActor false)
    (Variables|Default|SetbPatrol false)
    (Variables|Default|SetbEnterTransport false)
    (Variables|Default|SetFollowActor 0)
    (else
      (Variables|Default|SetbSetMoving false)
      (CallFunction|NegateOrder))))

(fn OnRepBSetMoving
  (CallFunction|ResetMoving))

(fn OnRepBPatrol
  (bind _patrolchain (Variables|Default|GetPatrolChain))
  (bind _item (Utilities|Array|Get(acopy) _patrolchain))
  (if (Variables|Default|GetbPatrol)
    (Variables|Default|SetbMoving false)
    (Variables|Default|SetbMoveToRally false)
    (Variables|Default|SetbFollowActor false)
    (Variables|Default|SetFollowActor 0)
    (CallFunction|DestroyPlacement)
    (else
      (bind _asbp_mech (Utilities|Casting|CastToBP_Mech (Pawn|GetControlledPawn)))
      (for _array_element _patrolchain
        (Utilities|IsValid _array_element
          (:Is%20Valid
            (Utilities|Array|RemoveItem (Variables|/Game/Blueprints/BP_PatrolTo.BP_PatrolTo_C|GetMechs _array_element) _asbp_mech))))
      (Utilities|IsValid _item
        (:Is%20Valid
          (bind _output_get (LocalVariables|SetTestPatrol _item))
          (Utilities|Array|Clear _patrolchain)
          (Default|MechTest _output_get))
        (:Is%20Not%20Valid
          (Utilities|Array|Clear _patrolchain))))))

(fn OnRepBMovetoRally
  (if (Variables|Default|GetbMoveToRally)
    (Variables|Default|SetbMoving false)
    (Variables|Default|SetbFollowActor false)
    (Variables|Default|SetbPatrol false)
    (Variables|Default|SetFollowActor 0)
    (CallFunction|DestroyPlacement)))

(fn OnRepBFollowActor
  (if (Variables|Default|GetbFollowActor)
    (Variables|Default|SetbMoving false)
    (Variables|Default|SetbPatrol false)
    (Variables|Default|SetbMoveToRally false)
    (Variables|Default|SetbEnterTransport false)
    (CallFunction|DestroyPlacement)))

(fn OnRepBEnterTransport
  (bind _bentertransport (Variables|Default|GetbEnterTransport))
  (bind _transport (Variables|Default|GetTransport))
  (bind (_size _index) (Utilities|Struct|BreakTransportTarget _transport))
  (bind _currenttransport (Variables|Default|GetCurrentTransport)
    (:then
      (if _bentertransport
        (Variables|Default|SetDestination (.Location (Default|GetSeatLocation _currenttransport _size _index)))
        (Variables|Default|SetbTransform false)
        (Variables|Default|SetFollowActor 0)
        (CallFunction|DestroyPlacement)
        (else
          (Default|SetOccupied _currenttransport _index _size true))))
    (:else
      (if _bentertransport
        (Variables|Default|SetbMoving false)))))