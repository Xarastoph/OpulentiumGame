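; Behavior tree task that moves a BP_MechBot's controlled mech to the MoveTo blackboard location and handles what happens on arrival.
; It detaches the mech from any parent it follows, runs AI MoveTo, then updates the Idle key and bot movement flags.
; Depending on the move result and bot flags, it boards or clears a transport slot, or triggers a pacifist mech's turret transform.
; Move success and failure share this logic, and the task finishes as successful.
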(event EventReceiveExecute
  (params (OwnerActor :type Actor%20Object%20Reference))
  (bind _idle (Variables|Default|GetIdle))
  ;[1 1 1] Move To
  (bind _asbp_mech_bot (Utilities|Casting|CastToBP_MechBot OwnerActor)
    (:then
      (bind _asbp_mech (Utilities|Casting|CastToBP_Mech (Pawn|GetControlledPawn _asbp_mech_bot))
        (:then
          (bind _parent (Variables|/Game/Blueprints/BP_CombatActor.BP_CombatActor_C|GetParent _asbp_mech)
            (:then
              (Default|RemoveFollowActor _parent _asbp_mech))
            (:else
              _))
          (bind _movementresult (AI|AIMoveTo (Pawn|GetControlledPawn _asbp_mech_bot) (Class|BTFunctionLibrary|GetBlackboardValueasVector (Variables|Default|GetMoveTo)) 0 1.0 false)
            (:OnSuccess
              _)
            (:OnFail
              _))
          (if (Variables|/Game/Blueprints/AI/BP_MechBot.BP_MechBot_C|GetbSetBoolMoving _asbp_mech_bot)
            (Variables|/Game/Blueprints/AI/BP_MechBot.BP_MechBot_C|SetbSetBoolMoving _asbp_mech_bot false)
            (Class|BTFunctionLibrary|SetBlackboardValueasBool _idle false)
            (else
              (Class|BTFunctionLibrary|SetBlackboardValueasBool _idle true)))
          (if (Variables|/Game/Blueprints/AI/BP_MechBot.BP_MechBot_C|GetbSetMoving _asbp_mech_bot)
            (Variables|/Game/Blueprints/AI/BP_MechBot.BP_MechBot_C|SetbMoving _asbp_mech_bot false))
          (if (Utilities|Enum|NotEqual(Enum) _movementresult "Success")
            ;[1 1 1] Turret
            (if (Variables|/Game/Blueprints/AI/BP_MechBot.BP_MechBot_C|GetbEnterTransport _asbp_mech_bot) :!label _label
              (bind _currenttransport (Variables|/Game/Blueprints/AI/BP_MechBot.BP_MechBot_C|GetCurrentTransport _asbp_mech_bot)
                (:then
                  (if (not (Variables|/Game/Blueprints/BP_Vehicle.BP_Vehicle_C|GetbBeginFly _currenttransport))
                    (Default|AddPassenger _currenttransport (.Size (Utilities|Struct|BreakTransportTarget (Variables|/Game/Blueprints/AI/BP_MechBot.BP_MechBot_C|GetTransport _asbp_mech_bot))) (.Index (Utilities|Struct|BreakTransportTarget (Variables|/Game/Blueprints/AI/BP_MechBot.BP_MechBot_C|GetTransport _asbp_mech_bot))) _asbp_mech)
                    (else
                      (Default|ClearPassenger _currenttransport (.Size (Utilities|Struct|BreakTransportTarget (Variables|/Game/Blueprints/AI/BP_MechBot.BP_MechBot_C|GetTransport _asbp_mech_bot))) (.Index (Utilities|Struct|BreakTransportTarget (Variables|/Game/Blueprints/AI/BP_MechBot.BP_MechBot_C|GetTransport _asbp_mech_bot)))))))
                (:else
                  _)))
            (elif (Variables|/Game/Blueprints/BP_CombatActor.BP_CombatActor_C|GetbPacifist _asbp_mech)
              (if (Variables|/Game/Blueprints/AI/BP_MechBot.BP_MechBot_C|GetbTransform _asbp_mech_bot)
                (Variables|/Game/Blueprints/BP_Mech.BP_Mech_C|SetbLookat _asbp_mech true)
                (Variables|/Game/Blueprints/AI/BP_MechBot.BP_MechBot_C|SetbTransform _asbp_mech_bot false)
                (bind _currentplacement (Variables|/Game/Blueprints/BP_Mech.BP_Mech_C|GetCurrentPlacement _asbp_mech)
                  (:then
                    (Actor|DestroyActor _currentplacement))
                  (:else
                    (Variables|/Game/Blueprints/BP_PlayerPrimary.BP_PlayerPrimary_C|GetAI (Variables|/Game/Blueprints/BP_OpulentiumActor.BP_OpulentiumActor_C|GetPrimaryOwner _asbp_mech)
                      (:then
                        (Variables|/Game/Blueprints/BP_Mech.BP_Mech_C|SetSpawnTransform _asbp_mech (Math|Transform|MakeTransform (+ (.Location (Math|Transform|BreakTransform (Transformation|GetActorTransform _asbp_mech))) (Math|Vector|MakeVector 0.0 0.0 (- (Utilities|GetClassDefaults (Variables|/Game/Blueprints/BP_Mech.BP_Mech_C|GetDeployedClass _asbp_mech)) (Components|Capsule|GetScaledCapsuleHalfHeight (Variables|/Script/Engine.Character|GetCapsuleComponent _asbp_mech))))) (.Rotation (Math|Transform|BreakTransform (Transformation|GetActorTransform _asbp_mech))) (.Scale (Math|Transform|BreakTransform (Transformation|GetActorTransform _asbp_mech))))))
                      (:else
                        _))))
                (Variables|/Game/Blueprints/BP_Mech.BP_Mech_C|SetbTransform _asbp_mech true)
                (else
                  (goto _label)))
              (else
                (goto _label)))))
        (:CastFailed
          _)))
    (:CastFailed
      _))
  (AI|BehaviorTree|FinishExecute true))