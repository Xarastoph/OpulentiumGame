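; Behavior tree task that sends a mech bot's controlled pawn to the rally point actor stored in the blackboard.
; It runs AI MoveTo, then on either success or failure clears the bot's MoveToRally flag and the RallyPoint and GoToRally keys.
; It always finishes as successful, even if the cast to BP_MechBot fails, while an abort only resets GoToRally.
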(event EventReceiveExecute
  (params (OwnerActor :type Actor%20Object%20Reference))
  ;[1 1 1] GoToRallyPoint
  (bind _asbp_mech_bot (Utilities|Casting|CastToBP_MechBot OwnerActor)
    (:then
      (AI|AIMoveTo (Pawn|GetControlledPawn _asbp_mech_bot) "0, 0, 0" (AI|BehaviorTree|GetBlackboardValueasActor (Variables|Default|GetRallyPoint)) 16.0 false
        (:OnSuccess
          _)
        (:OnFail
          _))
      (Variables|/Game/Blueprints/AI/BP_MechBot.BP_MechBot_C|SetbMoveToRally _asbp_mech_bot false)
      (Class|BTFunctionLibrary|SetBlackboardValueasObject (Variables|Default|GetRallyPoint))
      (Class|BTFunctionLibrary|SetBlackboardValueasBool (Variables|Default|GetGoToRally) false))
    (:CastFailed
      _))
  (AI|BehaviorTree|FinishExecute true))

(event EventReceiveAbort
  (params (OwnerActor :type Actor%20Object%20Reference))
  (Class|BTFunctionLibrary|SetBlackboardValueasBool (Variables|Default|GetGoToRally) false))