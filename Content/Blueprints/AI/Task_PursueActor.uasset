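; Behavior tree task that sends a BP_Mech pawn after the actor in the Follow blackboard key.
; On execute it sets the BP_MechBot controller's Destination to the pawn's current location, then runs AIMoveTo, finishing successfully even if the move fails.
; Each tick it stops movement once the mech can see the followed BP_OpulentiumActor and is within about two-thirds of its TriggerRadius.
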(event EventReceiveExecuteAI
  (params (OwnerController :type AI%20Controller%20Object%20Reference) (ControlledPawn :type Pawn%20Object%20Reference))
  (bind _asbp_mech_bot (Utilities|Casting|CastToBP_MechBot OwnerController))
  (Variables|/Game/Blueprints/AI/BP_MechBot.BP_MechBot_C|SetDestination _asbp_mech_bot (Transformation|GetActorLocation ControlledPawn))
  (bind _asbp_mech (Utilities|Casting|CastToBP_Mech ControlledPawn))
  (AI|AIMoveTo ControlledPawn "0, 0, 0" (AI|BehaviorTree|GetBlackboardValueasActor (Variables|Default|GetFollow)) 128.0 false
    (:OnSuccess
      _)
    (:OnFail
      _))
  (AI|BehaviorTree|FinishExecute true))

(event EventReceiveTickAI
  (params (OwnerController :type AI%20Controller%20Object%20Reference) (ControlledPawn :type Pawn%20Object%20Reference) (DeltaSeconds :type Float%20%28single-precision%29))
  (bind _asbp_opulentium_actor (Utilities|Casting|CastToBP_OpulentiumActor (AI|BehaviorTree|GetBlackboardValueasActor (Variables|Default|GetFollow))))
  (if (and (Default|CanSeeActor (stale EventReceiveExecuteAI _asbp_mech) _asbp_opulentium_actor) (<= (Transformation|GetDistanceTo ControlledPawn _asbp_opulentium_actor) (* (Variables|/Script/Engine.SphereComponent|GetSphereRadius (Variables|/Game/Blueprints/BP_CombatActor.BP_CombatActor_C|GetTriggerRadius (stale EventReceiveExecuteAI _asbp_mech))) 0.67)))
    (AI|Navigation|StopMovement OwnerController)))