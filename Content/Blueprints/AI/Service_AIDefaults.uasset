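; Behavior Tree service that feeds Opulentium AI building orders from CommandInfo into the Blackboard.
; On activation it caches the AI controller and primary pawn, then each tick sets BBuild if any build flag is active.
; For Command Centre orders, it sets the structure class and places it at the territory's averaged core deposit position.
; The Destination is offset from that point, rotated by a look-at from the summed deposit position to the pawn.
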(event EventReceiveTickAI
  (params (OwnerController :type AI%20Controller%20Object%20Reference) (ControlledPawn :type Pawn%20Object%20Reference) (DeltaSeconds :type Float%20%28single-precision%29))
  (bind _ai (Variables|Default|GetAI)
    (:then
      (bind _primary (Variables|Default|GetPrimary)
        (:then
          (Class|BTFunctionLibrary|SetBlackboardValueasBool (Variables|Default|GetbBuild) (Math|Boolean|ORBoolean (.bCommandCentre (Utilities|Struct|BreakAICommands (Variables|/Game/Blueprints/BP_OpulentiumAI.BP_OpulentiumAI_C|GetCommandInfo _ai))) (.bCoreHelium (Utilities|Struct|BreakAICommands (Variables|/Game/Blueprints/BP_OpulentiumAI.BP_OpulentiumAI_C|GetCommandInfo _ai))) (.bBuildFactory (Utilities|Struct|BreakAICommands (Variables|/Game/Blueprints/BP_OpulentiumAI.BP_OpulentiumAI_C|GetCommandInfo _ai)))))
          (if (.bCommandCentre (Utilities|Struct|BreakAICommands (Variables|/Game/Blueprints/BP_OpulentiumAI.BP_OpulentiumAI_C|GetCommandInfo _ai)))
            (Class|BTFunctionLibrary|SetBlackboardValueasClass (Variables|Default|GetStructureClass) (Variables|/Game/Blueprints/BP_PlayerPrimary.BP_PlayerPrimary_C|GetCommandCentreBP_Build _primary))
            (bind _currentterritory (Variables|/Game/Blueprints/BP_OpulentiumAI.BP_OpulentiumAI_C|GetCurrentTerritory _ai)
              (:then
                (for _array_element (Default|GetCoreDeposits _ai _currentterritory)
                  (Variables|Default|SetCorePos (+ (Variables|Default|GetCorePos) (Transformation|GetActorLocation _array_element))))
                (AI|BehaviorTree|SetBlackboardValueasVector (Variables|Default|GetStructureLocation) (/ (Variables|Default|GetCorePos) (Utilities|Array|Length (Default|GetCoreDeposits _ai _currentterritory))))
                (AI|BehaviorTree|SetBlackboardValueasVector (Variables|Default|GetDestination) (+ (/ (Variables|Default|GetCorePos) (Utilities|Array|Length (Default|GetCoreDeposits _ai _currentterritory))) (Math|Vector|RotateVector "512.000000, 0, 0" (Math|Rotator|FindLookatRotation (Variables|Default|GetCorePos) (Transformation|GetActorLocation _primary)))))
                (Variables|Default|SetCorePos "0, 0, 0"))
              (:else))))
        (:else)))
    (:else)))

(event EventReceiveActivationAI
  (params (OwnerController :type AI%20Controller%20Object%20Reference) (ControlledPawn :type Pawn%20Object%20Reference))
  (bind _asbp_opulentium_ai (Utilities|Casting|CastToBP_OpulentiumAI OwnerController))
  (Variables|Default|SetAI _asbp_opulentium_ai)
  (bind _asbp_player_primary (Utilities|Casting|CastToBP_PlayerPrimary ControlledPawn))
  (Variables|Default|SetPrimary _asbp_player_primary))