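; Behavior tree task that moves a BP_MechBot's controlled pawn and advances its patrol index.
; It requires the Patrol blackboard value to be a BP_PatrolTo, but the AI move targets the bot's FollowActor.
; On either success or failure, it increments PatrolOrder, resetting to zero at PatrolChain length minus two, and finishes successfully.
; A failed cast stops execution without finishing the task.
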(event EventReceiveExecute
  (params (OwnerActor :type Actor%20Object%20Reference))
  (bind _asbp_mech_bot (Utilities|Casting|CastToBP_MechBot OwnerActor))
  (Utilities|Casting|CastToBP_PatrolTo (Class|BTFunctionLibrary|GetBlackboardValueasObject (Variables|Default|GetPatrol)))
  (AI|AIMoveTo (Pawn|GetControlledPawn _asbp_mech_bot) "0, 0, 0" (Variables|/Game/Blueprints/AI/BP_MechBot.BP_MechBot_C|GetFollowActor _asbp_mech_bot) 32.0 false
    (:OnSuccess
      _)
    (:OnFail
      _))
  (if (>= (Variables|/Game/Blueprints/AI/BP_MechBot.BP_MechBot_C|GetPatrolOrder _asbp_mech_bot) (- (Utilities|Array|Length (Variables|/Game/Blueprints/AI/BP_MechBot.BP_MechBot_C|GetPatrolChain _asbp_mech_bot)) 2))
    (Variables|/Game/Blueprints/AI/BP_MechBot.BP_MechBot_C|SetPatrolOrder _asbp_mech_bot 0)
    (else
      (Variables|/Game/Blueprints/AI/BP_MechBot.BP_MechBot_C|SetPatrolOrder _asbp_mech_bot (+ (Variables|/Game/Blueprints/AI/BP_MechBot.BP_MechBot_C|GetPatrolOrder _asbp_mech_bot) 1))))
  (AI|BehaviorTree|FinishExecute true))