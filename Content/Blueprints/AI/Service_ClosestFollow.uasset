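; AI service that picks which follow point a bot-controlled mech should take around its parent mech.
; Each tick it copies the parent's follow points, dropping invalid ones and any nearly on top of the parent.
; It also drops points that another follower's bot already targets from a closer position.
; The nearest remaining point becomes the bot controller's FollowActor.
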(event EventReceiveActivation
  (params (OwnerActor :type Actor%20Object%20Reference))
  (bind _asbp_mech_bot (Utilities|Casting|CastToBP_MechBot OwnerActor))
  (bind _asbp_mech (Utilities|Casting|CastToBP_Mech (Pawn|GetControlledPawn _asbp_mech_bot)))
  (Variables|Default|SetMech _asbp_mech))

(event EventTick
  (params (OwnerActor :type Actor%20Object%20Reference) (DeltaSeconds :type Float%20%28single-precision%29))
  (bind _mech (Variables|Default|GetMech)
    (:then
      (bind _parent (Variables|/Game/Blueprints/BP_CombatActor.BP_CombatActor_C|GetParent _mech)
        (:then
          (bind _output_get (Variables|Default|SetValidArray (Variables|/Game/Blueprints/BP_CombatActor.BP_CombatActor_C|GetFollowPoints _parent)))
          (bind _output_get_2 (Variables|Default|SetLocalArray _output_get))
          (for _array_element _output_get_2
            (Utilities|IsValid _array_element
              (:Is%20Valid
                (if (< (Transformation|GetDistanceTo _array_element _parent) 5.0)
                  (Utilities|Array|RemoveItem _output_get _array_element :!label _label)))
              (:Is%20Not%20Valid
                (goto _label))))
          (for _array_element_2 (Variables|/Game/Blueprints/BP_CombatActor.BP_CombatActor_C|GetFollowActors _parent)
            (if (!= _array_element_2 _mech)
              (bind _output_get_3 (Variables|Default|SetLocalArray _output_get))
              (for _array_element_3 _output_get_3
                (Utilities|IsValid (Pawn|GetController _array_element_2)
                  (:Is%20Valid
                    (bind _asbp_mech_bot (Utilities|Casting|CastToBP_MechBot (Pawn|GetController _array_element_2)))
                    (if (and (< (Transformation|GetDistanceTo _array_element_3 _array_element_2) (Transformation|GetDistanceTo _array_element_3 _mech)) (== (Variables|/Game/Blueprints/AI/BP_MechBot.BP_MechBot_C|GetFollowActor _asbp_mech_bot) _array_element_3))
                      (Utilities|Array|RemoveItem _output_get _array_element_3)))))))
          (for (_array_element_4 _array_index) _output_get
            (if (== _array_index 0)
              (bind _output_get_4 (Variables|Default|SetClosest _array_element_4))
              (bind _output_get_5 (Variables|Default|SetDistance (Transformation|GetDistanceTo _array_element_4 _mech)))
              (elif (< (Transformation|GetDistanceTo _array_element_4 _mech) _output_get_5)
                (Variables|Default|SetClosest _array_element_4)
                (Variables|Default|SetDistance (Transformation|GetDistanceTo _array_element_4 _mech)))))
          (Utilities|IsValid _output_get_4
            (:Is%20Valid
              (Variables|/Game/Blueprints/AI/BP_MechBot.BP_MechBot_C|SetFollowActor (stale EventReceiveActivation _asbp_mech_bot) _output_get_4))))
        (:else)))
    (:else)))