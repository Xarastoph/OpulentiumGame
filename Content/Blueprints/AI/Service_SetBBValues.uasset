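; Behavior tree service that mirrors BP_MechBot's order state into the Blackboard for the mech bot's AI.
; On activation it seeds the rally keys and picks a random debug colour.
; Each tick it copies rally, move, patrol, follow and idle state, selecting the rally and follow objects by their conditions.
; It also draws a debug sphere at the controlled pawn and prints the states in that colour.
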(event EventReceiveActivation
  (params (OwnerActor :type Actor%20Object%20Reference))
  (bind _returnvalue (Math|Random|RandomFloat))
  (bind _returnvalue_2 (Math|Random|RandomFloat))
  (bind _returnvalue_3 (- 1.0 _returnvalue_2))
  (bind _returnvalue_4 (* _returnvalue_3 _returnvalue))
  ;[1 1 1] SetConditions
  (bind _asbp_mech_bot (Utilities|Casting|CastToBP_MechBot OwnerActor))
  (Class|BTFunctionLibrary|SetBlackboardValueasObject (Variables|Default|GetRallyPoint) (Variables|/Game/Blueprints/AI/BP_MechBot.BP_MechBot_C|GetRallyPoint _asbp_mech_bot))
  (Class|BTFunctionLibrary|SetBlackboardValueasBool (Variables|Default|GetGoToRally) (Variables|/Game/Blueprints/AI/BP_MechBot.BP_MechBot_C|GetbMoveToRally _asbp_mech_bot))
  (bind _output_get (Variables|Default|SetRandColour (Math|Color|MakeColor _returnvalue_2 _returnvalue_4 (- _returnvalue _returnvalue_4) 1.0))))

(event EventTick
  (params (OwnerActor :type Actor%20Object%20Reference) (DeltaSeconds :type Float%20%28single-precision%29))
  (bind _asbp_mech_bot (Utilities|Casting|CastToBP_MechBot OwnerActor))
  (Class|BTFunctionLibrary|SetBlackboardValueasBool (Variables|Default|GetGoToRally) (Variables|/Game/Blueprints/AI/BP_MechBot.BP_MechBot_C|GetbMoveToRally _asbp_mech_bot))
  (Class|BTFunctionLibrary|SetBlackboardValueasObject (Variables|Default|GetRallyPoint) (Utilities|SelectObject (Variables|/Game/Blueprints/AI/BP_MechBot.BP_MechBot_C|GetRallyPoint _asbp_mech_bot) 0 (Variables|/Game/Blueprints/AI/BP_MechBot.BP_MechBot_C|GetbMoveToRally _asbp_mech_bot)))
  (Class|BTFunctionLibrary|SetBlackboardValueasBool (Variables|Default|GetMoveToPoint) (Variables|/Game/Blueprints/AI/BP_MechBot.BP_MechBot_C|GetbMoving _asbp_mech_bot))
  (Class|BTFunctionLibrary|SetBlackboardValueasBool (Variables|Default|GetPatrol) (Variables|/Game/Blueprints/AI/BP_MechBot.BP_MechBot_C|GetbPatrol _asbp_mech_bot))
  (Class|BTFunctionLibrary|SetBlackboardValueasBool (Variables|Default|GetFollowing) (Variables|/Game/Blueprints/AI/BP_MechBot.BP_MechBot_C|GetbFollowActor _asbp_mech_bot))
  (Class|BTFunctionLibrary|SetBlackboardValueasObject (Variables|Default|GetFollowActor) (Utilities|SelectObject (Variables|/Game/Blueprints/AI/BP_MechBot.BP_MechBot_C|GetFollowActor _asbp_mech_bot) 0 (Variables|/Game/Blueprints/AI/BP_MechBot.BP_MechBot_C|GetbFollowActor _asbp_mech_bot)))
  (Class|BTFunctionLibrary|SetBlackboardValueasBool (Variables|Default|GetIdle) (Variables|/Game/Blueprints/AI/BP_MechBot.BP_MechBot_C|GetbIdle _asbp_mech_bot))
  (Rendering|Debug|DrawDebugSphere (Transformation|GetActorLocation (Pawn|GetControlledPawn _asbp_mech_bot)) 128.0 12 (stale EventReceiveActivation _output_get) 0.1)
  (Development|PrintString (Utilities|String|Append "Rally: " (Utilities|String|ToString(Boolean) (Variables|/Game/Blueprints/AI/BP_MechBot.BP_MechBot_C|GetbMoveToRally _asbp_mech_bot))) true true (stale EventReceiveActivation _output_get) 0.05)
  (Development|PrintString (Utilities|String|Append "MoveTo: " (Utilities|String|ToString(Boolean) (Variables|/Game/Blueprints/AI/BP_MechBot.BP_MechBot_C|GetbMoving _asbp_mech_bot))) true true (stale EventReceiveActivation _output_get) 0.05)
  (Development|PrintString (Utilities|String|Append "Follow: " (Utilities|String|ToString(Boolean) (Variables|/Game/Blueprints/AI/BP_MechBot.BP_MechBot_C|GetbFollowActor _asbp_mech_bot))) true true (stale EventReceiveActivation _output_get) 0.05)
  (Development|PrintString (Utilities|String|Append "Patrol: " (Utilities|String|ToString(Boolean) (Variables|/Game/Blueprints/AI/BP_MechBot.BP_MechBot_C|GetbPatrol _asbp_mech_bot))) true true (stale EventReceiveActivation _output_get) 0.05)
  (Development|PrintString (Utilities|String|Append "Idle: " (Utilities|String|ToString(Boolean) (Variables|/Game/Blueprints/AI/BP_MechBot.BP_MechBot_C|GetbIdle _asbp_mech_bot))) true true (stale EventReceiveActivation _output_get) 0.05)
  (Development|PrintString "" true true (stale EventReceiveActivation _output_get) 0.05))