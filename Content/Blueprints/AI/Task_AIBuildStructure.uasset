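; Behavior tree task that has the Opulentium AI build the structure class stored in the blackboard at the blackboard location.
; It checks the class's build cost against the AI's He3, retrying every second until affordable.
; It then spawns the structure raised by its root offset, clears the Structure key, spends the He3, resets the build flag and finishes successfully.
; Failed casts also finish as success.
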(event EventReceiveExecuteAI
  (params (OwnerController :type AI%20Controller%20Object%20Reference) (ControlledPawn :type Pawn%20Object%20Reference))
  (bind _asbp_structure_build (Utilities|Casting|CastToBP_StructureBuildClass (Class|BTFunctionLibrary|GetBlackboardValueasClass (Variables|Default|GetStructure)))
    (:then
      (if (Utilities|IsValidClass _asbp_structure_build)
        (bind _asbp_opulentium_ai (Utilities|Casting|CastToBP_OpulentiumAI OwnerController)
          (:then
            (if (<= (.BuildCost (Utilities|GetClassDefaults _asbp_structure_build)) (Variables|/Game/Blueprints/BP_OpulentiumAI.BP_OpulentiumAI_C|GetHe3 _asbp_opulentium_ai)) :!label _label
              (Default|SpawnStructure _asbp_opulentium_ai _asbp_structure_build (+ (Class|BTFunctionLibrary|GetBlackboardValueasVector (Variables|Default|GetLocation)) (Math|Vector|MakeVector 0.0 0.0 (.RootOffset (Utilities|GetClassDefaults _asbp_structure_build)))))
              (Class|BTFunctionLibrary|SetBlackboardValueasClass (Variables|Default|GetStructure))
              (Default|SpendHe3 _asbp_opulentium_ai (.BuildCost (Utilities|GetClassDefaults _asbp_structure_build)))
              (Class|BTFunctionLibrary|SetBlackboardValueasBool (Variables|Default|GetbBuild) false)
              (else
                (Utilities|FlowControl|Delay 1.0)
                (goto _label))))
          (:CastFailed
            _))
        (AI|BehaviorTree|FinishExecute true :!label _label_2)))
    (:CastFailed
      (goto _label_2))))