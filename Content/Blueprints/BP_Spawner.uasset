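; Spawner actor that keeps one instance of a configurable class alive at its transform, respawning it after it becomes invalid.
; On BeginPlay it spawns immediately, passing a fixed team and applying configured health and shields.
; A looping timer polls the spawned reference and respawns after a delay while the tally is within SpawnMax.
; Negative SpawnMax means unlimited; exceeding the limit clears the timer.
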(event Custom|SpawnCheck
  (bind _spawnmax (Variables|Default|GetSpawnMax))
  (if (or (<= (Variables|Default|GetSpawnTally) _spawnmax) (< _spawnmax 0))
    (Variables|Default|GetSpawned
      (:then)
      (:else
        (Utilities|FlowControl|Delay (Variables|Default|GetRespawnTime))
        (CallFunction|Spawn)))
    (else
      (Class|KismetSystemLibrary|ClearTimerHandle (stale EventBeginPlay _returnvalue)))))

(event Custom|Spawn
  (bind _returnvalue (Game|SpawnActorfromClass (Variables|Default|GetSpawnClass) (Transformation|GetActorTransform) "AdjustIfPossibleButDontSpawnIfColliding" 0 0 256))
  (Utilities|IsValid _returnvalue
    (:Is%20Valid
      (Variables|/Game/Blueprints/BP_OpulentiumActor.BP_OpulentiumActor_C|SetHealthMax _returnvalue (Variables|Default|GetHealth))
      (Variables|/Game/Blueprints/BP_OpulentiumActor.BP_OpulentiumActor_C|SetHealth _returnvalue (Variables|Default|GetHealth))
      (Variables|/Game/Blueprints/BP_CombatActor.BP_CombatActor_C|SetShields _returnvalue (Variables|Default|GetShields))
      (Variables|/Game/Blueprints/BP_CombatActor.BP_CombatActor_C|SetShieldsMax _returnvalue (Variables|Default|GetShields))
      (Variables|Default|SetSpawned _returnvalue)
      (Math|Integer|IncrementInt (Variables|Default|GetSpawnTally)))))

(event EventBeginPlay
  (CallFunction|Spawn)
  (bind _returnvalue (Utilities|Time|SetTimerbyEvent (delegate Custom|SpawnCheck) 0.5 true)))

(fn ConstructionScript)

(fn OnRepSpawnTally)