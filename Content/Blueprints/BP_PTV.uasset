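; BP_PTV is a player-controlled Blueprint that tracks firing input and steers projectiles toward the camera's aim point.
; Either mouse button sets the shooting state and its own blend time; a timer clears the state five seconds after both are released.
; SpawnTrackActor places a dummy actor at the camera trace's hit or end point as the projectile's homing target.
; The trace ignores the game mode's Territories.
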(event Custom|ResetShooting
  (Variables|Default|SetbShooting false))

(event Input|MouseEvents|RightMouseButton
  (params (Key :type Key%20Structure :default "AnyKey"))
  (:Pressed
    (bind _output_get (Variables|Default|SetbRMB true))
    (Variables|Default|SetBlendTime 0.5)
    (Variables|Default|SetbShooting true)
    (Class|KismetSystemLibrary|ClearTimerHandle (stale _returnvalue)))
  (:Released
    (Variables|Default|SetbRMB false)
    (if (Math|Boolean|NORBoolean (stale Input|MouseEvents|LeftMouseButton _output_get) _output_get)
      (bind _returnvalue (Utilities|Time|SetTimerbyEvent (delegate Custom|ResetShooting) 5.0)))))

(event Input|MouseEvents|LeftMouseButton
  (params (Key :type Key%20Structure :default "AnyKey"))
  (:Pressed
    (bind _output_get (Variables|Default|SetbLMB true))
    (Variables|Default|SetBlendTime 0.2)
    (Variables|Default|SetbShooting true)
    (Class|KismetSystemLibrary|ClearTimerHandle (stale _returnvalue)))
  (:Released
    (Variables|Default|SetbLMB false)
    (if (Math|Boolean|NORBoolean _output_get (stale Input|MouseEvents|RightMouseButton _output_get))
      (bind _returnvalue (Utilities|Time|SetTimerbyEvent (delegate Custom|ResetShooting) 5.0)))))

(fn ConstructionScript)

(fn SpawnTrackActor
  (params (Projectile :type BP%20Projectile%20Object%20Reference))
  (bind _hitinfo (CallFunction|VisionTrace))
  (bind (_bblockinghit _binitialoverlap _time _location _impactpoint _normal _impactnormal _physmat _hitactor _hitcomponent _hitbonename _hititem _tracestart _traceend) (Collision|BreakHitResult _hitinfo))
  (if (Math|Vector|NotEqual(Vector) _location "0, 0, 0" 0.0001)
    (bind _output_get (LocalVariables|SetLocalPos _location))
    (else
      (LocalVariables|SetLocalPos _traceend)))
  (bind _returnvalue (Game|SpawnActorfromClass "/Game/Blueprints/DummyActor.DummyActor_C" (Math|Conversions|ToTransform(Vector) _output_get) "Undefined" 0 0))
  (Utilities|IsValid _returnvalue
    (:Is%20Valid
      (Variables|/Script/Engine.ProjectileMovementComponent|SetHomingTargetComponent (Variables|/Game/Blueprints/BP_Projectile.BP_Projectile_C|GetProjectileMovement Projectile) (VehicleSound|GetRootComponent _returnvalue))
      (Variables|/Game/Blueprints/BP_Projectile.BP_Projectile_C|SetTrackActor Projectile _returnvalue))))

(fn VisionTrace
  (bind _camera (Variables|Default|GetCamera))
  (bind _returnvalue (Transformation|GetWorldLocation _camera))
  (bind _asbp_opulentium (Utilities|Casting|CastToBP_Opulentium (Game|GetGameMode))
    (:then
      _)
    (:CastFailed
      _))
  (bind _outhit (Collision|LineTraceByChannel _returnvalue (+ _returnvalue (Math|Vector|RotateVector (Math|Vector|MakeVector 1e+04 0.0 0.0) (Transformation|GetWorldRotation _camera))) "TraceTypeQuery1" false (Variables|/Game/Blueprints/BP_Opulentium.BP_Opulentium_C|GetTerritories _asbp_opulentium) "None"))
  (return _outhit))