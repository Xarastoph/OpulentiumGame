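; Placeholder actor for a unit under construction, which spawns the built mech and then destroys itself.
; A Build timeline scaled by BuildTime animates the build material, then spawns if the overlap area is clear, with CanSpawn's RepNotify retrying once unblocked.
; The new unit joins its owner's team and Owned list, and its bot controller receives the rally point.
; On destruction, unless cancelled, it updates the Builder's build queue.
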(event OnComponentBeginOverlap(OverlapMesh)
  (params (OtherActor :type Actor%20Object%20Reference) (OtherComp :type Primitive%20Component%20Object%20Reference) (OtherBodyIndex :type Integer) (bFromSweep :type Boolean) (SweepResult :type Hit%20Result%20Structure%20%28by%20ref%29))
  (if (and (!= OtherActor (Variables|Default|GetBuilder)) (not (.bSuccess (Utilities|Casting|CastToBP_Projectile OtherActor))))
    (Variables|Default|SetbCanSpawn false)))

(event OnComponentEndOverlap(OverlapMesh)
  (params (OtherActor :type Actor%20Object%20Reference) (OtherComp :type Primitive%20Component%20Object%20Reference) (OtherBodyIndex :type Integer))
  (Variables|Default|SetbCanSpawn true))

(event Custom|SpawnMech
  (bind _returnvalue (Transformation|GetActorTransform))
  (bind (_location _rotation _scale) (Math|Transform|BreakTransform _returnvalue))
  (Utilities|FlowControl|DoOnce false
    (:Completed
      (bind _primaryowner (Variables|Default|GetPrimaryOwner)
        (:then
          (bind _returnvalue_2 (Game|SpawnActorfromClass (Variables|Default|GetBuildClass) (Math|Transform|MakeTransform (+ _location (Math|Vector|MakeVector 0.0 0.0 (Variables|Default|GetZOffset))) _rotation _scale) "AlwaysSpawn" (Components|GetOwner) _primaryowner (Variables|/Game/Blueprints/BP_OpulentiumActor.BP_OpulentiumActor_C|GetTeam _primaryowner)))
          (Utilities|IsValid _returnvalue_2
            (:Is%20Valid
              (Utilities|Array|Add (Variables|/Game/Blueprints/BP_PlayerPrimary.BP_PlayerPrimary_C|GetOwned _primaryowner) _returnvalue_2)
              (bind _asbp_mech_bot (Utilities|Casting|CastToBP_MechBot (Pawn|GetController _returnvalue_2))
                (:then
                  (Variables|/Game/Blueprints/AI/BP_MechBot.BP_MechBot_C|SetDestination _asbp_mech_bot (Transformation|GetActorLocation (Variables|Default|GetRallyPoint)))
                  (Variables|/Game/Blueprints/AI/BP_MechBot.BP_MechBot_C|SetRallyPoint _asbp_mech_bot (Variables|Default|GetRallyPoint)))
                (:CastFailed
                  _))
              (Actor|DestroyActor))))
        (:else)))))

(event EventBeginPlay
  (bind _returnvalue (Rendering|Material|CreateDynamicMaterialInstance (Variables|Default|GetBuildMesh) 0 "/Game/Environment/Materials/Static/GreenStaticPanner_Inst.GreenStaticPanner_Inst" :!class /Script/Engine.PrimitiveComponent))
  (Components|Timeline|SetPlayRate (Variables|Default|GetBuild) (/ 1.0 (Variables|Default|GetBuildTime)))
  (bind _time (Timeline|Build Play)
    (:Update
      (Rendering|Material|SetScalarParameterValue _returnvalue "Time" _time :!class /Script/Engine.MaterialInstanceDynamic))
    (:Finished
      (bind _builder (Variables|Default|GetBuilder)
        (:then
          (Variables|/Game/Blueprints/BP_Builder.BP_Builder_C|SetCurrentType _builder "NewEnumerator3")
          (if (Variables|Default|GetbCanSpawn)
            (CallFunction|SpawnMech)))
        (:else)))))

(event EventDestroyed
  (if (not (Variables|Default|GetbCancel))
    (bind _builder (Variables|Default|GetBuilder)
      (:then
        (Default|SetBuildQueue _builder))
      (:else))))

(fn ConstructionScript)

(fn OnRepBCanSpawn
  (if (Math|Boolean|ANDBoolean (not (Components|Activation|IsActive (Variables|Default|GetBuild))) (Variables|Default|GetbCanSpawn) (Utilities|IsValid (Variables|Default|GetBuilder)))
    (CallFunction|SpawnMech)))