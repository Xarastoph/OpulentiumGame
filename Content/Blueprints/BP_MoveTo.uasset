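; BP_MoveTo is a destination marker that the player places to order mechs around.
; While locating, it tracks the owner's vision trace, switching to a follow marker over owned mechs and hiding over patrol points.
; Once placed, it destroys itself if following or unused by mechs' moves and chains, and auto-hides unless a mech is selected or looked at.
; On destruction, it advances mechs to their next queued MoveTo unless terminated.
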(event Custom|Hide
  ;[1 1 1] Set Visibility
  (Rendering|SetActorHiddenInGame true))

(event Custom|ChangeVisibility
  (params (bFollowMarker :type Boolean :default false))
  (bind _self self)
  (bind _followmarker (Variables|Default|GetFollowMarker))
  ;[1 1 1] Change Visibility
  (if (Variables|Default|GetbHide)
    (Rendering|SetActorHiddenInGame _self true)
    (else
      (Rendering|SetActorHiddenInGame _self false)
      (if bFollowMarker
        (Development|SetHiddeninGame _followmarker false false)
        (Development|SetHiddeninGame true false)
        (else
          (Development|SetHiddeninGame _followmarker true false)
          (Development|SetHiddeninGame false false))))))

(event EventTick
  (params (DeltaSeconds :type Float%20%28single-precision%29))
  (bind _blocating (Variables|Default|GetbLocating))
  ;[1 1 1] Set Location
  (Variables|Default|SetbPendKill true)
  (if (Variables|Default|GetbLocating)
    (bind _primaryowner (Variables|Default|GetPrimaryOwner)
      (:then
        (Variables|Default|SetbHide (.bSuccess (Utilities|Casting|CastToBP_PatrolTo (.HitActor (Collision|BreakHitResult (Default|VisionTrace _primaryowner))))))
        (bind _bvalid (CallFunction|TestforTarget (.HitActor (Collision|BreakHitResult (Default|VisionTrace _primaryowner)))))
        (if _bvalid
          (Transformation|SetActorLocation (+ (Transformation|GetActorLocation (.HitActor (Collision|BreakHitResult (Default|VisionTrace _primaryowner)))) (Math|Vector|MakeVector 0.0 0.0 (.Z (Math|Vector|BreakVector (.BoxExtent (Collision|GetActorBounds (.HitActor (Collision|BreakHitResult (Default|VisionTrace _primaryowner))) false)))))) false false)
          (Variables|Default|SetCurrentTarget (.HitActor (Collision|BreakHitResult (Default|VisionTrace _primaryowner))))
          (CallFunction|ChangeVisibility true)
          (Variables|Default|SetbFollowing true)
          (else
            (Transformation|SetActorLocation (.Location (Collision|BreakHitResult (Default|VisionTrace _primaryowner))) false false)
            (Variables|Default|SetCurrentTarget 0)
            (CallFunction|ChangeVisibility false)
            (Variables|Default|SetbFollowing false)))
        ;[1 1 1] Kill Test
        (for _array_element (Variables|Default|GetMechs) :!label _label
          (Utilities|IsValid _array_element
            (:Is%20Valid
              (bind _asbp_mech_bot (Utilities|Casting|CastToBP_MechBot (Pawn|GetController _array_element)))
              (if (and (Variables|/Game/Blueprints/AI/BP_MechBot.BP_MechBot_C|GetbMoving _asbp_mech_bot) (== (Variables|/Game/Blueprints/AI/BP_MechBot.BP_MechBot_C|GetCurrentMoveTo _asbp_mech_bot) self))
                (Variables|Default|SetbPendKill false :!label _label_2)
                (elif (CallFunction|InChain _asbp_mech_bot)
                  (goto _label_2))))))
        (if (Variables|Default|GetbPendKill)
          (if _blocating
            ;[1 1 1] Set Visibility
            (Class|KismetSystemLibrary|ClearTimerHandle (stale _returnvalue) :!label _label_3)
            (Rendering|SetActorHiddenInGame (Variables|Default|GetbHide))
            (else
              (Actor|DestroyActor :!label _label_4)))
          (elif _blocating
            (goto _label_3)
            (else
              (if (Utilities|Time|IsTimerActivebyHandle (stale _returnvalue))
                _
                (else
                  (bind _returnvalue (Utilities|Time|SetTimerbyEvent (delegate Custom|Hide) 3.0))))
              (bind _asbp_player_primary (Utilities|Casting|CastToBP_PlayerPrimary (Components|GetOwner)))
              (for _array_element_2 (Variables|Default|GetMechs)
                (if (== (Variables|/Game/Blueprints/BP_PlayerPrimary.BP_PlayerPrimary_C|GetLookatObject _asbp_player_primary) _array_element_2)
                  (goto _label_3)
                  (elif (Variables|/Game/Blueprints/BP_OpulentiumActor.BP_OpulentiumActor_C|GetbSelected _array_element_2)
                    (goto _label_3))))
              (if (Variables|Default|GetbLocating)
                (goto _label_3))))))
      (:else))
    (elif (Variables|Default|GetbFollowing)
      (goto _label_4)
      (else
        (goto _label)))))

(event EventBeginPlay
  ;[1 1 1] Set Location
  (bind _asbp_player_primary (Utilities|Casting|CastToBP_PlayerPrimary (Components|GetOwner)))
  (Variables|Default|SetPrimaryOwner _asbp_player_primary))

(event EventDestroyed
  ;[1 1 1] Kill Test
  ;;[1 1 1] Destroyed
  (CallFunction|GetNextMoveto))

(fn ConstructionScript)

(fn TestforTarget
  (params (TestActor :type Actor%20Object%20Reference))
  ;[1 1 1] Find Closest Mech
  (bind _asbp_mech (Utilities|Casting|CastToBP_Mech TestActor)
    (:then
      (bind _output_get (LocalVariables|SetbLocalValid (== (Variables|/Game/Blueprints/BP_Mech.BP_Mech_C|GetPrimaryOwner _asbp_mech) (Variables|Default|GetPrimaryOwner)))))
    (:CastFailed
      (LocalVariables|SetbLocalValid false)))
  (return _output_get))

(fn InChain
  (params (Bot :type BP%20Mech%20Bot%20Object%20Reference))
  (LocalVariables|SetbValid false)
  (bind _array_element (Utilities|Array|ForEachLoopwithBreak (Variables|/Game/Blueprints/AI/BP_MechBot.BP_MechBot_C|GetMoveToChain Bot) :!label _label)
    (:LoopBody
      (if (== (Utilities|Struct|BreakMoveToInfo _array_element) self)
        (bind _output_get (LocalVariables|SetbValid true))
        (goto _label Break)))
    (:Completed
      (return _output_get))))

(fn GetNextMoveto
  (bind _routed (LocalVariables|GetRouted))
  (if (not (Variables|Default|GetbTerminate))
    (for _array_element (Variables|Default|GetMechs)
      (bind _asbp_mech_bot (Utilities|Casting|CastToBP_MechBot (Pawn|GetController _array_element)))
      (bind _primaryowner (Variables|/Game/Blueprints/BP_Mech.BP_Mech_C|GetPrimaryOwner _array_element)
        (:then
          (if (and (Utilities|IsValid (Default|GetCurrentMoveto _asbp_mech_bot)) (not (Utilities|Array|ContainsItem _routed (Default|GetCurrentMoveto _asbp_mech_bot))))
            (Utilities|Array|Add _routed (Default|GetCurrentMoveto _asbp_mech_bot))
            (Default|SetDestination _primaryowner (Default|GetCurrentMoveto _asbp_mech_bot))
            (Default|SetNextMoveto _asbp_mech_bot)))
        (:else)))))