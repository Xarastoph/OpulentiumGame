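; BP_Structure is a base Blueprint for team-owned structures that spawn upgrade builds linked to their parent.
; SpawnUpgrade spawns the given class at UpgradeTransform, lowered by RootOffset, and sets itself as ParentStructure.
; Only when the structure is a BP_Conduit does it also record CurrentBuild and pass on its Team.
; ShowTree, SetPopulation, the construction script and the IconOffset RepNotify are empty here.
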(event Custom|SetPopulation)

(event Custom|SpawnUpgrade
  (params (BuildClass :type BP%20Upgrade%20Build%20Class%20Reference))
  (bind _self self)
  (bind _upgradetransform (Variables|Default|GetUpgradeTransform))
  (bind (_location _rotation _scale) (Math|Transform|BreakTransform _upgradetransform))
  (bind _returnvalue (Game|SpawnActorfromClass BuildClass (Math|Transform|MakeTransform (- _location (Math|Vector|MakeVector 0.0 0.0 (Variables|Default|GetRootOffset))) _rotation _scale) "AlwaysSpawn" (Components|GetOwner) 0))
  (Variables|/Game/Blueprints/BP_UpgradeBuild.BP_UpgradeBuild_C|SetParentStructure _returnvalue self)
  (CallFunction|SetParentStructure _self _returnvalue)
  (bind _asbp_conduit (Utilities|Casting|CastToBP_Conduit _self))
  (Variables|/Game/Blueprints/BP_Conduit.BP_Conduit_C|SetCurrentBuild _asbp_conduit _returnvalue)
  (Variables|/Game/Blueprints/BP_UpgradeBuild.BP_UpgradeBuild_C|SetTeam _returnvalue (Variables|Default|GetTeam)))

(event Custom|SetParentStructure
  (params (Build :type BP%20Upgrade%20Build%20Object%20Reference))
  (Variables|/Game/Blueprints/BP_UpgradeBuild.BP_UpgradeBuild_C|SetParentStructure Build self))

(event Custom|ShowTree)

(fn ConstructionScript)

(fn OnRepIconOffset)