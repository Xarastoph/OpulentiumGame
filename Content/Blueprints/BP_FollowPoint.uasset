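; BP_FollowPoint is an actor that keeps itself at an offset from its owner, oriented to the owner's direction of travel.
; Each tick, while the owner moves above a small speed threshold, it builds a rotation from the velocity plus a yaw offset.
; It rotates the Relative vector by that rotation and does a swept move to the owner's location plus the result.
; Below the threshold, its location is not updated.
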(event EventTick
  (params (DeltaSeconds :type Float%20%28single-precision%29))
  (bind _returnvalue (Components|GetOwner))
  (bind _returnvalue_2 (Transformation|GetVelocity _returnvalue))
  (Utilities|IsValid _returnvalue
    (:Is%20Valid
      (if (> (Math|Vector|VectorLength _returnvalue_2) 2e+01)
        (bind _output_get (Variables|Default|SetRotOffset (Math|Rotator|CombineRotators (Math|Rotator|MakeRotfromX _returnvalue_2) (Math|Rotator|MakeRotator 0.0 0.0 (Variables|Default|GetYawOffset)))))
        (Transformation|SetActorLocation (+ (Transformation|GetActorLocation _returnvalue) (Math|Vector|RotateVector (Variables|Default|GetRelative) _output_get)) true false)))))

(fn ConstructionScript)