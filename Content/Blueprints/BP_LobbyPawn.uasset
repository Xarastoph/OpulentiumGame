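; Lobby player character with standard move, turn, look and jump input, which also drives a starfield effect from the camera's orientation.
; On BeginPlay it caches the first BP_Starfield actor in the level.
; Each tick it stores the camera's world rotation in HeadRot and sets starfield intensity from the scaled magnitude of absolute pitch and yaw, so intensity follows view angle rather than turning speed.
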(event Custom|SetHeadRot
  (Variables|Default|SetHeadRot (Transformation|GetWorldRotation (Variables|Default|GetCamera))))

(event EventTick
  (params (DeltaSeconds :type Float%20%28single-precision%29))
  (bind _camera (Variables|Default|GetCamera))
  (bind _returnvalue (Transformation|GetWorldRotation _camera))
  (bind (_roll _pitch _yaw) (Math|Rotator|BreakRotator _returnvalue))
  (CallFunction|SetHeadRot)
  (bind _starfield (Variables|Default|GetStarField)
    (:then
      (Default|SetIntensity _starfield (/ (Math|Vector|VectorLength (Math|Vector|MakeVector (Math|Float|Absolute(Float) _pitch) (Math|Float|Absolute(Float) _yaw) 0.0)) 7.2e+02)))
    (:else)))

(event EventBeginPlay
  (bind _outactors (Actor|GetAllActorsOfClass "/Game/Environment/Objects/Planets/BP_Starfield.BP_Starfield_C"))
  (Variables|Default|SetStarField (Utilities|Array|Get(acopy) _outactors)))

(event Input|ActionEvents|InputActionJump
  (params (Key :type Key%20Structure :default "AnyKey"))
  (:Pressed
    (Character|Jump)))

(event Input|AxisEvents|InputAxisMoveForward
  (params (AxisValue :type Float%20%28single-precision%29))
  (Pawn|Input|AddMovementInput (Math|Vector|GetForwardVector (Math|Rotator|MakeRotator 0.0 0.0 (.Yaw (Math|Rotator|BreakRotator (Pawn|GetControlRotation :!class /Script/Engine.Pawn))))) AxisValue false))

(event Input|AxisEvents|InputAxisMoveRight
  (params (AxisValue :type Float%20%28single-precision%29))
  (Pawn|Input|AddMovementInput (Math|Vector|GetRightVector (Math|Rotator|MakeRotator 0.0 0.0 (.Yaw (Math|Rotator|BreakRotator (Pawn|GetControlRotation :!class /Script/Engine.Pawn))))) AxisValue false))

(event Input|AxisEvents|InputAxisTurn
  (params (AxisValue :type Float%20%28single-precision%29))
  (Pawn|Input|AddControllerYawInput AxisValue))

(event Input|AxisEvents|InputAxisLookUp
  (params (AxisValue :type Float%20%28single-precision%29))
  (Pawn|Input|AddControllerPitchInput AxisValue))

(fn ConstructionScript)