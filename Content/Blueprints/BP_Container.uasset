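; BP_Container is a storage structure that raises its owning player's He3 cap while it exists.
; On BeginPlay it adds He3CapBoost to the PrimaryOwner's PlayerController and increments the ContainerPop count in that controller's StructureCap struct.
; On Destroyed it reverses both changes, reaching the controller by casting its Owner to BP_OpulentiumPlayerController instead of going through PrimaryOwner.
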(event EventDestroyed
  ;[1 1 1] Destroyed
  (bind _asbp_opulentium_player_controller (Utilities|Casting|CastToBP_OpulentiumPlayerController (Components|GetOwner)))
  (bind _structout (Utilities|Struct|SetmembersinStructureCap (Variables|/Game/Blueprints/BP_OpulentiumPlayerController.BP_OpulentiumPlayerController_C|GetStructureCap _asbp_opulentium_player_controller) (- (Utilities|Struct|BreakStructureCap (Variables|/Game/Blueprints/BP_OpulentiumPlayerController.BP_OpulentiumPlayerController_C|GetStructureCap _asbp_opulentium_player_controller)) 1)))
  (Variables|/Game/Blueprints/BP_OpulentiumPlayerController.BP_OpulentiumPlayerController_C|SetStructureCap _asbp_opulentium_player_controller _structout)
  (Variables|/Game/Blueprints/BP_OpulentiumPlayerController.BP_OpulentiumPlayerController_C|SetHe3Cap _asbp_opulentium_player_controller (- (Variables|/Game/Blueprints/BP_OpulentiumPlayerController.BP_OpulentiumPlayerController_C|GetHe3Cap _asbp_opulentium_player_controller) (Variables|Default|GetHe3CapBoost))))

(event EventBeginPlay
  ;[1 1 1] Increase Cap
  (|CallParentFunction)
  (bind _primaryowner (Variables|Default|GetPrimaryOwner)
    (:then
      (bind _playercontroller (Variables|/Game/Blueprints/BP_PlayerPrimary.BP_PlayerPrimary_C|GetPlayerController _primaryowner)
        (:then
          (Variables|/Game/Blueprints/BP_OpulentiumPlayerController.BP_OpulentiumPlayerController_C|SetHe3Cap _playercontroller (+ (Variables|/Game/Blueprints/BP_OpulentiumPlayerController.BP_OpulentiumPlayerController_C|GetHe3Cap _playercontroller) (Variables|Default|GetHe3CapBoost)))
          (bind _structout (Utilities|Struct|SetmembersinStructureCap (Variables|/Game/Blueprints/BP_OpulentiumPlayerController.BP_OpulentiumPlayerController_C|GetStructureCap _playercontroller) (+ (Utilities|Struct|BreakStructureCap (Variables|/Game/Blueprints/BP_OpulentiumPlayerController.BP_OpulentiumPlayerController_C|GetStructureCap _playercontroller)) 1)))
          (Variables|/Game/Blueprints/BP_OpulentiumPlayerController.BP_OpulentiumPlayerController_C|SetStructureCap _playercontroller _structout))
        (:else)))
    (:else)))

(fn ConstructionScript
  (|CallParentFunction))