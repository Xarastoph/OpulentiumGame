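; AI controller for an RTS computer player that possesses BP_PlayerPrimary, runs BT_AI and tracks its He3 economy.
; A looping StatusCheck sets CommandInfo build priorities in order: command centre, helium deposit, then factory.
; Each pass also buys assault mechs for factory queues and sends squads of five idle mechs to an enemy command centre via BP_MoveTo.
; Territory is found by tracing upward into BP_TerritoryVolume; spawning a structure re-runs StatusCheck.
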(event Custom|SpawnStructure
  (params (Class :type BP%20Structure%20Build%20Class%20Reference) (Location :type Vector))
  (bind _primaryowner (Variables|Default|GetPrimaryOwner))
  (Game|SpawnActorfromClass Class (Math|Conversions|ToTransform(Vector) Location) "AlwaysSpawn" self _primaryowner (Variables|/Game/Blueprints/BP_OpulentiumActor.BP_OpulentiumActor_C|GetTeam _primaryowner))
  (CallFunction|StatusCheck))

(event Custom|SpendHe3
  (params (Amount :type Integer))
  (Variables|Default|SetHe3 (- (Variables|Default|GetHe3) Amount)))

(event Custom|GainHe3
  (params (Amount :type Integer))
  (Variables|Default|SetHe3 (Math|Integer|Clamp(Integer) (+ (Variables|Default|GetHe3) Amount) 0 (Variables|Default|GetHe3Cap))))

(event Custom|StatusCheck
  (Variables|Default|SetCurrentBuilder 0)
  (Variables|Default|SetCurrentDeposit 0)
  (bind _bcontinue (CallFunction|CommandCentreCheck))
  (if _bcontinue
    (bind _bcontinue_2 (CallFunction|CoreDepositCheck))
    (if _bcontinue_2
      (CallFunction|FactoryCheck)))
  (CallFunction|MechBuildCheck)
  (CallFunction|SkirmishCheck))

(event EventBeginPlay
  (Utilities|FlowControl|Delay 0.2)
  (AI|RunBehaviorTree "/Game/Blueprints/AI/BT_AI.BT_AI")
  (Class|AIController|UseBlackboard "/Game/Blueprints/AI/AI_Blackboard.AI_Blackboard")
  (bind _asbp_player_primary (Utilities|Casting|CastToBP_PlayerPrimary (Pawn|GetControlledPawn)))
  (bind _output_get (Variables|Default|SetPrimaryOwner _asbp_player_primary))
  (Variables|/Game/Blueprints/BP_PlayerPrimary.BP_PlayerPrimary_C|SetAI _output_get self)
  (Utilities|IsValid (.Territory (CallFunction|GetTerritory _output_get))
    (:Is%20Valid
      (Variables|Default|SetCurrentTerritory (.Territory (CallFunction|GetTerritory _output_get)))
      (Variables|Default|SetStartLocation (Transformation|GetActorLocation _asbp_player_primary))
      (Utilities|Time|SetTimerbyEvent (delegate Custom|StatusCheck) 2.0 true))))

(fn ConstructionScript)

(fn GetTerritory
  (params (Actor :type Actor%20Object%20Reference))
  (bind _returnvalue (Transformation|GetActorLocation Actor))
  (bind _primaryowner (Variables|Default|GetPrimaryOwner)
    (:then
      (bind _outhit (Collision|LineTraceForObjects _returnvalue (+ _returnvalue "0, 0,10000.000000") (Utilities|Array|MakeArray "ObjectTypeQuery7") false 0 "None"))
      (bind _asbp_territory_volume (Utilities|Casting|CastToBP_TerritoryVolume (.HitActor (Collision|BreakHitResult _outhit)))
        (:then
          (bind _array_element (Utilities|Array|ForEachLoopwithBreak 0 :!label _label)
            (:LoopBody
              (if (== (.Primary (Utilities|Struct|BreakTerritoryInfo _array_element)) _primaryowner)
                (bind _output_get (LocalVariables|SetLocalInfo _array_element))
                (goto _label Break)))
            (:Completed
              (return _asbp_territory_volume _output_get))))
        (:CastFailed
          (return 0 ""))))
    (:else
      (return 0 ""))))

(fn CommandCentreCheck
  (bind _primaryowner (Variables|Default|GetPrimaryOwner)
    (:then
      (bind _currentterritory (Variables|Default|GetCurrentTerritory)
        (:then
          (if (== _currentterritory (.Territory (CallFunction|GetTerritory _primaryowner)))
            (if (Utilities|Struct|BreakTerritoryInfo (.Info (CallFunction|GetTerritory _primaryowner)))
              (Variables|Default|SetCommandInfo (Utilities|Struct|MakeAICommands false (.bCoreHelium (Utilities|Struct|BreakAICommands (Variables|Default|GetCommandInfo))) (.bBuildFactory (Utilities|Struct|BreakAICommands (Variables|Default|GetCommandInfo))) (.bBuildUnits (Utilities|Struct|BreakAICommands (Variables|Default|GetCommandInfo)))) :!label _label)
              (return true)
              (else
                _))
            (else
              (bind _outdex (Default|GetTerritoryInfo _currentterritory _primaryowner))
              (if (Utilities|Struct|BreakTerritoryInfo (Utilities|Array|Get(acopy) (Variables|/Game/Environment/Objects/TerritoryVolume/BP_TerritoryVolume.BP_TerritoryVolume_C|GetTerritoryInfo _currentterritory) _outdex))
                _
                (else
                  (goto _label)))))
          (Variables|Default|SetCommandInfo (Utilities|Struct|MakeAICommands true false false false)))
        (:else
          _)))
    (:else
      _))
  (return false))

(fn GetCoreDeposits
  (params (Territory :type BP%20Territory%20Volume%20Object%20Reference))
  (bind _localdeposits (LocalVariables|GetLocalDeposits))
  (for _array_element (Variables|/Game/Environment/Objects/TerritoryVolume/BP_TerritoryVolume.BP_TerritoryVolume_C|GetDeposits Territory)
    (if (Variables|/Game/Environment/Objects/He3Deposit/BP_He3Deposit.BP_He3Deposit_C|GetbCore _array_element)
      (Utilities|Array|Add _localdeposits _array_element)))
  (return _localdeposits))

(fn CoreDepositCheck
  (bind _currentterritory (Variables|Default|GetCurrentTerritory)
    (:then
      (Variables|Default|SetCurrentDeposit 0)
      (bind _array_element (Utilities|Array|ForEachLoopwithBreak (Variables|/Game/Environment/Objects/TerritoryVolume/BP_TerritoryVolume.BP_TerritoryVolume_C|GetDeposits _currentterritory) :!label _label)
        (:LoopBody
          (Utilities|IsValid _array_element
            (:Is%20Valid
              (if (not (Variables|/Game/Environment/Objects/He3Deposit/BP_He3Deposit.BP_He3Deposit_C|GetbUsed _array_element))
                (Variables|Default|SetCurrentDeposit _array_element)
                (goto _label Break)))))
        (:Completed
          (Variables|Default|GetCurrentDeposit
            (:then
              (Variables|Default|SetCommandInfo (Utilities|Struct|MakeAICommands false true false false))
              (return false))
            (:else
              (Variables|Default|SetCommandInfo (Utilities|Struct|MakeAICommands (.bCommandCentre (Utilities|Struct|BreakAICommands (Variables|Default|GetCommandInfo))) false (.bBuildFactory (Utilities|Struct|BreakAICommands (Variables|Default|GetCommandInfo))) (.bBuildUnits (Utilities|Struct|BreakAICommands (Variables|Default|GetCommandInfo)))))
              (return true))))))
    (:else
      (return false))))

(fn FactoryCheck
  (bind _structurecap (Variables|Default|GetStructureCap))
  (bind (_t1faccap _t1facpop _containerpop _t1beaconpop) (Utilities|Struct|BreakStructureCap _structurecap))
  (if (Math|Boolean|ANDBoolean (< _t1facpop _t1faccap) (<= _t1facpop _containerpop) (<= _t1facpop _t1beaconpop))
    (Variables|Default|SetCommandInfo (Utilities|Struct|MakeAICommands false false true false))
    (return false)
    (else
      (Variables|Default|SetCommandInfo (Utilities|Struct|MakeAICommands (.bCommandCentre (Utilities|Struct|BreakAICommands (Variables|Default|GetCommandInfo))) (.bCoreHelium (Utilities|Struct|BreakAICommands (Variables|Default|GetCommandInfo))) false (.bBuildUnits (Utilities|Struct|BreakAICommands (Variables|Default|GetCommandInfo)))))
      (return true))))

(fn MechBuildCheck
  (bind _primaryowner (Variables|Default|GetPrimaryOwner)
    (:then
      (if (and (< (Variables|Default|GetMechPop) (Variables|Default|GetMechCap)) (<= (Variables|/Game/Blueprints/BP_PlayerPrimary.BP_PlayerPrimary_C|GetT1AssaultCost _primaryowner) (Variables|Default|GetHe3)))
        (bind _currentterritory (Variables|Default|GetCurrentTerritory)
          (:then
            (bind _array_element (Utilities|Array|ForEachLoopwithBreak (.T1Facs (Utilities|Struct|BreakStructureInventory (Variables|Default|GetStructureInventory))) :!label _label)
              (:LoopBody
                (if (== _currentterritory (.Territory (CallFunction|GetTerritory _array_element)))
                  (Variables|Default|SetCurrentBuilder _array_element)
                  (goto _label Break)))
              (:Completed
                (CallFunction|SpendHe3 (Variables|/Game/Blueprints/BP_PlayerPrimary.BP_PlayerPrimary_C|GetT1AssaultCost _primaryowner))
                (Math|Integer|IncrementInt (Variables|Default|GetMechPop)
                  (:%20%20
                    (bind _currentbuilder (Variables|Default|GetCurrentBuilder)
                      (:then
                        (Utilities|Array|Add (Variables|/Game/Blueprints/BP_Builder.BP_Builder_C|GetBuildQueue _currentbuilder) (Utilities|Struct|MakeBuildInfo (Variables|/Game/Blueprints/BP_PlayerPrimary.BP_PlayerPrimary_C|GetT1AssaultCost _primaryowner) 1 (Variables|/Game/Blueprints/BP_PlayerPrimary.BP_PlayerPrimary_C|GetBuildTime_T1Assault _primaryowner) "NewEnumerator0" (Variables|/Game/Blueprints/BP_PlayerPrimary.BP_PlayerPrimary_C|GetT1AssaultIcon _primaryowner)))
                        (if (Utilities|Enum|Equal(Enum) (Variables|/Game/Blueprints/BP_Builder.BP_Builder_C|GetCurrentType _currentbuilder) "NewEnumerator3")
                          (Default|BuildActor _currentbuilder)))
                      (:else)))))))
          (:else))))
    (:else)))

(fn SkirmishCheck
  (bind (_territory _info _bvalid) (CallFunction|GetEnemyTerritory))
  (bind _unitinventory (Variables|Default|GetUnitInventory))
  (bind _squad (LocalVariables|GetSquad))
  (bind _t1assault (Utilities|Struct|BreakUnitInventory _unitinventory))
  (bind _returnvalue (Utilities|Array|Length _squad))
  (if (and _bvalid (> (Utilities|Array|Length _t1assault) 0))
    (bind _primaryowner (Variables|Default|GetPrimaryOwner)
      (:then
        (Utilities|Array|Clear _squad)
        (bind _array_element (Utilities|Array|ForEachLoopwithBreak _t1assault :!label _label)
          (:LoopBody
            (Utilities|IsValid _array_element
              (:Is%20Valid
                (if (< _returnvalue 5)
                  (bind _asbp_mech_bot (Utilities|Casting|CastToBP_MechBot (Pawn|GetController _array_element)))
                  (if (Math|Boolean|NORBoolean (Variables|/Game/Blueprints/AI/BP_MechBot.BP_MechBot_C|GetbMoving _asbp_mech_bot) (Variables|/Game/Blueprints/AI/BP_MechBot.BP_MechBot_C|GetbMoveToRally _asbp_mech_bot))
                    (Utilities|Array|Add _squad _array_element))
                  (else
                    (goto _label Break))))))
          (:Completed
            (if (>= _returnvalue 5)
              (for _array_element_2 _squad
                (bind _asbp_mech_bot_2 (Utilities|Casting|CastToBP_MechBot (Pawn|GetController _array_element_2)))
                (Variables|/Game/Blueprints/AI/BP_MechBot.BP_MechBot_C|SetbAvailable _asbp_mech_bot_2 false))
              (bind _returnvalue_2 (Game|SpawnActorfromClass "/Game/Blueprints/BP_MoveTo.BP_MoveTo_C" (Math|Conversions|ToTransform(Vector) (Transformation|GetActorLocation (.CommandCentre (Utilities|Struct|BreakTerritoryInfo _info)))) "AlwaysSpawn" _primaryowner 0))
              (Variables|/Game/Blueprints/BP_MoveTo.BP_MoveTo_C|SetbLocating _returnvalue_2 false)
              (Variables|/Game/Blueprints/BP_MoveTo.BP_MoveTo_C|SetMechs _returnvalue_2 _squad)
              (Default|SetDestination _primaryowner _returnvalue_2)))))
      (:else))))

(fn GetEnemyTerritory
  (bind _primaryowner (Variables|Default|GetPrimaryOwner)
    (:then
      (bind _outactors (Actor|GetAllActorsOfClass "/Game/Environment/Objects/TerritoryVolume/BP_TerritoryVolume.BP_TerritoryVolume_C"))
      (bind _array_element (Utilities|Array|ForEachLoopwithBreak _outactors :!label _label)
        (:LoopBody
          (for _array_element_2 0
            (if (and (!= (Variables|/Game/Blueprints/BP_OpulentiumActor.BP_OpulentiumActor_C|GetTeam _primaryowner) (Variables|/Game/Blueprints/BP_OpulentiumActor.BP_OpulentiumActor_C|GetTeam (.Primary (Utilities|Struct|BreakTerritoryInfo _array_element_2)))) (Utilities|IsValid (.CommandCentre (Utilities|Struct|BreakTerritoryInfo _array_element_2))))
              (LocalVariables|SetReturn _array_element)
              (bind _output_get (LocalVariables|SetReturnInfo _array_element_2))
              (goto _label Break))))
        (:Completed
          (Utilities|IsValid (LocalVariables|GetReturn)
            (:Is%20Valid
              (return (LocalVariables|GetReturn) _output_get true))
            (:Is%20Not%20Valid
              (return 0 "" false))))))
    (:else
      (return 0 "" false))))