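; Player-pilotable command mech that lets its owner move and jump as the unit while still issuing RTS-style orders.
; Selection, group, move, patrol, build and interact inputs forward to server events on PrimaryOwner.
; Tab cycles possession through the owner and its other command mechs, returning this mech to its cached bot controller.
; Player possession makes it the owner's current leader and camera; other controllers trigger SetTarget instead.
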(event EventUnpossessed
  (params (OldController :type Controller%20Object%20Reference))
  (Utilities|Casting|CastToPlayerController OldController)
  (Variables|Default|SetbControlled false))

(event EventBeginPlay
  (|CallParentFunction)
  (bind _output_get (Variables|Default|SetBot (Pawn|GetController))))

(event EventPossessed
  (params (NewController :type Controller%20Object%20Reference))
  (Utilities|Casting|CastToPlayerController NewController
    (:then
      (bind _primaryowner (Variables|Default|GetPrimaryOwner)
        (:then
          (Variables|/Game/Blueprints/BP_PlayerPrimary.BP_PlayerPrimary_C|SetCurrentCamera _primaryowner (Variables|Default|GetCamera))
          (Variables|Default|SetbControlled true)
          (Variables|/Game/Blueprints/BP_PlayerPrimary.BP_PlayerPrimary_C|SetCurrentLeader _primaryowner self))
        (:else)))
    (:CastFailed
      (CallFunction|SetTarget 0.03))))

(event Input|ActionEvents|InputActionBuildT1Command
  (params (Key :type Key%20Structure :default "AnyKey"))
  (:Pressed
    (Default|ServerBuildT1Command (Variables|Default|GetPrimaryOwner))))

(event Input|ActionEvents|InputActionGroup1
  (params (Key :type Key%20Structure :default "AnyKey"))
  (:Pressed
    (Default|ServerGroup1 (Variables|Default|GetPrimaryOwner))))

(event Input|ActionEvents|InputActionGroup2
  (params (Key :type Key%20Structure :default "AnyKey"))
  (:Pressed
    (Default|ServerGroup2 (Variables|Default|GetPrimaryOwner))))

(event Input|ActionEvents|InputActionGroup3
  (params (Key :type Key%20Structure :default "AnyKey"))
  (:Pressed
    (Default|ServerGroup3 (Variables|Default|GetPrimaryOwner))))

(event Input|ActionEvents|InputActionGroup4
  (params (Key :type Key%20Structure :default "AnyKey"))
  (:Pressed
    (Default|ServerGroup4 (Variables|Default|GetPrimaryOwner))))

(event Input|ActionEvents|InputActionGroup5
  (params (Key :type Key%20Structure :default "AnyKey"))
  (:Pressed
    (Default|ServerGroup5 (Variables|Default|GetPrimaryOwner))))

(event Input|ActionEvents|InputActionShift
  (params (Key :type Key%20Structure :default "AnyKey"))
  (bind _primaryowner (Variables|Default|GetPrimaryOwner))
  (:Pressed
    (Default|ServerShiftPress _primaryowner))
  (:Released
    (Default|ServerShiftRelease _primaryowner)))

(event Input|ActionEvents|InputActionCtrl
  (params (Key :type Key%20Structure :default "AnyKey"))
  (bind _primaryowner (Variables|Default|GetPrimaryOwner))
  (:Pressed
    (Default|ServerCtrlPress _primaryowner))
  (:Released
    (Default|ServerCtrlRelease _primaryowner)))

(event Input|ActionEvents|InputActionMoveTo
  (params (Key :type Key%20Structure :default "AnyKey"))
  (bind _primaryowner (Variables|Default|GetPrimaryOwner))
  (:Pressed
    (Default|ServerMovetoPress _primaryowner))
  (:Released
    (Default|ServerMovetoRelease _primaryowner)))

(event Input|ActionEvents|InputActionSetPatrol
  (params (Key :type Key%20Structure :default "AnyKey"))
  (bind _primaryowner (Variables|Default|GetPrimaryOwner))
  (:Pressed
    (Default|ServerSetPatrol _primaryowner)
    (Variables|/Game/Blueprints/BP_PlayerPrimary.BP_PlayerPrimary_C|SetbRPressed _primaryowner true))
  (:Released
    (Default|ServerHidePatrols _primaryowner)
    (Variables|/Game/Blueprints/BP_PlayerPrimary.BP_PlayerPrimary_C|SetbRPressed _primaryowner false)))

(event Input|ActionEvents|InputActionInteract
  (params (Key :type Key%20Structure :default "AnyKey"))
  (:Pressed
    (Default|ServerInteract (Variables|Default|GetPrimaryOwner))))

(event Input|ActionEvents|InputActionSecondaryInteract
  (params (Key :type Key%20Structure :default "AnyKey"))
  (:Pressed
    (Default|ServerSecondaryInteract (Variables|Default|GetPrimaryOwner))))

(event Input|ActionEvents|InputActionSelect
  (params (Key :type Key%20Structure :default "AnyKey"))
  (:Pressed
    (Default|ServerSelect (Variables|Default|GetPrimaryOwner))))

(event Input|ActionEvents|InputActionBuildT1Support
  (params (Key :type Key%20Structure :default "AnyKey"))
  (:Pressed
    (Default|ServerBuildT1Support (Variables|Default|GetPrimaryOwner))))

(event Input|ActionEvents|InputActionBuildT1Assault
  (params (Key :type Key%20Structure :default "AnyKey"))
  (:Pressed
    (Default|ServerBuildT1Assault (Variables|Default|GetPrimaryOwner))))

(event Input|ActionEvents|InputActionJump
  (params (Key :type Key%20Structure :default "AnyKey"))
  (:Pressed
    (Character|Jump)))

(event Input|AxisEvents|InputAxisMoveForward
  (params (AxisValue :type Float%20%28single-precision%29))
  (Pawn|Input|AddMovementInput (Math|Vector|GetForwardVector (Math|Rotator|MakeRotator 0.0 0.0 (.Yaw (Math|Rotator|BreakRotator (Pawn|GetControlRotation :!class /Script/Engine.Pawn))))) AxisValue false))

(event Input|AxisEvents|InputAxisMoveRight
  (params (AxisValue :type Float%20%28single-precision%29))
  (Pawn|Input|AddMovementInput (Math|Vector|GetRightVector (Math|Rotator|MakeRotator 0.0 0.0 (.Yaw (Math|Rotator|BreakRotator (Pawn|GetControlRotation :!class /Script/Engine.Pawn))))) AxisValue false))

(event Input|AxisEvents|InputAxisTurn
  (params (AxisValue :type Float%20%28single-precision%29))
  (Pawn|Input|AddControllerYawInput AxisValue))

(event Input|AxisEvents|InputAxisLookUp
  (params (AxisValue :type Float%20%28single-precision%29))
  (Pawn|Input|AddControllerPitchInput AxisValue))

(event Input|KeyboardEvents|Tab
  (params (Key :type Key%20Structure :default "AnyKey"))
  (bind _return (CallFunction|GetNextMech))
  (:Pressed
    (Utilities|IsValid _return
      (:Is%20Valid
        (bind _output_get (Variables|Default|SetTemp (Pawn|GetController)))
        (Pawn|UnPossess _output_get)
        (Pawn|Possess _output_get _return)
        (Pawn|Possess (stale EventBeginPlay _output_get) self)))))

(fn ConstructionScript
  (|CallParentFunction))

(fn GetNextMech
  (bind _primaryowner (Variables|Default|GetPrimaryOwner))
  (bind _mechs (LocalVariables|GetMechs))
  (bind _outactors (Actor|GetAllActorsOfClass "BP_CommandMech_C"))
  (Utilities|Array|Add (LocalVariables|GetMechs) _primaryowner)
  (LocalVariables|SetMech _primaryowner)
  (for _array_element _outactors
    (if (== (Variables|/Game/Blueprints/BP_OpulentiumActor.BP_OpulentiumActor_C|GetPrimaryOwner _array_element) _primaryowner)
      (Utilities|Array|Add _mechs _array_element)))
  (bind (_array_element_2 _array_index) (Utilities|Array|ForEachLoopwithBreak _mechs :!label _label)
    (:LoopBody
      (if (== _array_element_2 self)
        (bind _output_get (LocalVariables|SetMech (select (== _array_index (Utilities|Array|LastIndex _mechs)) _primaryowner (Utilities|Array|Get(acopy) _mechs (+ _array_index 1)))))
        (goto _label Break)))
    (:Completed
      (return _output_get))))