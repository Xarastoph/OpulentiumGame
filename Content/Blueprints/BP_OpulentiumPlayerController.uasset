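; Multiplayer player controller for Opulentium that initializes each player's faction, team and primary pawn.
; Timed BeginPlay shows a loading screen on non-authority machines, spawns an AIController on authority, then applies game-instance lobby data by player ID, respawning the pawn for Callidus.
; A Tick-driven DoOnce retries until PrimaryOwner links to the controlled pawn.
; RepNotifies spawn its widgets, move it to an ID-indexed PlayerStart and refresh mech population text.
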(event Custom|SetFaction
  (bind _returnvalue (Pawn|GetControlledPawn))
  (bind _asbp_opulentium_instance (Utilities|Casting|CastToBP_OpulentiumInstance (Game|GetGameInstance)))
  (Utilities|FactionSwitch (Utilities|Array|Get(acopy) (Variables|/Game/Blueprints/BP_OpulentiumInstance.BP_OpulentiumInstance_C|GetFactions _asbp_opulentium_instance) (- (CallFunction|GetID) 1))
    (:Callidus
      (Utilities|IsValid _returnvalue
        (:Is%20Valid
          (Actor|DestroyActor _returnvalue))
        (:Is%20Not%20Valid
          _))
      (bind _returnvalue_2 (Game|SpawnActorfromClass "/Script/Engine.Pawn" (Transformation|GetActorTransform _returnvalue) "Undefined" 0 0))
      (Utilities|IsValid _returnvalue_2
        (:Is%20Valid
          (Pawn|Possess _returnvalue_2)
          (Variables|Default|SetPrimaryOwner 0)
          (Utilities|FlowControl|DoOnce false) ; enters at Reset
        )))))

(event Custom|SetTeam
  (bind _id (CallFunction|GetID))
  (bind _returnvalue (- _id 1))
  (bind _asbp_opulentium_instance (Utilities|Casting|CastToBP_OpulentiumInstance (Game|GetGameInstance)))
  (bind _primaryowner (Variables|Default|GetPrimaryOwner)
    (:then
      (Variables|/Game/Blueprints/BP_OpulentiumActor.BP_OpulentiumActor_C|SetTeam _primaryowner (Utilities|Array|Get(acopy) (Variables|/Game/Blueprints/BP_OpulentiumInstance.BP_OpulentiumInstance_C|GetTeams _asbp_opulentium_instance) _returnvalue))
      (Variables|/Game/Blueprints/BP_PlayerPrimary.BP_PlayerPrimary_C|SetPrimaryName _primaryowner (Utilities|Array|Get(acopy) (Variables|/Game/Blueprints/BP_OpulentiumInstance.BP_OpulentiumInstance_C|GetNames _asbp_opulentium_instance) _returnvalue)))
    (:else)))

(event Custom|Client_InputMode
  (Input|SetInputModeGameOnly self))

(event Custom|Server_InputMode
  (Input|SetInputModeGameOnly self))

(event Custom|ClientPopUpdate
  (bind _factorymenu (Variables|/Game/Blueprints/BP_PlayerPrimary.BP_PlayerPrimary_C|GetFactoryMenu (Variables|Default|GetPrimaryOwner))
    (:then
      (bind _populationtext (Variables|/Game/Blueprints/Widget/BP_FactoryWidget.BP_FactoryWidget_C|GetPopulationText _factorymenu)
        (:then
          (Rendering|Components|TextRender|SetText _populationtext (Utilities|Text|ToText(String) (Utilities|String|MakeLiteralString (Utilities|String|Append (Utilities|String|ToString(Integer) (Variables|Default|GetMechPop)) "/" (Utilities|String|ToString(Integer) (Variables|Default|GetMechCap)))))))
        (:else)))
    (:else)))

(event EventTick
  (params (DeltaSeconds :type Float%20%28single-precision%29))
  (Utilities|FlowControl|DoOnce false :!label _label
    (:Completed
      (bind _asbp_player_primary (Utilities|Casting|CastToBP_PlayerPrimary (Pawn|GetControlledPawn))
        (:then
          (bind _output_get (Variables|Default|SetPrimaryOwner _asbp_player_primary))
          (Variables|/Game/Blueprints/BP_PlayerPrimary.BP_PlayerPrimary_C|SetPlayerController _output_get self)
          (Variables|/Game/Blueprints/BP_PlayerPrimary.BP_PlayerPrimary_C|GetPlayerController _output_get
            (:then)
            (:else
              (goto _label Reset))))
        (:CastFailed
          (goto _label Reset))))))

(event EventBeginPlay
  (bind _self self)
  (Input|SetInputModeGameOnly _self)
  (bind _returnvalue (UserInterface|CreateWidget "/Game/Blueprints/Widget/BP_LoadScreen.BP_LoadScreen_C" _self))
  (Networking|SwitchHasAuthority
    (:Authority
      (bind _returnvalue_2 (Game|SpawnActorfromClass "/Script/AIModule.AIController" (Math|Transform|MakeTransform "0, 0, 0") "AlwaysSpawn" _self 0))
      (Variables|Default|SetTempController _returnvalue_2))
    (:Remote
      (UserInterface|Viewport|AddtoViewport _returnvalue 1)))
  (Utilities|FlowControl|Delay 1.0)
  (Networking|SwitchHasAuthority
    (:Authority
      (Variables|Default|SetID (CallFunction|GetID))
      (CallFunction|ClientInputMode))
    (:Remote
      (CallFunction|ServerInputMode)))
  (CallFunction|SetFaction)
  (CallFunction|SetTeam)
  (Variables|Default|SetbPrePlay false)
  (Utilities|FlowControl|Delay 2.0)
  (Input|EnableInput (Pawn|GetControlledPawn) _self)
  (Utilities|IsValid _returnvalue
    (:Is%20Valid
      (Widget|RemovefromParent _returnvalue))))

(fn ConstructionScript)

(fn OnRepMechCap
  (CallFunction|ClientPopUpdate))

(fn OnRepMechPop
  (bind _factorymenu (Variables|/Game/Blueprints/BP_PlayerPrimary.BP_PlayerPrimary_C|GetFactoryMenu (Variables|Default|GetPrimaryOwner))
    (:then
      (bind _populationtext (Variables|/Game/Blueprints/Widget/BP_FactoryWidget.BP_FactoryWidget_C|GetPopulationText _factorymenu)
        (:then
          (Rendering|Components|TextRender|SetText _populationtext (Utilities|Text|ToText(String) (Utilities|String|MakeLiteralString (Utilities|String|Append (Utilities|String|ToString(Integer) (Variables|Default|GetMechPop)) "/" (Utilities|String|ToString(Integer) (Variables|Default|GetMechCap)))))))
        (:else)))
    (:else)))

(fn GetID
  (bind _asbp_opulentium_instance (Utilities|Casting|CastToBP_OpulentiumInstance (Game|GetGameInstance))
    (:then
      (for _array_element (Variables|/Game/Blueprints/BP_OpulentiumInstance.BP_OpulentiumInstance_C|GetPlayerIDs _asbp_opulentium_instance)
        (if (== (+ (.PlayerID (Utilities|Struct|BreakPlayerIDInfo _array_element)) (Utilities|Array|Length (Variables|/Game/Blueprints/BP_OpulentiumInstance.BP_OpulentiumInstance_C|GetPlayerIDs _asbp_opulentium_instance))) (Variables|/Script/Engine.PlayerState|GetPlayerId (Variables|GetPlayerState)))
          (bind _output_get (LocalVariables|SetLocalID (.LobbyID (Utilities|Struct|BreakPlayerIDInfo _array_element)))))))
    (:CastFailed
      _))
  (return _output_get))

(fn OnRepPrimaryOwner
  (bind _primaryowner (Variables|Default|GetPrimaryOwner)
    (:then
      (Default|SpawnWidgets _primaryowner)
      (bind _outactors (Actor|GetAllActorsOfClass "/Script/Engine.PlayerStart"))
      (for (_array_element _array_index) _outactors
        (if (== _array_index (- (CallFunction|GetID) 1))
          (Transformation|SetActorLocation _primaryowner (Transformation|GetActorLocation _array_element) false false)
          (Transformation|SetActorRotation _primaryowner (Transformation|GetActorRotation _array_element))
          (Transformation|SetWorldRotation (Variables|/Game/Blueprints/BP_PlayerPrimary.BP_PlayerPrimary_C|GetCameraArm _primaryowner) (Transformation|GetActorRotation _array_element) false false))))
    (:else)))