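; BP_Placement is a placement preview actor, owned by a BP_PlayerPrimary, that shows whether its current spot is valid.
; BeginPlay caches the owner, resets CanPlace on authority and limits mesh visibility to the owner on remotes.
; The CanPlace RepNotify swaps every material slot between green and red.
; SurfaceSnap line-traces down, then up as fallback, returning the hit location and a normal-derived rotation, or the actor's location on a miss.
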(event EventBeginPlay
  (bind _asbp_player_primary (Utilities|Casting|CastToBP_PlayerPrimary (Components|GetOwner)))
  (Variables|Default|SetPrimaryOwner _asbp_player_primary)
  (Networking|SwitchHasAuthority
    (:Authority
      (Variables|Default|SetbCanPlace false))
    (:Remote
      (Rendering|SetOnlyOwnerSee (Variables|Default|GetStaticMesh) true :!class /Script/Engine.PrimitiveComponent))))

(fn ConstructionScript)

(fn SurfaceSnap
  (params (TraceDistance :type Float%20%28single-precision%29))
  (bind _returnvalue (Transformation|GetActorLocation))
  (bind _returnvalue_2 (Math|Vector|MakeVector 0.0 0.0 TraceDistance))
  (bind _outhit (Collision|LineTraceByChannel _returnvalue (- _returnvalue _returnvalue_2) "TraceTypeQuery1" false 0 "None"))
  (Utilities|IsValid (.HitActor (Collision|BreakHitResult _outhit))
    (:Is%20Valid
      (bind _output_get (LocalVariables|SetReturnLoc (.Location (Collision|BreakHitResult _outhit))))
      (bind _output_get_2 (LocalVariables|SetReturnRot (Math|Rotator|MakeRotfromX (Math|Vector|RotateVector (.Normal (Collision|BreakHitResult _outhit)) "-90.000000, 0, 0")))))
    (:Is%20Not%20Valid
      (bind _outhit_2 (Collision|LineTraceByChannel _returnvalue (+ _returnvalue _returnvalue_2) "TraceTypeQuery1" false 0 "None"))
      (Utilities|IsValid (.HitActor (Collision|BreakHitResult _outhit_2))
        (:Is%20Valid
          (LocalVariables|SetReturnLoc (.Location (Collision|BreakHitResult _outhit_2)))
          (LocalVariables|SetReturnRot (Math|Rotator|MakeRotfromX (Math|Vector|RotateVector (.Normal (Collision|BreakHitResult _outhit_2)) "-90.000000, 0, 0"))))
        (:Is%20Not%20Valid
          (LocalVariables|SetReturnLoc _returnvalue)))))
  (return _output_get _output_get_2))

(fn OnRepBCanPlace
  (bind _staticmesh (Variables|Default|GetStaticMesh))
  (bind _returnvalue (Rendering|Material|GetNumMaterials _staticmesh))
  (bind _returnvalue_2 (- _returnvalue 1))
  (if (Variables|Default|GetbCanPlace)
    (for _index (range 0 _returnvalue_2)
      (Rendering|Material|SetMaterial _staticmesh _index (Variables|Default|GetGreenMat)))
    (else
      (for _index_2 (range 0 _returnvalue_2)
        (Rendering|Material|SetMaterial _staticmesh _index_2 "/Game/Environment/Materials/Static/RedStatic.RedStatic")))))