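; Construction placeholder that stands in for a structure while it is being built, then replaces itself with the finished actor.
; A timeline scaled to BuildTime drives the build material, then the authority spawns BuildClass with proportional health, preserving selection.
; SetPopulation reserves player or AI structure caps, territory command-centre flags, or nearby deposit and power-node slots by class.
; Death releases population counts if the build was cancelled or failed.
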(event Custom|StopBuilding
  ;[1 1 1] SetScalar
  (bind _time (Timeline|BuildTimeline Stop)
    (:Update
      (Rendering|Material|SetScalarParameterValue (stale EventBeginPlay _returnvalue) "Time" _time :!class /Script/Engine.MaterialInstanceDynamic))
    (:Finished
      (if (not (Variables|Default|GetbCancel))
        (Networking|SwitchHasAuthority
          (:Authority
            (bind _primaryowner (Variables|Default|GetPrimaryOwner)
              (:then
                (bind _returnvalue (Game|SpawnActorfromClass (Variables|Default|GetBuildClass) (Transformation|GetActorTransform) "AlwaysSpawn" (Components|GetOwner) _primaryowner (Variables|/Game/Blueprints/BP_OpulentiumActor.BP_OpulentiumActor_C|GetTeam _primaryowner)))
                (Utilities|Array|Add (Variables|/Game/Blueprints/BP_PlayerPrimary.BP_PlayerPrimary_C|GetOwned _primaryowner) _returnvalue)
                (Variables|Default|SetbBuildSuccessful true)
                (Variables|/Game/Blueprints/BP_OpulentiumActor.BP_OpulentiumActor_C|SetHealth _returnvalue (Math|Float|Truncate (* (Variables|/Game/Blueprints/BP_OpulentiumActor.BP_OpulentiumActor_C|GetHealthMax _returnvalue) (/ (Math|Conversions|ToFloat(Integer) (Variables|Default|GetHealth)) (Math|Conversions|ToFloat(Integer) (Variables|Default|GetHealthMax))))))
                (if (Variables|Default|GetbSelected)
                  (Default|AddSelection _primaryowner _returnvalue (not (Utilities|IsValid (Variables|/Game/Blueprints/BP_PlayerPrimary.BP_PlayerPrimary_C|GetSelected _primaryowner)))))
                (CallFunction|Death))
              (:else))))))))

(event Custom|Cancel
  ;[1 1 1] Cancel
  (Variables|Default|SetbCancel true)
  (CallFunction|StopBuilding)
  (Utilities|FlowControl|Delay 1.2)
  (CallFunction|Death))

(event EventDeath
  ;[1 1 1] Destroyed
  (if (not (Variables|Default|GetbBuildSuccessful))
    (CallFunction|SetPopulation -1))
  (|CallParentFunction))

(event EventBeginPlay
  (bind _self self)
  ;[1 1 1] SetScalar
  (|CallParentFunction)
  (bind _returnvalue (Rendering|Material|CreateDynamicMaterialInstance (Variables|Character|GetMesh _self) (Variables|Default|GetMatIndex) (Variables|Default|GetBuildMat) :!class /Script/Engine.PrimitiveComponent))
  (CallFunction|SetPopulation _self 1)
  (Components|Timeline|SetPlayRate (Variables|Default|GetBuildTimeline) (/ 1.0 (Variables|Default|GetBuildTime)))
  (bind _time (Timeline|BuildTimeline PlayFromStart)
    (:Update
      (Rendering|Material|SetScalarParameterValue _returnvalue "Time" _time :!class /Script/Engine.MaterialInstanceDynamic))
    (:Finished
      (if (not (Variables|Default|GetbCancel))
        (Networking|SwitchHasAuthority
          (:Authority
            (bind _primaryowner (Variables|Default|GetPrimaryOwner)
              (:then
                (bind _returnvalue_2 (Game|SpawnActorfromClass (Variables|Default|GetBuildClass) (Transformation|GetActorTransform) "AlwaysSpawn" (Components|GetOwner) _primaryowner (Variables|/Game/Blueprints/BP_OpulentiumActor.BP_OpulentiumActor_C|GetTeam _primaryowner)))
                (Utilities|Array|Add (Variables|/Game/Blueprints/BP_PlayerPrimary.BP_PlayerPrimary_C|GetOwned _primaryowner) _returnvalue_2)
                (Variables|Default|SetbBuildSuccessful true)
                (Variables|/Game/Blueprints/BP_OpulentiumActor.BP_OpulentiumActor_C|SetHealth _returnvalue_2 (Math|Float|Truncate (* (Variables|/Game/Blueprints/BP_OpulentiumActor.BP_OpulentiumActor_C|GetHealthMax _returnvalue_2) (/ (Math|Conversions|ToFloat(Integer) (Variables|Default|GetHealth)) (Math|Conversions|ToFloat(Integer) (Variables|Default|GetHealthMax))))))
                (if (Variables|Default|GetbSelected)
                  (Default|AddSelection _primaryowner _returnvalue_2 (not (Utilities|IsValid (Variables|/Game/Blueprints/BP_PlayerPrimary.BP_PlayerPrimary_C|GetSelected _primaryowner)))))
                (CallFunction|Death))
              (:else))))))))

(fn ConstructionScript)

(fn SetPopulation
  (params (Multiplier :type Integer))
  (bind _returnvalue (== Multiplier 1))
  (bind _bbuildsuccessful (Variables|Default|GetbBuildSuccessful))
  (bind _returnvalue_2 (or _returnvalue _bbuildsuccessful))
  (bind _primaryowner (Variables|Default|GetPrimaryOwner)
    (:then
      (bind _playercontroller (Variables|/Game/Blueprints/BP_PlayerPrimary.BP_PlayerPrimary_C|GetPlayerController _primaryowner)
        (:then
          (Utilities|TypeSwitch
            (:Command
              (CallFunction|SetCommand _returnvalue_2))
            (:Container
              (bind _structout (Utilities|Struct|SetmembersinStructureCap (Variables|/Game/Blueprints/BP_OpulentiumPlayerController.BP_OpulentiumPlayerController_C|GetStructureCap _playercontroller) (+ (.ContainerPop (Utilities|Struct|BreakStructureCap (Variables|/Game/Blueprints/BP_OpulentiumPlayerController.BP_OpulentiumPlayerController_C|GetStructureCap _playercontroller))) Multiplier)))
              (Variables|/Game/Blueprints/BP_OpulentiumPlayerController.BP_OpulentiumPlayerController_C|SetStructureCap _playercontroller _structout))
            (:Factory
              (bind _structout_2 (Utilities|Struct|SetmembersinStructureCap (Variables|/Game/Blueprints/BP_OpulentiumPlayerController.BP_OpulentiumPlayerController_C|GetStructureCap _playercontroller) (+ (.T1FacPop (Utilities|Struct|BreakStructureCap (Variables|/Game/Blueprints/BP_OpulentiumPlayerController.BP_OpulentiumPlayerController_C|GetStructureCap _playercontroller))) Multiplier)))
              (Variables|/Game/Blueprints/BP_OpulentiumPlayerController.BP_OpulentiumPlayerController_C|SetStructureCap _playercontroller _structout_2))
            (:Beacon
              (bind _structout_3 (Utilities|Struct|SetmembersinStructureCap (Variables|/Game/Blueprints/BP_OpulentiumPlayerController.BP_OpulentiumPlayerController_C|GetStructureCap _playercontroller) (+ (.T1BeaconPop (Utilities|Struct|BreakStructureCap (Variables|/Game/Blueprints/BP_OpulentiumPlayerController.BP_OpulentiumPlayerController_C|GetStructureCap _playercontroller))) Multiplier)))
              (Variables|/Game/Blueprints/BP_OpulentiumPlayerController.BP_OpulentiumPlayerController_C|SetStructureCap _playercontroller _structout_3))
            (:Snap
              (CallFunction|SetUsed _returnvalue_2))))
        (:else
          (bind _ai (Variables|/Game/Blueprints/BP_PlayerPrimary.BP_PlayerPrimary_C|GetAI _primaryowner)
            (:then
              (Utilities|TypeSwitch
                (:Command
                  (CallFunction|SetCommand _returnvalue_2))
                (:Container
                  (bind _structout_4 (Utilities|Struct|SetmembersinStructureCap (Variables|/Game/Blueprints/BP_OpulentiumAI.BP_OpulentiumAI_C|GetStructureCap _ai) (+ (.ContainerPop (Utilities|Struct|BreakStructureCap (Variables|/Game/Blueprints/BP_OpulentiumAI.BP_OpulentiumAI_C|GetStructureCap _ai))) Multiplier)))
                  (Variables|/Game/Blueprints/BP_OpulentiumAI.BP_OpulentiumAI_C|SetStructureCap _ai _structout_4))
                (:Factory
                  (bind _structout_5 (Utilities|Struct|SetmembersinStructureCap (Variables|/Game/Blueprints/BP_OpulentiumAI.BP_OpulentiumAI_C|GetStructureCap _ai) (+ (.T1FacPop (Utilities|Struct|BreakStructureCap (Variables|/Game/Blueprints/BP_OpulentiumAI.BP_OpulentiumAI_C|GetStructureCap _ai))) Multiplier)))
                  (Variables|/Game/Blueprints/BP_OpulentiumAI.BP_OpulentiumAI_C|SetStructureCap _ai _structout_5))
                (:Beacon
                  (bind _structout_6 (Utilities|Struct|SetmembersinStructureCap (Variables|/Game/Blueprints/BP_OpulentiumAI.BP_OpulentiumAI_C|GetStructureCap _ai) (+ (.T1BeaconPop (Utilities|Struct|BreakStructureCap (Variables|/Game/Blueprints/BP_OpulentiumAI.BP_OpulentiumAI_C|GetStructureCap _ai))) Multiplier)))
                  (Variables|/Game/Blueprints/BP_OpulentiumAI.BP_OpulentiumAI_C|SetStructureCap _ai _structout_6))
                (:Snap
                  (CallFunction|SetUsed _returnvalue_2))))
            (:else)))))
    (:else)))

(fn SetCommandParam
  (bind _returnvalue (Transformation|GetActorLocation))
  (bind _primaryowner (Variables|Default|GetPrimaryOwner))
  (if (Utilities|ClassIsChildOf (Variables|Default|GetBuildClass) "/Game/Blueprints/BP_CommandCentre.BP_CommandCentre_C")
    (bind _outhit (Collision|LineTraceForObjects _returnvalue (+ _returnvalue "0, 0,10000.000000") (Utilities|Array|MakeArray "ObjectTypeQuery7") false 0 "None"))
    (bind _asbp_territory_volume (Utilities|Casting|CastToBP_TerritoryVolume (.HitActor (Collision|BreakHitResult _outhit))))
    (bind _outdex (Default|GetTerritoryInfo _asbp_territory_volume _primaryowner))
    (Default|SetTerritoryInfo _asbp_territory_volume _outdex (Utilities|Struct|MakeTerritoryInfo _primaryowner (.Tier (Utilities|Struct|BreakTerritoryInfo (Utilities|Array|Get(acopy) (Variables|/Game/Environment/Objects/TerritoryVolume/BP_TerritoryVolume.BP_TerritoryVolume_C|GetTerritoryInfo _asbp_territory_volume) _outdex))) true (.bHasResearchCentre (Utilities|Struct|BreakTerritoryInfo (Utilities|Array|Get(acopy) (Variables|/Game/Environment/Objects/TerritoryVolume/BP_TerritoryVolume.BP_TerritoryVolume_C|GetTerritoryInfo _asbp_territory_volume) _outdex))) (.bIsInVolume (Utilities|Struct|BreakTerritoryInfo (Utilities|Array|Get(acopy) (Variables|/Game/Environment/Objects/TerritoryVolume/BP_TerritoryVolume.BP_TerritoryVolume_C|GetTerritoryInfo _asbp_territory_volume) _outdex)))))))

(fn SetUsed
  (params (bNewUsed :type Boolean))
  (bind _buildclass (Variables|Default|GetBuildClass))
  (if (Utilities|ClassIsChildOf _buildclass "/Game/Blueprints/BP_Extractor.BP_Extractor_C")
    (bind _outactors (Actor|GetAllActorsOfClass "/Game/Environment/Objects/He3Deposit/BP_He3Deposit.BP_He3Deposit_C"))
    (bind _array_element (Utilities|Array|ForEachLoopwithBreak _outactors :!label _label)
      (:LoopBody
        (if (<= (Transformation|GetDistanceTo _array_element) 256.0)
          (Variables|/Game/Environment/Objects/He3Deposit/BP_He3Deposit.BP_He3Deposit_C|SetbUsed _array_element bNewUsed)
          (goto _label Break))))
    (elif (Utilities|ClassIsChildOf _buildclass "/Game/Blueprints/BP_Conduit.BP_Conduit_C")
      (bind _outactors_2 (Actor|GetAllActorsOfClass "/Game/Environment/Objects/PowerNode/BP_PowerNode.BP_PowerNode_C"))
      (bind _array_element_2 (Utilities|Array|ForEachLoopwithBreak _outactors_2 :!label _label_2)
        (:LoopBody
          (if (<= (Transformation|GetDistanceTo _array_element_2) 256.0)
            (Variables|/Game/Environment/Objects/PowerNode/BP_PowerNode.BP_PowerNode_C|SetbUsed _array_element_2 bNewUsed)
            (goto _label_2 Break)))))))

(fn SetCommand
  (params (bHasCommand :type Boolean))
  (bind _returnvalue (Transformation|GetActorLocation))
  (bind _outhit (Collision|LineTraceForObjects _returnvalue (+ _returnvalue "0, 0,10000.000000") (Utilities|Array|MakeArray "ObjectTypeQuery7") false 0 "None"))
  (bind _asbp_territory_volume (Utilities|Casting|CastToBP_TerritoryVolume (.HitActor (Collision|BreakHitResult _outhit))))
  (bind (_array_element _array_index) (Utilities|Array|ForEachLoopwithBreak (Variables|/Game/Environment/Objects/TerritoryVolume/BP_TerritoryVolume.BP_TerritoryVolume_C|GetTerritoryInfo _asbp_territory_volume) :!label _label)
    (:LoopBody
      (if (== (Variables|Default|GetPrimaryOwner) (.Primary (Utilities|Struct|BreakTerritoryInfo _array_element)))
        (Utilities|Array|SetArrayElem (Variables|/Game/Environment/Objects/TerritoryVolume/BP_TerritoryVolume.BP_TerritoryVolume_C|GetTerritoryInfo _asbp_territory_volume) _array_index (Utilities|Struct|MakeTerritoryInfo (.Primary (Utilities|Struct|BreakTerritoryInfo _array_element)) (.Tier (Utilities|Struct|BreakTerritoryInfo _array_element)) bHasCommand (.bHasResearchCentre (Utilities|Struct|BreakTerritoryInfo _array_element)) (.bIsInVolume (Utilities|Struct|BreakTerritoryInfo _array_element))))
        (Development|PrintString (Utilities|String|ToString(Boolean) (Utilities|Struct|BreakTerritoryInfo _array_element)))
        (goto _label Break)))))