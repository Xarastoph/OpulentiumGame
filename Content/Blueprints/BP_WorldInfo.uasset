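; BP_WorldInfo is a world manager actor that starts the background music and drives an optional day-night cycle.
; On BeginPlay it sets the music cue and, when day-night is enabled with valid light and sky references, plays the DayNight timeline.
; The timeline pitches the light, refreshes the sky's sun direction, and derives clamped fog density from the negated cubed sine of that pitch.
; A ChangeVolume event adjusts music volume instantly.
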(event Custom|ChangeVolume
  (params (NewVolume :type Float%20%28single-precision%29))
  (Audio|Components|Audio|AdjustVolume (Variables|Default|GetMusicAudio) 0.0 NewVolume :!class /Script/Engine.AudioComponent))

(event EventBeginPlay
  (Audio|Components|Audio|SetSound (Variables|Default|GetMusicAudio) (Variables|Default|GetMusicCue))
  (if (Variables|Default|GetbUseDayNight)
    (bind _light (Variables|Default|GetLight)
      (:then
        (bind _sky (Variables|Default|GetSky)
          (:then
            (bind _time (Timeline|DayNight Play)
              (:Update
                (Transformation|SetActorRotation _light (Math|Rotator|MakeRotator 0.0 _time 9e+01))
                (Default|UpdateSunDirection _sky)
                (bind _fog (Variables|Default|GetFog)
                  (:then
                    (Class|ExponentialHeightFogComponent|SetFogDensity (Variables|/Script/Engine.ExponentialHeightFog|GetComponent _fog) (Math|Float|Clamp(Float) (* (Math|Float|Power (Math|Trig|Sin(Degrees) _time) 3.0) -1.0) 0.0 0.03)))
                  (:else)))))
          (:else)))
      (:else))))

(fn ConstructionScript)