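; BP_WaveBoss is a wave manager that coordinates every BP_SpawnerParent in the level when enabled.
; On BeginPlay it gathers the spawners, sets ShowHUD if any exist, and starts the first wave, clearing FirstWave after a short delay.
; Each wave spreads intensity points, one per wave number, across random spawner groups.
; The RepBool OnRep counts down WaveTotal, launching the next wave when it runs out.
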(event EventBeginPlay
  (if (Variables|Default|GetbUse)
    (bind _outactors (Actor|GetAllActorsOfClass "/Game/Blueprints/BP_SpawnerParent.BP_SpawnerParent_C"))
    (bind _output_get (Variables|Default|SetbShowHUD (> (Utilities|Array|Length _outactors) 0)))
    (if _output_get
      (bind _output_get_2 (Variables|Default|SetWaveSpawns _outactors))
      (CallFunction|SetWaveIntensities)
      (Default|SpawnWave _output_get_2)
      (Utilities|FlowControl|Delay 5.1)
      (Variables|Default|SetbFirstWave false))))

(fn ConstructionScript)

(fn OnRepRepBool
  (bind _result (Math|Integer|DecrementInt (Variables|Default|GetWaveTotal))
    (:%20%20
      (if (<= _result 0)
        (Math|Integer|IncrementInt (Variables|Default|GetWaveNumber)
          (:%20%20
            (CallFunction|SetWaveIntensities)
            (for _array_element (Variables|Default|GetWaveSpawns)
              (Default|SpawnWave _array_element))))))))

(fn SetWaveIntensities
  (bind _wavespawns (Variables|Default|GetWaveSpawns))
  (for _array_element _wavespawns
    (Variables|/Game/Blueprints/BP_SpawnerParent.BP_SpawnerParent_C|SetWaveIntensity _array_element 0))
  (for _index (range 1 (Variables|Default|GetWaveNumber))
    (bind _output_get (LocalVariables|SetGroup (Math|Random|RandomIntegerinRange 1 (Variables|Default|GetGroupMax))))
    (for _array_element_2 _wavespawns
      (if (== (Variables|/Game/Blueprints/BP_SpawnerParent.BP_SpawnerParent_C|GetGroup _array_element_2) _output_get)
        (Math|Integer|IncrementInt (Variables|/Game/Blueprints/BP_SpawnerParent.BP_SpawnerParent_C|GetWaveIntensity _array_element_2))))))