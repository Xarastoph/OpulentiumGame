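; BP_TerritoryVolume is a territory volume that tracks the He3 deposits and power nodes belonging to it, plus per-primary territory info.
; On BeginPlay it line-traces upward from every deposit and power node, keeping those whose trace hits this volume.
; Helper functions find a TerritoryInfo index by Primary and overwrite entries by index.
; A CastSwitch macro branches an actor to player-primary or command-placement execution.
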(event EventBeginPlay
  (bind _array (Utilities|Array|MakeArray "ObjectTypeQuery7"))
  (bind _outactors (Actor|GetAllActorsOfClass "/Game/Environment/Objects/He3Deposit/BP_He3Deposit.BP_He3Deposit_C"))
  (for _array_element _outactors
    (bind _outhit (Collision|LineTraceForObjects (Transformation|GetActorLocation _array_element) (+ (Transformation|GetActorLocation _array_element) "0, 0,10000.000000") _array false 0 "None"))
    (if (== self (.HitActor (Collision|BreakHitResult _outhit)))
      (Utilities|Array|AddUnique (Variables|Default|GetDeposits) _array_element)))
  (bind _outactors_2 (Actor|GetAllActorsOfClass "/Game/Environment/Objects/PowerNode/BP_PowerNode.BP_PowerNode_C"))
  (for _array_element_2 _outactors_2
    (bind _outhit_2 (Collision|LineTraceForObjects (Transformation|GetActorLocation _array_element_2) (+ (Transformation|GetActorLocation _array_element_2) "0, 0,10000.000000") _array false 0 "None"))
    (if (== self (.HitActor (Collision|BreakHitResult _outhit_2)))
      (Utilities|Array|AddUnique (Variables|Default|GetPowerNodes) _array_element_2))))

(fn ConstructionScript)

(fn GetTerritoryInfo
  (params (Primary :type BP%20Player%20Primary%20Object%20Reference))
  (bind (_array_element _array_index) (Utilities|Array|ForEachLoopwithBreak (Variables|Default|GetTerritoryInfo) :!label _label)
    (:LoopBody
      (if (== (Utilities|Struct|BreakTerritoryInfo _array_element) Primary)
        (bind _output_get (LocalVariables|SetIndex _array_index))
        (goto _label Break)))
    (:Completed
      (return _output_get))))

(fn SetTerritoryInfo
  (params (Index :type Integer) (NewInfo :type Territory%20Info%20Structure))
  (Utilities|Array|SetArrayElem (Variables|Default|GetTerritoryInfo) Index NewInfo true))