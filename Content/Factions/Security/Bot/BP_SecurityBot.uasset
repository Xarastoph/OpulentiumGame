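; AI controller for a Security faction mech, running BT_Security with patrol and pursue states.
; Tick mirrors the mech's CurrentTarget into pursuit and look-at state, while a looping timer picks random patrol destinations around the start location.
; RotateDestination computes standoff or orbit points around the target.
; RepNotify setters push changes to the blackboard, movement orientation and BP_Squire tracking; destruction clears RepBool on a BP_WaveBoss.
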(event Custom|SetDest
  (bind _returnvalue (Math|Random|RandomUnitVector))
  (bind (_x _y) (Math|Vector|BreakVector _returnvalue))
  (if (Variables|Default|GetbPatrol)
    (Variables|Default|SetDestination (+ (Variables|Default|GetInitialLocation) (* (Math|Vector|MakeVector _x _y 0.0) (Math|Random|RandomFloatinRange 512.0 2048.0))))))

(event EventTick
  (params (DeltaSeconds :type Float%20%28single-precision%29))
  (CallFunction|SetPatrol))

(event EventDestroyed
  (bind _outactors (Actor|GetAllActorsOfClass "/Game/Blueprints/BP_WaveBoss.BP_WaveBoss_C"))
  (if (> (Utilities|Array|Length _outactors) 0)
    (Variables|/Game/Blueprints/BP_WaveBoss.BP_WaveBoss_C|SetRepBool (Utilities|Array|Get(acopy) _outactors) false)))

(event EventBeginPlay
  (Utilities|FlowControl|Delay 0.2)
  (AI|RunBehaviorTree "/Game/Factions/Security/Bot/BT_Security.BT_Security")
  (Class|AIController|UseBlackboard "/Game/Factions/Security/Bot/BB_Security.BB_Security")
  (bind _asbp_mech (Utilities|Casting|CastToBP_Mech (Pawn|GetControlledPawn)))
  (Variables|Default|SetSecurityMech _asbp_mech)
  (Variables|Default|SetInitialLocation (Transformation|GetActorLocation _asbp_mech))
  (CallFunction|SetDest)
  (Utilities|Time|SetTimerbyEvent (delegate Custom|SetDest) 1.0 true))

(fn ConstructionScript)

(fn SetPatrol
  (bind _securitymech (Variables|Default|GetSecurityMech)
    (:then
      (bind _currenttarget (Variables|/Game/Blueprints/BP_CombatActor.BP_CombatActor_C|GetCurrentTarget _securitymech)
        (:then
          (Variables|Default|SetPursue _currenttarget)
          (Variables|Default|SetLookat (Math|Rotator|MakeRotator (* (.Pitch (Math|Rotator|BreakRotator (Math|Rotator|FindLookatRotation (Transformation|GetActorLocation (Variables|Default|GetSecurityMech)) (Transformation|GetActorLocation (Variables|Default|GetPursue))))) -1.0) (.Roll (Math|Rotator|BreakRotator (Math|Rotator|FindLookatRotation (Transformation|GetActorLocation (Variables|Default|GetSecurityMech)) (Transformation|GetActorLocation (Variables|Default|GetPursue))))) (- (.Yaw (Math|Rotator|BreakRotator (Math|Rotator|FindLookatRotation (Transformation|GetActorLocation (Variables|Default|GetSecurityMech)) (Transformation|GetActorLocation (Variables|Default|GetPursue))))) 9e+01)))
          (Variables|Default|SetbPatrol false))
        (:else
          (Variables|Default|SetPursue 0)
          (Variables|Default|SetbPatrol true))))
    (:else)))

(fn RotateDestination
  (params (bAlign :type Boolean))
  (bind _pursue (Variables|Default|GetPursue)
    (:then
      (if bAlign
        (Variables|Default|SetDestination (+ (* (Math|Vector|Normalize (- (Transformation|GetActorLocation (Variables|Default|GetSecurityMech)) (Transformation|GetActorLocation _pursue))) 1024.0) (Transformation|GetActorLocation _pursue)))
        (else
          (Variables|Default|SetDestination (+ (Math|Vector|RotateVector (* (Math|Vector|Normalize (- (Transformation|GetActorLocation (Variables|Default|GetSecurityMech)) (Transformation|GetActorLocation _pursue))) 1024.0) (Math|Rotator|MakeRotator 0.0 0.0 (* (Variables|Default|GetMultiplier) 6e+01))) (Transformation|GetActorLocation _pursue))))))
    (:else)))

(fn OnRepBPatrol
  (bind _bpatrol (Variables|Default|GetbPatrol))
  (bind _securitymech (Variables|Default|GetSecurityMech))
  (if _bpatrol
    _
    (else
      (CallFunction|RotateDestination true)))
  (Variables|/Script/Engine.CharacterMovementComponent|SetbOrientRotationToMovement (Variables|/Script/Engine.Character|GetCharacterMovement _securitymech) _bpatrol)
  (bind _asbp_squire (Utilities|Casting|CastToBP_Squire _securitymech))
  (Variables|/Game/Factions/Security/Squire/Meshes/BP_Squire.BP_Squire_C|SetbTrack _asbp_squire (not _bpatrol)))

(fn OnRepDestination
  (AI|Components|Blackboard|SetValueasVector (AI|GetBlackboard self) (Utilities|String|StringToName "Destination") (Variables|Default|GetDestination)))

(fn OnRepPursue
  (bind _securitymech (Variables|Default|GetSecurityMech))
  (bind _pursue (Variables|Default|GetPursue)
    (:then
      (Variables|/Game/Blueprints/BP_CombatActor.BP_CombatActor_C|SetCurrentTarget _securitymech _pursue))
    (:else
      (Variables|/Game/Blueprints/BP_CombatActor.BP_CombatActor_C|SetCurrentTarget _securitymech 0))))

(fn OnRepLookat
  (Networking|SwitchHasAuthority
    (:Authority
      (bind _securitymech (Variables|Default|GetSecurityMech)
        (:then
          (bind _asbp_squire (Utilities|Casting|CastToBP_Squire _securitymech))
          (Variables|/Game/Factions/Security/Squire/Meshes/BP_Squire.BP_Squire_C|SetLookatRot _asbp_squire (Variables|Default|GetLookat)))
        (:else)))))