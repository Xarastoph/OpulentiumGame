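; Blueprint for the Squire, a unit of the Security faction, which rewards its killer with He3 when destroyed.
; The Destroyed event calls the parent handler, then runs a DoOnce gate so the reward is paid a single time.
; If KillActor is valid and below its He3Cap, it gains a fixed amount of He3, clamped to that cap.
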(event EventDestroyed
  (|CallParentFunction)
  (Utilities|FlowControl|DoOnce false
    (:Completed
      (bind _killactor (Variables|Default|GetKillActor)
        (:then
          (if (< (Variables|/Game/Blueprints/BP_OpulentiumPlayerController.BP_OpulentiumPlayerController_C|GetHe3 _killactor) (Variables|/Game/Blueprints/BP_OpulentiumPlayerController.BP_OpulentiumPlayerController_C|GetHe3Cap _killactor))
            (if (< (+ (Variables|/Game/Blueprints/BP_OpulentiumPlayerController.BP_OpulentiumPlayerController_C|GetHe3 _killactor) 100) (Variables|/Game/Blueprints/BP_OpulentiumPlayerController.BP_OpulentiumPlayerController_C|GetHe3Cap _killactor))
              (Variables|/Game/Blueprints/BP_OpulentiumPlayerController.BP_OpulentiumPlayerController_C|SetHe3 _killactor (+ (Variables|/Game/Blueprints/BP_OpulentiumPlayerController.BP_OpulentiumPlayerController_C|GetHe3 _killactor) 100))
              (else
                (Variables|/Game/Blueprints/BP_OpulentiumPlayerController.BP_OpulentiumPlayerController_C|SetHe3 _killactor (Variables|/Game/Blueprints/BP_OpulentiumPlayerController.BP_OpulentiumPlayerController_C|GetHe3Cap _killactor))))))
        (:else)))))

(fn ConstructionScript)