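; Python turret actor for the Callidus faction that fades in a hologram on one of its mesh materials.
; BeginPlay creates a dynamic instance of that material slot and starts it fully transparent.
; While PlayAnim is true, Tick accumulates clamped time over two seconds and feeds it straight into the Opacity parameter.
; Nothing in this Blueprint sets PlayAnim.
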(event EventBeginPlay
  (|CallParentFunction)
  (bind _returnvalue (Rendering|Material|CreateDynamicMaterialInstance (Variables|Character|GetMesh) 3 "/Game/Factions/Callidus/Python/Materials/PythonTurret_ID05_Diffuse_Mat_Inst.PythonTurret_ID05_Diffuse_Mat_Inst" :!class /Script/Engine.PrimitiveComponent))
  (bind _output_get (Variables|Default|SetHologram _returnvalue))
  (Rendering|Material|SetScalarParameterValue _output_get "Opacity" 0.0 :!class /Script/Engine.MaterialInstanceDynamic))

(event EventTick
  (params (DeltaSeconds :type Float%20%28single-precision%29))
  (|CallParentFunction DeltaSeconds)
  (if (Variables|Default|GetbPlayAnim)
    (if (< (Variables|Default|GetTime) 2.0)
      (bind _output_get (Variables|Default|SetTime (Math|Float|Clamp(Float) (+ (Variables|Default|GetTime) DeltaSeconds) 0.0 2.0)))
      (Rendering|Material|SetScalarParameterValue (stale EventBeginPlay _output_get) "Opacity" _output_get :!class /Script/Engine.MaterialInstanceDynamic))))

(fn ConstructionScript
  (|CallParentFunction))