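; Projectile for the Callidus Cobra weapon that homes in on the first Opulentium actor it detects ahead of it.
; Each tick without a homing target, it box-traces along its velocity, ignoring its owner, and sets the first matching actor's root component as the movement component's homing target.
; Tick also adds a relative mesh rotation that evaluates to zero, and the homing search runs only while the mesh is valid.
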(event EventTick
  (params (DeltaSeconds :type Float%20%28single-precision%29))
  (bind _returnvalue (Transformation|GetActorLocation))
  (bind _returnvalue_2 (Transformation|GetVelocity))
  (bind _returnvalue_3 (* 0.0 1e+02))
  (bind _returnvalue_4 (Math|Vector|Normalize _returnvalue_2))
  (bind _returnvalue_5 (* _returnvalue_4 512.0))
  (bind _returnvalue_6 (+ _returnvalue _returnvalue_5))
  (|CallParentFunction DeltaSeconds)
  (bind _projectilemesh (Variables|Default|GetProjectileMesh)
    (:then
      (Transformation|AddRelativeRotation _projectilemesh (Math|Rotator|MakeRotator _returnvalue_3 _returnvalue_3 _returnvalue_3) false false)
      (bind _projectilemovement (Variables|Default|GetProjectileMovement)
        (:then
          (Variables|/Script/Engine.ProjectileMovementComponent|GetHomingTargetComponent _projectilemovement
            (:then)
            (:else
              (bind _outhits (Class|KismetSystemLibrary|BoxTraceMultiforObjects _returnvalue_6 (+ _returnvalue_6 "0, 0,4.000000") "512.000000,200.000000,200.000000" (Math|Conversions|RotationFromXVector _returnvalue_2) (Utilities|Array|MakeArray "ObjectTypeQuery1" "ObjectTypeQuery2" "ObjectTypeQuery3" "ObjectTypeQuery5") false (Utilities|Array|MakeArray (Components|GetOwner)) "None" true))
              (bind _array_element (Utilities|Array|ForEachLoopwithBreak _outhits :!label _label)
                (:LoopBody
                  (Utilities|Casting|CastToBP_OpulentiumActor (.HitActor (Collision|BreakHitResult _array_element)))
                  (Variables|/Script/Engine.ProjectileMovementComponent|SetHomingTargetComponent _projectilemovement (VehicleSound|GetRootComponent (.HitActor (Collision|BreakHitResult _array_element))))
                  (goto _label Break))))))
        (:else)))
    (:else)))

(fn ConstructionScript
  (|CallParentFunction))