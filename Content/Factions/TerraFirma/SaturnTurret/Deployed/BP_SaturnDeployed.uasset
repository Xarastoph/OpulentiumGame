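; Deployed Saturn turret for the Terra Firma faction, a child Blueprint that adds recoil and AI inventory tracking to its parent.
; Each projectile spawn pulses a Recoil flag on for a brief moment.
; On begin play and destruction, it adds or removes itself from the T1 turret list in its owner's AI unit inventory, when that owner and AI are valid.
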(event Custom|SpawnProjectile
  (Variables|Default|SetbRecoil true)
  (Utilities|FlowControl|Delay 0.05)
  (Variables|Default|SetbRecoil false))

(event EventBeginPlay
  (|CallParentFunction)
  (bind _primaryowner (Variables|Default|GetPrimaryOwner)
    (:then
      (bind _ai (Variables|/Game/Blueprints/BP_PlayerPrimary.BP_PlayerPrimary_C|GetAI _primaryowner)
        (:then
          (Utilities|Array|Add (Utilities|Struct|BreakUnitInventory (Variables|/Game/Blueprints/BP_OpulentiumAI.BP_OpulentiumAI_C|GetUnitInventory _ai)) self))
        (:else)))
    (:else)))

(event EventDestroyed
  (|CallParentFunction)
  (bind _primaryowner (Variables|Default|GetPrimaryOwner)
    (:then
      (bind _ai (Variables|/Game/Blueprints/BP_PlayerPrimary.BP_PlayerPrimary_C|GetAI _primaryowner)
        (:then
          (Utilities|Array|RemoveItem (Utilities|Struct|BreakUnitInventory (Variables|/Game/Blueprints/BP_OpulentiumAI.BP_OpulentiumAI_C|GetUnitInventory _ai)) self))
        (:else)))
    (:else)))

(fn ConstructionScript
  (|CallParentFunction))