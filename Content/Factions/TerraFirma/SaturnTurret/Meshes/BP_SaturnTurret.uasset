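; BP_SaturnTurret is the Terra Firma Saturn Turret unit, tracked as tier-1 support in its owner's AI inventory.
; It adds itself to the PrimaryOwner AI's T1Support list on BeginPlay and removes itself on Destroyed.
; Each Tick it draws debug text above itself showing the Moving and Transform values of its BP_MechBot controller, if it has one.
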(event EventTick
  (params (DeltaSeconds :type Float%20%28single-precision%29))
  (bind _asbp_mech_bot (Utilities|Casting|CastToBP_MechBot (Pawn|GetController)))
  (Rendering|Debug|DrawDebugString "0, 0,128.000000" (Utilities|String|Append "Moving: " (Utilities|String|ToString(Boolean) (Variables|/Game/Blueprints/AI/BP_MechBot.BP_MechBot_C|GetbMoving _asbp_mech_bot)) " || " "Transform: " (Utilities|String|ToString(Boolean) (Variables|/Game/Blueprints/AI/BP_MechBot.BP_MechBot_C|GetbTransform _asbp_mech_bot))) self "(R=1.000000,G=1.000000,B=1.000000,A=1.000000)" DeltaSeconds))

(event EventBeginPlay
  (|CallParentFunction)
  (bind _primaryowner (Variables|Default|GetPrimaryOwner)
    (:then
      (bind _ai (Variables|/Game/Blueprints/BP_PlayerPrimary.BP_PlayerPrimary_C|GetAI _primaryowner)
        (:then
          (Utilities|Array|Add (Utilities|Struct|BreakUnitInventory (Variables|/Game/Blueprints/BP_OpulentiumAI.BP_OpulentiumAI_C|GetUnitInventory _ai)) self))
        (:else)))
    (:else)))

(event EventDestroyed
  (|CallParentFunction)
  (bind _primaryowner (Variables|Default|GetPrimaryOwner)
    (:then
      (bind _ai (Variables|/Game/Blueprints/BP_PlayerPrimary.BP_PlayerPrimary_C|GetAI _primaryowner)
        (:then
          (Utilities|Array|RemoveItem (Utilities|Struct|BreakUnitInventory (Variables|/Game/Blueprints/BP_OpulentiumAI.BP_OpulentiumAI_C|GetUnitInventory _ai)) self))
        (:else)))
    (:else)))

(fn ConstructionScript
  (|CallParentFunction))