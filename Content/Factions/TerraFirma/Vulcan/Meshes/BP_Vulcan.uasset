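; Vulcan character Blueprint for the Terra Firma faction, which toggles between walking and a stationary gun mode with right mouse.
; A GunMode RepNotify disables movement in gun mode, or stops fire and waits briefly before restoring walking on exit.
; While in gun mode, Yaw tracks the camera and holding left mouse fires the first weapon after a short timer delay, cancelled on release.
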(event Custom|EventRepGunMode
  (if (Variables|Default|GetbGunMode)
    _
    (else
      (CallFunction|StopFire)
      (Utilities|FlowControl|Delay 0.888888888)))
  (Pawn|Components|CharacterMovement|SetMovementMode (Variables|Character|GetCharacterMovement) (select (Variables|Default|GetbGunMode) "MOVE_None" "MOVE_Walking") 0))

(event Custom|StopFire
  (Variables|/Game/Blueprints/BP_Weapon.BP_Weapon_C|SetbFiring (Utilities|Array|Get(acopy) (Variables|Default|GetWeapons)) false)
  (Variables|Default|SetbFiring false))

(event Custom|StartFire
  (Variables|/Game/Blueprints/BP_Weapon.BP_Weapon_C|SetbFiring (Utilities|Array|Get(acopy) (Variables|Default|GetWeapons)) true)
  (Variables|Default|SetbFiring true))

(event EventTick
  (params (DeltaSeconds :type Float%20%28single-precision%29))
  (|CallParentFunction DeltaSeconds)
  (if (Variables|Default|GetbGunMode)
    (Variables|Default|SetYaw (.Yaw (Math|Rotator|BreakRotator (Transformation|GetWorldRotation (Variables|Default|GetCamera)))))))

(event EventPossessed
  (params (NewController :type Controller%20Object%20Reference))
  (|CallParentFunction NewController)
  (if (Variables|Default|GetbGunMode)
    (Pawn|Components|CharacterMovement|SetMovementMode (Variables|Character|GetCharacterMovement) "MOVE_None" 0)))

(event Input|MouseEvents|RightMouseButton
  (params (Key :type Key%20Structure :default "AnyKey"))
  (:Pressed
    (bind _output_get (Variables|Default|SetbGunMode (not (stale _output_get))))))

(event Input|MouseEvents|LeftMouseButton
  (params (Key :type Key%20Structure :default "AnyKey"))
  (bind _bgunmode (Variables|Default|GetbGunMode))
  (:Pressed
    (if _bgunmode
      (bind _returnvalue (Utilities|Time|SetTimerbyEvent (delegate Custom|StartFire) 0.3))))
  (:Released
    (if _bgunmode
      (Class|KismetSystemLibrary|ClearTimerHandle _returnvalue)
      (CallFunction|StopFire))))

(fn ConstructionScript
  (|CallParentFunction)
  (Class|SceneComponent|Attachto (Variables|Default|GetVulcan_Handle) (Variables|Character|GetMesh) "HandleSocket" "KeepRelativeOffset" true))

(fn OnRepBGunMode
  (CallFunction|EventRepGunMode))