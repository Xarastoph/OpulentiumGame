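; Weapon for the TerraFirma PTV that steers each fired projectile toward what the vehicle camera is aimed at.
; After the parent fire logic, if the pilot is the vehicle's primary owner, it traces from the camera, ignoring territory volumes, vehicle and pilot.
; An enemy Opulentium actor hit becomes the projectile's homing target.
; Otherwise, a dummy actor spawned at the hit point or trace end serves as the target.
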(event EventStartFire
  (|CallParentFunction)
  (bind _currentproj (Variables|Default|GetCurrentProj)
    (:then
      (bind _combatowner (Variables|Default|GetCombatOwner)
        (:then
          (bind _asbp_vehicle (Utilities|Casting|CastToBP_Vehicle _combatowner))
          (if (== (Variables|/Game/Blueprints/BP_Vehicle.BP_Vehicle_C|GetPilot _asbp_vehicle) (Variables|/Game/Blueprints/BP_OpulentiumActor.BP_OpulentiumActor_C|GetPrimaryOwner _asbp_vehicle))
            (bind (_outhit _returnvalue) (Collision|LineTraceByChannel (Transformation|GetWorldLocation (Variables|/Game/Blueprints/BP_Vehicle.BP_Vehicle_C|GetCamera _asbp_vehicle)) (+ (Math|Vector|RotateVector "10000.000000,0.000000,0.000000" (Transformation|GetWorldRotation (Variables|/Game/Blueprints/BP_Vehicle.BP_Vehicle_C|GetCamera _asbp_vehicle))) (Transformation|GetWorldLocation (Variables|/Game/Blueprints/BP_Vehicle.BP_Vehicle_C|GetCamera _asbp_vehicle))) "TraceTypeQuery1" false (CallFunction|IgnoreActors) "None"))
            (bind _asbp_opulentium_actor (Utilities|Casting|CastToBP_OpulentiumActor (.HitActor (Collision|BreakHitResult _outhit)))
              (:then
                (if (!= (Variables|/Game/Blueprints/BP_OpulentiumActor.BP_OpulentiumActor_C|GetTeam _asbp_opulentium_actor) (Variables|/Game/Blueprints/BP_OpulentiumActor.BP_OpulentiumActor_C|GetTeam _combatowner))
                  (Variables|/Script/Engine.ProjectileMovementComponent|SetHomingTargetComponent (Variables|/Game/Blueprints/BP_Projectile.BP_Projectile_C|GetProjectileMovement _currentproj) (VehicleSound|GetRootComponent _asbp_opulentium_actor))
                  (else
                    (bind _returnvalue_2 (Game|SpawnActorfromClass "/Game/Blueprints/DummyActor.DummyActor_C" (Math|Conversions|ToTransform(Vector) (+ (* (.Location (Collision|BreakHitResult _outhit)) (Math|Conversions|ToInteger(Boolean) _returnvalue)) (* (.TraceEnd (Collision|BreakHitResult _outhit)) (Math|Conversions|ToInteger(Boolean) (not _returnvalue))))) "AlwaysSpawn" 0 0 :!label _label))
                    (Utilities|IsValid _returnvalue_2
                      (:Is%20Valid
                        (Variables|/Script/Engine.ProjectileMovementComponent|SetHomingTargetComponent (Variables|/Game/Blueprints/BP_Projectile.BP_Projectile_C|GetProjectileMovement _currentproj) (Variables|/Game/Blueprints/DummyActor.DummyActor_C|GetDefaultSceneRoot _returnvalue_2)))))))
              (:CastFailed
                (goto _label)))))
        (:else)))
    (:else)))

(fn ConstructionScript
  (|CallParentFunction))

(fn IgnoreActors
  (bind _combatowner (Variables|Default|GetCombatOwner)
    (:then
      (bind _asbp_vehicle (Utilities|Casting|CastToBP_Vehicle _combatowner)
        (:then
          (bind _pilot (Variables|/Game/Blueprints/BP_Vehicle.BP_Vehicle_C|GetPilot _asbp_vehicle)
            (:then
              (bind _outactors (Actor|GetAllActorsOfClass "/Game/Environment/Objects/TerritoryVolume/BP_TerritoryVolume.BP_TerritoryVolume_C"))
              (bind _output_get (LocalVariables|SetReturn _outactors))
              (Utilities|Array|Add _output_get _asbp_vehicle)
              (Utilities|Array|Add _output_get _pilot))
            (:else
              _)))
        (:CastFailed
          _)))
    (:else
      _))
  (return _output_get))