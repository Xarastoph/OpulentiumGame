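; BP_TFPTV is the Terra Firma faction's PTV, a pilotable child Blueprint with a movement component.
; Each tick, it gives its Cube physics-only collision when it has no pilot and is not falling, and disables that collision otherwise.
; Shortly after BeginPlay, it adopts the first BP_PlayerPrimary's team and player controller as owner, running parent BeginPlay only if that player is valid.
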(event EventBeginPlay
  (Utilities|FlowControl|Delay 0.2)
  (bind _outactors (Actor|GetAllActorsOfClass "/Game/Blueprints/BP_PlayerPrimary.BP_PlayerPrimary_C"))
  (Utilities|IsValid (Utilities|Array|Get(acopy) _outactors)
    (:Is%20Valid
      (bind _output_get (Variables|Default|SetPrimaryOwner (Utilities|Array|Get(acopy) _outactors)))
      (Variables|Default|SetTeam (Variables|/Game/Blueprints/BP_OpulentiumActor.BP_OpulentiumActor_C|GetTeam _output_get))
      (Actor|SetOwner (Variables|/Game/Blueprints/BP_PlayerPrimary.BP_PlayerPrimary_C|GetPlayerController _output_get))
      (|CallParentFunction))))

(event EventTick
  (params (DeltaSeconds :type Float%20%28single-precision%29))
  (bind _cube (Variables|Default|GetCube))
  (|CallParentFunction DeltaSeconds)
  (if (Math|Boolean|NORBoolean (Utilities|IsValid (Variables|Default|GetPilot)) (AI|Components|NavMovement|IsFalling (Pawn|GetMovementComponent)))
    (Collision|SetCollisionEnabled _cube "PhysicsOnly")
    (else
      (Collision|SetCollisionEnabled _cube "NoCollision"))))

(fn ConstructionScript
  (|CallParentFunction))