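; Terra Firma Vehicle Beacon, a production structure that adds a scan visual to its parent's build queue behavior.
; On BeginPlay it creates a dynamic material on the mesh with the scan hidden.
; Each valid build starts timers that show the scan after a short delay and hide it shortly before build time ends, by toggling the ShowScan parameter.
; Cancelling a unit that empties the queue clears both timers and hides the scan.
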(event Custom|SetScanHidden
  (bind _scanmat (Variables|Default|GetScanMat)
    (:then
      (Rendering|Material|SetScalarParameterValue _scanmat "ShowScan" 0.0 :!class /Script/Engine.MaterialInstanceDynamic))
    (:else)))

(event Custom|SetScanVisible
  (bind _scanmat (Variables|Default|GetScanMat)
    (:then
      (Rendering|Material|SetScalarParameterValue _scanmat "ShowScan" 1.0 :!class /Script/Engine.MaterialInstanceDynamic))
    (:else)))

(event EventBeginPlay
  (|CallParentFunction)
  (bind _returnvalue (Rendering|Material|CreateDynamicMaterialInstance (Variables|Character|GetMesh) 1 "/Game/Factions/TerraFirma/VehicleBeacon/Materials/TFVB_ID03_Inst.TFVB_ID03_Inst" :!class /Script/Engine.PrimitiveComponent))
  (bind _output_get (Variables|Default|SetScanMat _returnvalue))
  (Rendering|Material|SetScalarParameterValue _output_get "ShowScan" 0.0 :!class /Script/Engine.MaterialInstanceDynamic))

(event EventCancelUnit
  (params (Index :type Integer))
  (|CallParentFunction Index)
  (if (== (Utilities|Array|Length (Variables|Default|GetBuildQueue)) 0)
    (Class|KismetSystemLibrary|ClearTimerHandle (stale EventBuildActor _returnvalue))
    (Class|KismetSystemLibrary|ClearTimerHandle (stale EventBuildActor _returnvalue_2))
    (CallFunction|SetScanHidden)))

(event EventBuildActor
  (|CallParentFunction)
  (bind _currentbuild (Variables|Default|GetCurrentBuild)
    (:then
      (Rendering|Material|SetScalarParameterValue (stale EventBeginPlay _output_get) "ShowScan" 0.0 :!class /Script/Engine.MaterialInstanceDynamic)
      (bind _returnvalue (Utilities|Time|SetTimerbyEvent (delegate Custom|SetScanVisible) 2.0))
      (bind _returnvalue_2 (Utilities|Time|SetTimerbyEvent (delegate Custom|SetScanHidden) (- (Variables|/Game/Blueprints/BP_UnitBuild.BP_UnitBuild_C|GetBuildTime _currentbuild) 3.0))))
    (:else)))

(fn ConstructionScript
  (|CallParentFunction))