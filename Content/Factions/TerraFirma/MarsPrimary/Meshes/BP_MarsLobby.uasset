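; BP_MarsLobby is the lobby variant of the Terra Firma Mars character, holding a weapon and supplying aim data for it.
; BeginPlay spawns BP_MarsWeapon01 at the right-hand socket, attaches it to the mesh and stores it as Weapon.
; Each Tick, on authority only, it sets WeaponRot from the gun pivot toward a point far ahead of the camera, and IKTargetOffset as a short vector toward the camera.
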(event EventBeginPlay
  (bind _mesh (Variables|Character|GetMesh))
  (|CallParentFunction)
  (bind _returnvalue (Game|SpawnActorfromClass "/Game/Factions/TerraFirma/MarsPrimary/Weapon/BP_MarsWeapon01.BP_MarsWeapon01_C" (Transformation|GetSocketTransform _mesh "Socket_WeaponRH" "RTS_World") "AlwaysSpawn" self 0))
  (Class|Actor|AttachRootComponentto _returnvalue _mesh "SOcket_WeaponRH" "KeepWorldPosition" true)
  (Variables|Default|SetWeapon _returnvalue))

(event EventTick
  (params (DeltaSeconds :type Float%20%28single-precision%29))
  (bind _camera (Variables|Default|GetCamera))
  (bind _returnvalue (Transformation|GetWorldLocation _camera))
  (|CallParentFunction DeltaSeconds)
  (Networking|SwitchHasAuthority
    (:Authority
      (bind _weapon (Variables|Default|GetWeapon)
        (:then
          (Variables|Default|SetWeaponRot (Math|Rotator|FindLookatRotation (Transformation|GetSocketLocation (Variables|/Game/Blueprints/BP_Weapon.BP_Weapon_C|GetSkeletalMesh _weapon) (Variables|/Game/Blueprints/BP_Weapon.BP_Weapon_C|GetGunPivotName _weapon)) (+ _returnvalue (* (Math|Vector|GetForwardVector (Transformation|GetWorldRotation _camera)) 2048.0))))
          (Variables|Default|SetIKTargetOffset (* (Math|Vector|Normalize (- _returnvalue (Transformation|GetSocketLocation (Variables|/Game/Blueprints/BP_Weapon.BP_Weapon_C|GetSkeletalMesh _weapon) (Variables|/Game/Blueprints/BP_Weapon.BP_Weapon_C|GetGunPivotName _weapon)))) 1e+01)))
        (:else)))))

(fn ConstructionScript)